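; Title logo actor that animates a billboard's opacity mask after a short delay at BeginPlay.
; The Count timeline acts as an update driver, stepping RefVal down while it stays above a floor and applying it as the Billboard's opacity mask threshold.
; Lowering the threshold gradually reveals more of the sprite, at a frame-rate-dependent speed because each update subtracts a fixed amount.
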(event EventTick
  (params (DeltaSeconds :type Float%20%28single-precision%29)))

(event EventBeginPlay
  (Utilities|FlowControl|Delay 0.5)
  (Timeline|count Play
    (:Update
      (if (> (Variables|Default|GetRef%20Val) 0.5)
        (Variables|Default|SetRef%20Val (- (Variables|Default|GetRef%20Val) 0.002))
        (Class|BillboardComponent|SetOpacityMaskRefVal (Variables|Default|GetBillboard) (Variables|Default|GetRef%20Val))))))

(fn ConstructionScript)