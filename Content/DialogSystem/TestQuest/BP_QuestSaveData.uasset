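; Save data container for the quest system that records and restores each quest's stage and objective progress.
; QuestSaveDatalist stores a quest's current stage and objective progress in the QuestProgress map, keyed by its quest ID.
; LoadQuest re-adds each ID in CrrentActiveQuests through the quest log component, then applies the saved values to the returned quest.
; The active quest list is only read here, not filled.
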(fn QuestSaveDatalist
  (params (QuestID :type BP%20Quest%20Bass%20Object%20Reference))
  (Utilities|Map|Add (Variables|Default|GetQuestProgress) (Variables|/Game/DialogSystem/TestQuest/BP_Quest_Bass.BP_Quest_Bass_C|GetQuestID QuestID) (Utilities|Struct|MakeS_QuestSaveData (Variables|/Game/DialogSystem/TestQuest/BP_Quest_Bass.BP_Quest_Bass_C|GetCurrentObjectiveProgress QuestID) (Variables|/Game/DialogSystem/TestQuest/BP_Quest_Bass.BP_Quest_Bass_C|GetCurrentStage QuestID))))

(fn LoadQuest
  (params (LogQuestComponent :type BPC%20Quest%20Log%20Component%20Object%20Reference))
  (for _array_element (Variables|Default|GetCrrentActiveQuests)
    (bind _returnvalue (Default|AddNewQuest LogQuestComponent _array_element))
    (Variables|/Game/DialogSystem/TestQuest/BP_Quest_Bass.BP_Quest_Bass_C|SetCurrentStage _returnvalue (.Current (Utilities|Struct|BreakS_QuestSaveData (.Value (Utilities|Map|Find (Variables|Default|GetQuestProgress) _array_element)))))
    (Variables|/Game/DialogSystem/TestQuest/BP_Quest_Bass.BP_Quest_Bass_C|SetCurrentObjectiveProgress _returnvalue (.Progress (Utilities|Struct|BreakS_QuestSaveData (.Value (Utilities|Map|Find (Variables|Default|GetQuestProgress) _array_element)))))))