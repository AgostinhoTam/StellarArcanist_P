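; Quest actor, apparently a base, that tracks objective progress for the current stage of a quest read from DT_QuestTable.
; It listens to the player's objective ID event and seeds one objective type from quest inventory counts at BeginPlay.
; Reaching a required quantity shows a notification; completing all objectives saves the quest log and active quests to the save slot.
; The delayed level-open event has no live caller here.
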(event Custom|openlevel
  (if (Variables|Default|GetIsCompleted)
    (Utilities|FlowControl|Delay 1.0)
    (Game|OpenLevel(byObjectReference) "/Game/Level/Clear1_Bar2.Clear1_Bar2")))

(event EventBeginPlay
  (CallFunction|GetQuestDatalist)
  (EventDispatchers|BindEventtoOnObjectiveIDCalled (CallFunction|GetMyPlayerCharacter) (EventDispatchers|CreateEvent :!event OnObjectiveIDHeard))
  (for _array_element (.Objectivs (Utilities|Struct|BreakS_Stage_Datalist (Variables|Default|GetCurrentStageDatalist)))
    (if (Utilities|Enum|Equal(Enum) (.type (Utilities|Struct|BreakS_Object_Datalist _array_element)) "NewEnumerator3")
      (bind _value (Default|QueryInventory (Variables|/Game/ThirdPerson/Blueprints/BP_ThirdPersonCharacter.BP_ThirdPersonCharacter_C|GetBPC_Quest_InventoryComponent (CallFunction|GetMyPlayerCharacter)) (Utilities|String|StringToName (.ObjectiveID (Utilities|Struct|BreakS_Object_Datalist _array_element)))))
      (CallFunction|OnObjectiveIDHeard (.ObjectiveID (Utilities|Struct|BreakS_Object_Datalist _array_element)) _value)))
  (bind _return (CallFunction|AreObjectiveComplted))
  (if _return
    _))

(fn ConstructionScript)

(fn OnObjectiveIDHeard
  (params (ObjectiveID :type String) (Value :type Integer))
  (bind _currentobjectiveprogress (Variables|Default|GetCurrentObjectiveProgress))
  (bind (_value _returnvalue) (Utilities|Map|Find _currentobjectiveprogress ObjectiveID))
  (if _returnvalue
    (if (< _value (Utilities|Struct|BreakS_Object_Datalist (CallFunction|GetObjectiveDatabyID ObjectiveID)))
      (Utilities|Map|Add (Variables|Default|GetCurrentObjectiveProgress) ObjectiveID (+ _value Value))
      (CallFunction|IsObjectiveComplted ObjectiveID)
      (return)
      (else
        (return)))
    (else
      (Utilities|Map|Add (Variables|Default|GetCurrentObjectiveProgress) ObjectiveID (+ (.Value (Utilities|Map|Find (Variables|Default|GetCurrentObjectiveProgress) ObjectiveID)) Value))
      (return))))

(fn GetQuestDatalist
  (bind _returnvalue (Utilities|GetDataTableRow "/Game/DialogSystem/TestQuest/DT_QuestTable.DT_QuestTable" (Variables|Default|GetQuestID))
    (:then
      (bind _output_get (Variables|Default|SetQuestDatalist _returnvalue))
      (bind _output_get_2 (Variables|Default|SetCurrentStageDatalist (Utilities|Array|Get(acopy) (.Stages (Utilities|Struct|BreakS_Quest_Datalist _output_get)) (Variables|Default|GetCurrentStage))))
      (Utilities|Map|Clear (Variables|Default|GetCurrentObjectiveProgress))
      (for _array_element (.Objectivs (Utilities|Struct|BreakS_Stage_Datalist _output_get_2))
        (Utilities|Map|Add (Variables|Default|GetCurrentObjectiveProgress) (.ObjectiveID (Utilities|Struct|BreakS_Object_Datalist _array_element)) 0)))))

(fn GetObjectiveDatabyID
  (params (ObjectiveID :type String))
  (for _array_element (.Objectivs (Utilities|Struct|BreakS_Stage_Datalist (Variables|Default|GetCurrentStageDatalist)))
    (if (Utilities|Enum|Equal(Enum) (.ObjectiveID (Utilities|Struct|BreakS_Object_Datalist _array_element)) ObjectiveID)
      (return _array_element))))

(fn IsObjectiveComplted
  (params (ObjectiveID :type String))
  (bind _array_element (CallFunction|GetObjectiveDatabyID ObjectiveID))
  (bind (_description _quantity) (Utilities|Struct|BreakS_Object_Datalist _array_element))
  (if (>= (.Value (Utilities|Map|Find (Variables|Default|GetCurrentObjectiveProgress) ObjectiveID)) _quantity)
    (bind _returnvalue (UserInterface|CreateWidget "/Game/DialogSystem/TestQuest/W_QuestNotification.W_QuestNotification_C" 0 _description))
    (UserInterface|Viewport|AddtoViewport _returnvalue 0)
    (bind _return (CallFunction|AreObjectiveComplted))
    (Default|GetQuestActor (Variables|/Game/ThirdPerson/Blueprints/BP_ThirdPersonCharacter.BP_ThirdPersonCharacter_C|GetBPC_Quest_LogComponent (CallFunction|GetMyPlayerCharacter)) (.rowname (Variables|Default|GetQuestData)))
    (bind _output_get (Variables|Default|SetIsCompleted _return))
    (if _output_get
      (bind _asbp_magic_game_instance (Utilities|Casting|CastToBP_MagicGameInstance (Game|GetGameInstance)))
      (bind _asbp_third_person_character (Utilities|Casting|CastToBP_ThirdPersonCharacter (Game|GetPlayerCharacter 0)))
      (Variables|Default|SetAs%20BP%20Magic%20Game%20Instance _asbp_magic_game_instance)
      (for _array_element_2 (Variables|/Game/DialogSystem/TestQuest/BPC_Quest_LogComponent.BPC_Quest_LogComponent_C|GetCurrentQuest (Variables|/Game/ThirdPerson/Blueprints/BP_ThirdPersonCharacter.BP_ThirdPersonCharacter_C|GetBPC_Quest_LogComponent _asbp_third_person_character))
        (Default|SaveQuestDatalist (Variables|/Game/Scene/BP_MagicGameInstance.BP_MagicGameInstance_C|GetSaveData (Variables|Default|GetAs%20BP%20Magic%20Game%20Instance)) _array_element_2))
      (Default|SaveQuestLog (Variables|/Game/Scene/BP_MagicGameInstance.BP_MagicGameInstance_C|GetSaveData (Variables|Default|GetAs%20BP%20Magic%20Game%20Instance)) (Variables|/Game/ThirdPerson/Blueprints/BP_ThirdPersonCharacter.BP_ThirdPersonCharacter_C|GetBPC_Quest_LogComponent _asbp_third_person_character))
      (SaveGame|SaveGametoSlot (Variables|/Game/Scene/BP_MagicGameInstance.BP_MagicGameInstance_C|GetSaveData (Variables|Default|GetAs%20BP%20Magic%20Game%20Instance)) "savedata"))))

(fn AreObjectiveComplted
  (for _array_element (.Objectivs (Utilities|Struct|BreakS_Stage_Datalist (Variables|Default|GetCurrentStageDatalist)))
    (if (not (>= (.Value (Utilities|Map|Find (Variables|Default|GetCurrentObjectiveProgress) (.ObjectiveID (Utilities|Struct|BreakS_Object_Datalist _array_element)))) (.Quantity (Utilities|Struct|BreakS_Object_Datalist (CallFunction|GetObjectiveDatabyID (.ObjectiveID (Utilities|Struct|BreakS_Object_Datalist _array_element)))))))
      (bind _output_get (LocalVariables|SetLocalAllComplete false))
      (return _output_get)))
  (return (LocalVariables|GetLocalAllComplete)))