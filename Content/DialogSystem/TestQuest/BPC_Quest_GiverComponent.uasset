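; Quest giver component that handles player interaction with its owning actor for the quest stored in its QuestData.
; InteractWith queries the player's quest log component, opening a quest select widget if the quest is not active, or calling DisplayReward if its quest actor is completed.
; Both branches return the owner's display name.
; DisplayReward is unfinished: it only looks up the quest table row, with its AddToViewport left unwired.
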(fn DisplayQuest
  (bind _returnvalue (UserInterface|CreateWidget "/Game/DialogSystem/TestQuest/WBP_QuestSelect.WBP_QuestSelect_C"))
  (UserInterface|Viewport|AddtoViewport _returnvalue 0))

(fn DisplayReward
  (Utilities|GetDataTableRow "/Game/DialogSystem/TestQuest/DT_QuestTable.DT_QuestTable" (.rowname (Variables|Default|GetQuestData))))

(fn Interactwith
  (bind _returnvalue (Components|GetOwner))
  (bind _returnvalue_2 (Utilities|GetDisplayName _returnvalue))
  (if (not (Default|QueryActiveQuest (Variables|/Game/ThirdPerson/Blueprints/BP_ThirdPersonCharacter.BP_ThirdPersonCharacter_C|GetBPC_Quest_LogComponent (CallFunction|GetMyPlayerCharacter)) (.rowname (Variables|Default|GetQuestData))))
    (CallFunction|DisplayQuest)
    (return _returnvalue_2)
    (else
      (bind _array_element (Default|GetQuestActor (Variables|/Game/ThirdPerson/Blueprints/BP_ThirdPersonCharacter.BP_ThirdPersonCharacter_C|GetBPC_Quest_LogComponent (CallFunction|GetMyPlayerCharacter)) (.rowname (Variables|Default|GetQuestData))))
      (if (Variables|/Game/DialogSystem/TestQuest/BP_Quest_Bass.BP_Quest_Bass_C|GetIsCompleted _array_element)
        (CallFunction|DisplayReward)
        (return _returnvalue_2)))))