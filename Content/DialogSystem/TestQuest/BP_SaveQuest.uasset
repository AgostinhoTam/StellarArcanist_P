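; BP_SaveQuest holds saved quest state: active and completed quest lists, plus a map of stage and objective progress per quest ID.
; SaveQuestLog copies both lists from the quest log component, while SaveQuestDatalist records one quest's progress in the map.
; LoadQuestData re-adds each active quest through the component, restores its stage and progress from the map, then writes both lists back.
; No disk read or write happens in these functions.
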(fn SaveQuestDatalist
  (params (Quest :type BP%20Quest%20Bass%20Object%20Reference))
  (Utilities|Map|Add (Variables|Default|GetQuestProgress) (Variables|/Game/DialogSystem/TestQuest/BP_Quest_Bass.BP_Quest_Bass_C|GetQuestID Quest) (Utilities|Struct|MakeS_QuestSaveData (Variables|/Game/DialogSystem/TestQuest/BP_Quest_Bass.BP_Quest_Bass_C|GetCurrentObjectiveProgress Quest) (Variables|/Game/DialogSystem/TestQuest/BP_Quest_Bass.BP_Quest_Bass_C|GetCurrentStage Quest))))

(fn LoadQuestData
  (params (QuestLogComponent :type BPC%20Quest%20Log%20Component%20Object%20Reference))
  (for _array_element (Variables|Default|GetCurrentActiveQuest)
    (bind _returnvalue (Default|AddNewQuest QuestLogComponent _array_element))
    (Variables|/Game/DialogSystem/TestQuest/BP_Quest_Bass.BP_Quest_Bass_C|SetCurrentStage _returnvalue (.CurrentStage (Utilities|Struct|BreakS_QuestSaveData (.Value (Utilities|Map|Find (Variables|Default|GetQuestProgress) _array_element)))))
    (Variables|/Game/DialogSystem/TestQuest/BP_Quest_Bass.BP_Quest_Bass_C|SetCurrentObjectiveProgress _returnvalue (.Progress (Utilities|Struct|BreakS_QuestSaveData (.Value (Utilities|Map|Find (Variables|Default|GetQuestProgress) _array_element))))))
  (Variables|/Game/DialogSystem/TestQuest/BPC_Quest_LogComponent.BPC_Quest_LogComponent_C|SetCurrentActiveQuest QuestLogComponent (Variables|Default|GetCurrentActiveQuest))
  (Variables|/Game/DialogSystem/TestQuest/BPC_Quest_LogComponent.BPC_Quest_LogComponent_C|SetCompletedQuest QuestLogComponent (Variables|Default|GetCompletedQuest)))

(fn SaveQuestLog
  (params (QuestLogComponent :type BPC%20Quest%20Log%20Component%20Object%20Reference))
  (Variables|Default|SetCurrentActiveQuest (Variables|/Game/DialogSystem/TestQuest/BPC_Quest_LogComponent.BPC_Quest_LogComponent_C|GetCurrentActiveQuest QuestLogComponent))
  (Variables|Default|SetCompletedQuest (Variables|/Game/DialogSystem/TestQuest/BPC_Quest_LogComponent.BPC_Quest_LogComponent_C|GetCompletedQuest QuestLogComponent)))