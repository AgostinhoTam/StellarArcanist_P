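; Quest log component that tracks active quests and handles turn-in rewards.
; AddNewQuest records the quest ID and spawns a BP_Quest_Bass actor, which GetQuestActor finds by ID.
; TurnInQuest adds a hardcoded Attribute_Fire magic chip to the player's inventory, saves the chip list to BP_SavePlayerData, then removes the ID from the active list.
; TrackQuest is an empty stub, and completed quest actors remain stored.
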(event EventBeginPlay)

(event EventTick
  (params (DeltaSeconds :type Float%20%28single-precision%29)))

(fn AddNewQuest
  (params (QuestID :type Name))
  (Utilities|Array|AddUnique (Variables|Default|GetCurrentActiveQuest) QuestID)
  (bind _returnvalue (Game|SpawnActorfromClass "/Game/DialogSystem/TestQuest/BP_Quest_Bass.BP_Quest_Bass_C" (Math|Transform|MakeTransform "0, 0, 0" "0, 0, 0" "1.000000,1.000000,1.000000") "Undefined" "MultiplyWithRoot" 0 QuestID 0))
  (Utilities|Array|Add (Variables|Default|GetCurrentQuest) _returnvalue))

(fn CompleteQuest
  (params (QuestID :type Name%20%28by%20ref%29))
  (Utilities|Array|AddUnique (Variables|Default|GetCurrentActiveQuest) QuestID)
  (Utilities|Array|RemoveItem (Variables|Default|GetCurrentActiveQuest) QuestID))

(fn QueryActiveQuest
  (params (QuestID :type Name))
  (return (Utilities|Array|ContainsItem (Variables|Default|GetCurrentActiveQuest) QuestID)))

(fn TrackQuest)

(fn GetQuestActor
  (params (QuestID :type Name))
  (for _array_element (Variables|Default|GetCurrentQuest)
    (if (== (Variables|/Game/DialogSystem/TestQuest/BP_Quest_Bass.BP_Quest_Bass_C|GetQuestID _array_element) QuestID)
      (return _array_element))))

(fn TurninQuest
  (params (QuestID :type Name))
  (bind _returnvalue (Game|GetPlayerCharacter 0))
  (Utilities|FlowControl|Sequence
    (:then_0
      (bind _array_element (CallFunction|GetQuestActor QuestID))
      (Utilities|FlowControl|Sequence
        (:then_0
          (|SetBy-RefVar (.ItemReward (Utilities|Struct|BreakS_Stage_Datalist (Variables|/Game/DialogSystem/TestQuest/BP_Quest_Bass.BP_Quest_Bass_C|GetCurrentStageDatalist _array_element))) (Variables|Default|GetItem%20Reward))
          (bind _returnvalue_2 (Utilities|GetDataTableRow "/Game/DataTables/DT_MagicChipInfo_Ver2.DT_MagicChipInfo_Ver2" "Attribute_Fire")
            (:then
              (Class|BPIMagicInventorySystem|AddInventory(Message) _returnvalue _returnvalue_2)
              (bind _magicchiplists (Class|BPIMagicInventorySystem|GetInventory(Message) _returnvalue))
              (bind _returnvalue_3 (SaveGame|LoadGamefromSlot "BP_SavePlayerData"))
              (bind _asbp_save_player_data (Utilities|Casting|CastToBP_SavePlayerData _returnvalue_3))
              (Variables|/Game/save/BP_SavePlayerData.BP_SavePlayerData_C|SetMagicChipList _asbp_save_player_data _magicchiplists)
              (SaveGame|SaveGametoSlot _asbp_save_player_data "BP_SavePlayerData"))))))
    (:then_1
      (CallFunction|CompleteQuest QuestID))))