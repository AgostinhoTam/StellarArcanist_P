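; Dialogue component for a quest receptionist, who asks whether the player takes a quest and offers two subjugation quests.
; It overrides Dialogue, branching on AddDialogue option indices; declining shows a farewell and closes the conversation.
; Either quest choice copies the player's current quests and quest log into the game instance's SaveData and saves it to slot.
; Each choice's level open is called inside the quest loop, before the save.
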(event EventBeginPlay
  (|CallParentFunction) ; このノードは無効になっているため呼び出せません。\n機能をビルドするにはピンをドラッグしてください。
)

(event EventTick
  (params (DeltaSeconds :type Float%20%28single-precision%29))
  (|CallParentFunction DeltaSeconds) ; このノードは無効になっているため呼び出せません。\n機能をビルドするにはピンをドラッグしてください。
)

(fn Dialogue
  (|CallParentFunction)
  (switch int (Variables|Default|GetDialogueTreeindex	)
    (:0
      (bind (_state _option_index) (CallFunction|AddDialogue "受付人" "本日はどのような御用でしょうか？" (Utilities|Array|MakeArray "クエストを受ける" "クエストを受けない")))
      (switch Utilities|FlowControl|Switch|SwitchonEnum_DialogueState _state
        (:NewEnumerator0
          (switch int _option_index
            (:0
              (bind (_state_2 _option_index_2) (CallFunction|AddDialogue "受付人" "どのクエストを受注しますか。" (Utilities|Array|MakeArray "討伐クエスト1" "討伐クエスト2")))
              (switch Utilities|FlowControl|Switch|SwitchonEnum_DialogueState _state_2
                (:NewEnumerator0
                  (switch int _option_index_2
                    (:0
                      (bind _asbp_magic_game_instance (Utilities|Casting|CastToBP_MagicGameInstance (Game|GetGameInstance)))
                      (bind _asbp_third_person_character (Utilities|Casting|CastToBP_ThirdPersonCharacter (Game|GetPlayerCharacter 0)))
                      (Variables|Default|SetAs%20BP%20Magic%20Game%20Instance _asbp_magic_game_instance)
                      (for _array_element (Variables|/Game/DialogSystem/TestQuest/BPC_Quest_LogComponent.BPC_Quest_LogComponent_C|GetCurrentQuest (Variables|/Game/ThirdPerson/Blueprints/BP_ThirdPersonCharacter.BP_ThirdPersonCharacter_C|GetBPC_Quest_LogComponent _asbp_third_person_character))
                        (Default|SaveQuestDatalist (Variables|/Game/Scene/BP_MagicGameInstance.BP_MagicGameInstance_C|GetSaveData (Variables|Default|GetAs%20BP%20Magic%20Game%20Instance)) _array_element)
                        (Utilities|Casting|CastToBP_ThirdPersonCharacter (Game|GetPlayerCharacter 0))
                        (Game|OpenLevel(byObjectReference) (Variables|Default|GetLevel)))
                      (Default|SaveQuestLog (Variables|/Game/Scene/BP_MagicGameInstance.BP_MagicGameInstance_C|GetSaveData (Variables|Default|GetAs%20BP%20Magic%20Game%20Instance)) (Variables|/Game/ThirdPerson/Blueprints/BP_ThirdPersonCharacter.BP_ThirdPersonCharacter_C|GetBPC_Quest_LogComponent _asbp_third_person_character))
                      (SaveGame|SaveGametoSlot (Variables|/Game/Scene/BP_MagicGameInstance.BP_MagicGameInstance_C|GetSaveData (Variables|Default|GetAs%20BP%20Magic%20Game%20Instance)) "savedata"))
                    (:1
                      (bind _asbp_magic_game_instance_2 (Utilities|Casting|CastToBP_MagicGameInstance (Game|GetGameInstance)))
                      (bind _asbp_third_person_character_2 (Utilities|Casting|CastToBP_ThirdPersonCharacter (Game|GetPlayerCharacter 0)))
                      (Variables|Default|SetAs%20BP%20Magic%20Game%20Instance _asbp_magic_game_instance_2)
                      (for _array_element_2 (Variables|/Game/DialogSystem/TestQuest/BPC_Quest_LogComponent.BPC_Quest_LogComponent_C|GetCurrentQuest (Variables|/Game/ThirdPerson/Blueprints/BP_ThirdPersonCharacter.BP_ThirdPersonCharacter_C|GetBPC_Quest_LogComponent _asbp_third_person_character_2))
                        (Default|SaveQuestDatalist (Variables|/Game/Scene/BP_MagicGameInstance.BP_MagicGameInstance_C|GetSaveData (Variables|Default|GetAs%20BP%20Magic%20Game%20Instance)) _array_element_2)
                        (Utilities|Casting|CastToBP_ThirdPersonCharacter (Game|GetPlayerCharacter 0))
                        (Game|OpenLevel(byObjectReference) (Variables|Default|GetLevel_1)))
                      (Default|SaveQuestLog (Variables|/Game/Scene/BP_MagicGameInstance.BP_MagicGameInstance_C|GetSaveData (Variables|Default|GetAs%20BP%20Magic%20Game%20Instance)) (Variables|/Game/ThirdPerson/Blueprints/BP_ThirdPersonCharacter.BP_ThirdPersonCharacter_C|GetBPC_Quest_LogComponent _asbp_third_person_character_2))
                      (SaveGame|SaveGametoSlot (Variables|/Game/Scene/BP_MagicGameInstance.BP_MagicGameInstance_C|GetSaveData (Variables|Default|GetAs%20BP%20Magic%20Game%20Instance)) "savedata"))))))
            (:1
              (CallFunction|AddDialogue "受付人" "またのご利用お待ちしております。" (Utilities|Array|MakeArray ""))
              (CallFunction|ClearDialogueProgress)
              (CallFunction|CloseConversation))))))))