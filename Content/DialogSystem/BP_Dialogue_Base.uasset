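; Base dialogue Blueprint that runs branching conversations through a W_Dialogue widget, with an empty Dialogue function as the hook for the conversation script.
; Each ProgressDialogue resets the index and replays Dialogue from the start.
; AddDialogue returns the saved option for answered steps or displays the first unanswered one.
; UpdateSelectedOption records choices in the DialogueProgress map and replays; other helpers remove steps or switch tree index and clear progress.
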(event EventBeginPlay)

(event Collision|EventActorBeginOverlap
  (params (OtherActor :type Actor%20Object%20Reference)))

(event EventTick
  (params (DeltaSeconds :type Float%20%28single-precision%29)))

(fn ConstructionScript)

(fn OpenConversation
  (bind _returnvalue (UserInterface|CreateWidget "/Game/DialogSystem/W_Dialogue.W_Dialogue_C" 0 self))
  (bind _output_get (Variables|Default|SetDialogueWidget _returnvalue))
  (UserInterface|Viewport|AddtoViewport _output_get 0)
  (CallFunction|ProgressDialogue))

(fn CloseConversation
  (Widget|RemovefromParent (Variables|Default|GetDialogueWidget)))

(fn ProgressDialogue
  (Variables|Default|SetDialogueindex -1)
  (CallFunction|Dialogue))

(fn Dialogue)

(fn AddDialogue
  (params (Speaker :type Text) (Dialogue :type Text) (Options%20text :type Array%20of%20Texts))
  (bind _dialogueprogress (Variables|Default|GetDialogueProgress))
  (bind _dialogueindex (Variables|Default|GetDialogueindex))
  (bind (_value _returnvalue) (Utilities|Map|Find _dialogueprogress _dialogueindex))
  (Math|Integer|IncrementInt (Variables|Default|GetDialogueindex)
    (:%20%20
      (if _returnvalue
        (return "NewEnumerator0" _value)
        (else
          (Default|UpDateDialogueText (Variables|Default|GetDialogueWidget) (Variables|Default|GetDialogueindex) Speaker Dialogue Options%20text)
          (return "NewEnumerator1" 0))))))

(fn UpdateSelectedOption
  (params (Progress%20Index :type Integer%20%28by%20ref%29) (OptionIndex :type Integer%20%28by%20ref%29))
  (Utilities|Map|Add (Variables|Default|GetDialogueProgress) Progress%20Index OptionIndex)
  (CallFunction|ProgressDialogue))

(fn ClearDialogueProgress
  (Utilities|Map|Clear (Variables|Default|GetDialogueProgress)))

(fn SetDialogTreeindex
  (params (DialogueTreeindex	 :type Integer))
  (Variables|Default|SetDialogueTreeindex	 DialogueTreeindex	)
  (CallFunction|ClearDialogueProgress))

(fn RemoveDialogueProgress
  (params (ProgressSteps :type Integer))
  (for _index (range 0 ProgressSteps)
    (Utilities|Map|Remove (Variables|Default|GetDialogueProgress) (- (Variables|Default|GetDialogueindex) _index))))