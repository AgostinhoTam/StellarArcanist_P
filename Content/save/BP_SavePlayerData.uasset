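; BP_SavePlayerData holds saved player data for created magic and equipped magic, exposed through getter functions.
; Created-magic getters index parallel arrays by magic number for chip data, name, attack, cast time, composition and stamina.
; GetEquipmentNumber looks up an equipment slot number by index.
; GetEquipmentMagic only prints a debug string, as its return of equipped chip data is disconnected and never runs.
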(fn GetCreateMagic
  (params (MagicNumber :type Integer))
  (return (Utilities|Struct|BreakS_MakeMagicData (Utilities|Array|Get(acopy) (Variables|Default|GetCreateMagic) MagicNumber))))

(fn GetCreateMagicAttack
  (params (MagicNumber :type Integer))
  (return (Utilities|Array|Get(acopy) (Variables|Default|GetAttackValue) MagicNumber)))

(fn GetCreateMagicCastTime
  (params (MagicNumber :type Integer))
  (return (Utilities|Array|Get(acopy) (Variables|Default|GetCastTime) MagicNumber)))

(fn GetCreateMagicComposition
  (params (MagicNumber :type Integer))
  (return (Utilities|Array|Get(acopy) (Variables|Default|GetCompositionValue) MagicNumber)))

(fn GetCreateMagicName
  (params (MagicNumber :type Integer))
  (return (Utilities|Array|Get(acopy) (Variables|Default|GetMagicCreateName) MagicNumber)))

(fn GetCreateMagicStamina
  (params (MagicNumber :type Integer))
  (return (Utilities|Array|Get(acopy) (Variables|Default|GetStamina) MagicNumber)))

(fn GetEquipmentMagic
  (params (EquipmentNumber :type Integer))
  (Development|PrintString 0 "使ってます"))

(fn GetEquipmentNumber
  (params (InNumber :type Integer))
  (return (Utilities|Array|Get(acopy) (Variables|Default|GetEquipmentNumber) InNumber)))