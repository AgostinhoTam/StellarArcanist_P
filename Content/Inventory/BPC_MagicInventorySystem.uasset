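; Magic chip inventory component that stores collected MagicChips in an array and exposes it through GetInventory.
; AddInventory adds directly to an empty array, otherwise loops over entries comparing ChipName and breaks after one add.
; The add fires on the first differing name, so a chip is rejected only when every stored entry shares its name, rather than when any does.
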(event Custom|Break
  (Utilities|FlowControl|ForLoopwithBreak 0 (- (Utilities|Array|Length (Variables|Default|GetMagicChipInventory)) 1)) ; enters at Break
)

(event EventBeginPlay)

(event EventTick
  (params (DeltaSeconds :type Float%20%28single-precision%29)))

(event EventAddInventory
  (params (MagicChip :type S%20Magic%20Chip%20Info%20Ver%202%20Structure))
  (bind _magicchipinventory (Variables|Default|GetMagicChipInventory))
  (bind _returnvalue (Utilities|Array|Length _magicchipinventory))
  (if (== _returnvalue 0)
    (Utilities|Array|Add (Variables|Default|GetMagicChipInventory) MagicChip)
    (else
      (bind _index (Utilities|FlowControl|ForLoopwithBreak 0 (- _returnvalue 1))
        (:LoopBody
          (if (not (== (.chipname (.chipstatas (Utilities|Array|Get(acopy) (Variables|Default|GetMagicChipInventory) _index))) (.chipname (.ChipStatas (Utilities|Struct|BreakS_MagicChipInfo_Ver2 MagicChip)))))
            (Utilities|Array|Add (Variables|Default|GetMagicChipInventory) MagicChip)
            (CallFunction|Break)))))))

(fn GetInventory
  (return (Variables|Default|GetMagicChipInventory)))