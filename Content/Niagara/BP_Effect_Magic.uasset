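; BP_Effect_Magic is a magic projectile actor that drives a Niagara bullet effect and spawns explosions from its particle data.
; An endpoint passed to SetEndPoint feeds the effect every tick, and the actor registers itself as the effect's export callback.
; Exported particles trigger zero-length sphere traces, spawning BP_Explosion at the result location without a hit check.
; The actor destroys itself shortly afterward, or after a fixed lifetime.
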(event Custom|SetEndPoint
  (params (Vector :type Vector))
  (Variables|Default|SetVector Vector))

(event EventBeginPlay
  (Class|NiagaraComponent|SetVariableObject (Variables|Default|GetNS_Bullet) "BP_Hit" self)
  (Utilities|FlowControl|Delay 1e+01)
  (Actor|DestroyActor))

(event Collision|EventActorBeginOverlap
  (params (OtherActor :type Actor%20Object%20Reference)))

(event EventTick
  (params (DeltaSeconds :type Float%20%28single-precision%29))
  (Niagara|SetNiagaraVariable(Vector3) (Variables|Default|GetNS_Bullet) "EP" (Variables|Default|GetVector)))

(event EventParticleData
  (params (Data :type Array%20of%20Basic%20Particle%20Data%20Structures) (NiagaraSystem :type Niagara%20System%20Object%20Reference) (SimulationPositionOffset :type Vector%20%28by%20ref%29 :default "0, 0, 0"))
  (for _array_element Data
    (bind _outhit (Collision|SphereTraceByChannel (.Position (Utilities|Struct|BreakBasicParticleData _array_element)) (+ (.Position (Utilities|Struct|BreakBasicParticleData _array_element)) (* (.Velocity (Utilities|Struct|BreakBasicParticleData _array_element)) "")) (* (.Size (Utilities|Struct|BreakBasicParticleData _array_element)) 1.0) "TraceTypeQuery1" false 0 "None"))
    (Game|SpawnActorfromClass "/Game/Niagara/BP_Explosion.BP_Explosion_C" (Math|Conversions|ToTransform(Vector) (.Location (Collision|BreakHitResult _outhit))) "Undefined" "MultiplyWithRoot" 0 0)
    (Utilities|FlowControl|Delay 2.0)
    (Actor|DestroyActor)))

(fn ConstructionScript)