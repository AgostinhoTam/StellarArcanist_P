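; BP_Portal_Scene is a level-transition portal that loads its assigned Level when a BP_ThirdPersonCharacter overlaps its Box.
; Its Billboard shows a configurable Sprite, set at BeginPlay.
; In the Tutorial_MagicCreateMap_new level, entry also reports the "createmagic" objective on the character and saves a newly created BP_SavePlayerData to the Tutorial slot.
; The level opens after a short delay in every case.
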(event OnComponentBeginOverlap(Box)
  (params (OverlappedComponent :type Primitive%20Component%20Object%20Reference) (OtherActor :type Actor%20Object%20Reference) (OtherComp :type Primitive%20Component%20Object%20Reference) (OtherBodyIndex :type Integer) (bFromSweep :type Boolean) (SweepResult :type Hit%20Result%20Structure%20%28by%20ref%29))
  (bind _asbp_third_person_character (Utilities|Casting|CastToBP_ThirdPersonCharacter OtherActor))
  (bind _returnvalue (Game|GetCurrentLevelName true))
  (Utilities|FlowControl|Sequence
    (:then_0
      (if (== _returnvalue "Tutorial_MagicCreateMap_new")
        (Default|CallOnObjectiveIDCalled _asbp_third_person_character "createmagic" 1)
        (bind _returnvalue_2 (SaveGame|CreateSaveGameObject "/Game/save/BP_SavePlayerData.BP_SavePlayerData_C"))
        (SaveGame|SaveGametoSlot _returnvalue_2 "Tutorial")))
    (:then_1
      (Utilities|FlowControl|Delay 0.4)
      (Game|OpenLevel(byObjectReference) (Variables|Default|GetLevel)))))

(event EventBeginPlay
  (Rendering|Components|Sprite|SetSprite (Variables|Default|GetBillboard) (Variables|Default|Getsprite)))

(fn ConstructionScript)