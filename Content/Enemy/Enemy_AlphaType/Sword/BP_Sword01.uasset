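; Enemy sword Blueprint that deals SwordDamage to actors overlapping its SwordCollision, intended to hit the player.
; SwordActive and SwordDeactive custom events, meant for AnimNotifies, toggle the collision during attacks.
; Overlaps pass through a DoOnce that resets one second after damage to limit repeat hits.
; The player-character comparison feeds that DoOnce, while the preceding Branch is fixed to true.
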(event OnComponentBeginOverlap(SwordCollision)
  (params (OverlappedComponent :type Primitive%20Component%20Object%20Reference) (OtherActor :type Actor%20Object%20Reference) (OtherComp :type Primitive%20Component%20Object%20Reference) (OtherBodyIndex :type Integer) (bFromSweep :type Boolean) (SweepResult :type Hit%20Result%20Structure%20%28by%20ref%29))
  ;[1 1 1] overlapした時にプレイヤーだった場合、applydamageで敵にダメージを与える
  (if true
    (Utilities|FlowControl|DoOnce (== OtherActor (Game|GetPlayerCharacter 0)) :!label _label
      (:Completed
        (Game|Damage|ApplyDamage OtherActor (Variables|Default|GetSwordDamage) 0 0)
        (Utilities|FlowControl|Delay 1.0)
        (goto _label Reset)))))

(event Custom|SwordActive
  ;[1 1 1] SwordCollisionを有効無効を切り替える.Animnotifyで使用するカスタムイベント
  (Collision|SetCollisionProfileName (Variables|Default|GetSwordCollision) "OverlapAll" true :!class /Script/Engine.PrimitiveComponent))

(event Custom|SwordDeactive
  ;[1 1 1] SwordCollisionを有効無効を切り替える.Animnotifyで使用するカスタムイベント
  (Collision|SetCollisionEnabled (Variables|Default|GetSwordCollision) "NoCollision"))

(event EventBeginPlay)

(event Collision|EventActorBeginOverlap
  (params (OtherActor :type Actor%20Object%20Reference)))

(event EventTick
  (params (DeltaSeconds :type Float%20%28single-precision%29)))

(fn ConstructionScript)