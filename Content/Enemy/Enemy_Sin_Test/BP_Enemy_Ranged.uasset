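; Ranged bow-wielding enemy character that supplies its own attack, movement speeds, combat ranges and damage handling.
; Attack plays the shoot-arrow montage, whose notifies tell the bow mechanics component to spawn and fire the arrow, then signals attack end on completion or interruption.
; Damage is forwarded to the damage system component.
; EquipWeapon is called at BeginPlay but is empty; weapon spawn/attach and line-of-sight trace logic are disconnected.
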(event EventBeginPlay
  (|CallParentFunction)
  (CallFunction|EquipWeapon))

(event EventEquipWeapon)

(event EventAttack
  (bind _notifyname (Animation|Montage|PlayMontage (Variables|Character|GetMesh) "/Game/Enemy/Enemy_Sin_Test/Resources/Archer/AM_ShootArrow.AM_ShootArrow")
    (:OnCompleted
      (Default|CallOnAttackEnd :!label _label))
    (:OnInterrupted
      (goto _label))
    (:OnNotifyBegin
      (switch name _notifyname
        (:DrawArrow
          (Default|SpawnArrow (Variables|Default|GetAC_BowMechanics)))
        (:Fire
          (Default|FireArrowBegin (Variables|Default|GetAC_BowMechanics)))))))

(fn ConstructionScript
  (|CallParentFunction))

(fn SetMovementSpeed
  (params (Speed :type E_EnemySpeed%20Enum :default "NewEnumerator0"))
  (bind _output_get (Variables|/Script/Engine.CharacterMovementComponent|SetMaxWalkSpeed (Variables|Character|GetCharacterMovement) (Utilities|Select :Index Speed :NewEnumerator0 0.0 :NewEnumerator1 2e+02 :NewEnumerator2 3e+02 :NewEnumerator3 5e+02)))
  (return _output_get))

(fn GetIdealRange
  (return 2e+03 2e+03))

(fn TakeDamage
  (params (DamageInfo :type S%20Damage%20Info%20Structure))
  (bind _wasdamaged (Default|TakeDamage (Variables|Default|GetBPC_DamageSystem) DamageInfo))
  (return _wasdamaged))