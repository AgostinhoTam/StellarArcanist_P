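; BP_EnemyTest is a test enemy character driven by AI_Controller_Sin, with a dagger and a magic attack montage.
; BeginPlay spawns the dagger, attaches it to a right-hand socket and signals that it is equipped.
; Attack plays the montage, signals its end, and on a notify line-traces from weapon to AI target, only printing a hit when unobstructed.
; Helper functions supply attack and defend ranges and handle movement speed by state.
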(event Collision|EventActorBeginOverlap
  (params (OtherActor :type Actor%20Object%20Reference))
  (|CallParentFunction OtherActor) ; このノードは無効になっているため呼び出せません。\n機能をビルドするにはピンをドラッグしてください。
)

(event EventTick
  (params (DeltaSeconds :type Float%20%28single-precision%29))
  (|CallParentFunction DeltaSeconds) ; このノードは無効になっているため呼び出せません。\n機能をビルドするにはピンをドラッグしてください。
)

(event EventEquipWeapon
  (bind _returnvalue (Game|SpawnActorfromClass "/Game/Enemy/Enemy_Sin_Test/Weapons/BP_Weapon_Dagger.BP_Weapon_Dagger_C" (Transformation|GetActorTransform) "Undefined" "MultiplyWithRoot" 0 0))
  (bind _output_get (Variables|Default|SetWeaponActor _returnvalue))
  (bind _returnvalue_2 (Transformation|AttachComponentToComponent _output_get (Variables|Character|GetMesh) "RHand_DaggerSocket" "SnapToTarget" "SnapToTarget" "SnapToTarget" true))
  (Variables|Default|SetisWieldingWeapon _returnvalue_2)
  (Default|CallOnWeaponEquipped))

(event EventAttack
  (bind _notifyname (Animation|Montage|PlayMontage (Variables|Character|GetMesh) "/Game/Characters/Mannequins/Animations/Manny/AddAnimationMontage/AM_MagicAttack.AM_MagicAttack")
    (:OnCompleted
      (Default|CallOnAttackEnd :!label _label))
    (:OnInterrupted
      (goto _label))
    (:OnNotifyBegin
      (switch name _notifyname
        (:Fire
          (bind _asai_controller_sin (Utilities|Casting|CastToAI_Controller_Sin (AI|GetAIController self)))
          (bind _attack_target (Variables|/Game/Enemy/Enemy_Sin_Test/AI_Controller_Sin.AI_Controller_Sin_C|GetAttack%20Target _asai_controller_sin)
            (:then
              (bind _returnvalue (Collision|LineTraceByChannel (Transformation|GetActorLocation (Variables|Default|GetWeaponActor)) (Transformation|GetActorLocation _attack_target) "TraceTypeQuery1" false 0 "ForDuration"))
              (if (not _returnvalue)
                (Development|PrintString "HitTarget")))
            (:else)))))))

(event EventBeginPlay
  (CallFunction|EquipWeapon))

(fn ConstructionScript
  (|CallParentFunction))

(fn SetMovementSpeed
  (params (Speed :type E_EnemySpeed%20Enum :default "NewEnumerator0"))
  (Variables|/Script/Engine.CharacterMovementComponent|SetMaxWalkSpeed (Variables|Character|GetCharacterMovement) 0.0)
  (return (Utilities|Select :Index Speed :NewEnumerator0 0.0 :NewEnumerator1 2e+02 :NewEnumerator2 3e+02 :NewEnumerator3 5e+02)))

(fn GetIdealRange
  (return 6e+02 6e+02))