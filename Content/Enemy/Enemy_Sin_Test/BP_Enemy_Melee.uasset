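; BP_Enemy_Melee is a sword-wielding melee enemy that handles attacking, drawing and sheathing its weapon.
; Attack plays a sword montage and signals attack end whether it completes or is interrupted.
; Equip and unequip montages use notifies to spawn and attach the sword to a hand socket or destroy it, updating the wielding flag.
; Both signal only on montage completion, so an interrupted equip or unequip sends no callback.
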(event EventBeginPlay
  (|CallParentFunction) ; このノードは無効になっているため呼び出せません。\n機能をビルドするにはピンをドラッグしてください。
)

(event Collision|EventActorBeginOverlap
  (params (OtherActor :type Actor%20Object%20Reference))
  (|CallParentFunction OtherActor) ; このノードは無効になっているため呼び出せません。\n機能をビルドするにはピンをドラッグしてください。
)

(event EventTick
  (params (DeltaSeconds :type Float%20%28single-precision%29))
  (|CallParentFunction DeltaSeconds) ; このノードは無効になっているため呼び出せません。\n機能をビルドするにはピンをドラッグしてください。
)

(event EventUnequipWeapon
  (bind _notifyname (Animation|Montage|PlayMontage (Variables|Character|GetMesh) "/Game/Enemy/Enemy_Sin_Test/Resources/AM_SheathSword.AM_SheathSword")
    (:OnCompleted
      (Default|CallOnWeaponUnequipped))
    (:OnNotifyBegin
      (switch name _notifyname
        (:DropSword
          (Actor|DestroyActor (Variables|Default|GetWeaponActor))
          (Variables|Default|SetisWieldingWeapon false))))))

(event EventEquipWeapon
  (bind _notifyname (Animation|Montage|PlayMontage (Variables|Character|GetMesh) "/Game/Enemy/Enemy_Sin_Test/Resources/AM_WieldSword.AM_WieldSword")
    (:OnCompleted
      (Default|CallOnWeaponEquipped))
    (:OnNotifyBegin
      (switch name _notifyname
        (:HoldSword
          (bind _returnvalue (Game|SpawnActorfromClass "/Game/Enemy/Enemy_Sin_Test/Weapons/BP_Weapon_Sword.BP_Weapon_Sword_C" (Transformation|GetActorTransform) "Undefined" "MultiplyWithRoot" 0 0))
          (Variables|Default|SetWeaponActor _returnvalue)
          (bind _returnvalue_2 (Transformation|AttachComponentToComponent _returnvalue (Variables|Character|GetMesh) "RHand_SwordSocket" "SnapToTarget" "SnapToTarget" "SnapToTarget" true))
          (Variables|Default|SetisWieldingWeapon _returnvalue_2))))))

(event EventAttack
  (Animation|Montage|PlayMontage (Variables|Character|GetMesh) "/Game/Enemy/Enemy_AlphaType/SwordAttack01.SwordAttack01"
    (:OnCompleted
      _)
    (:OnInterrupted
      _))
  (Default|CallOnAttackEnd))

(fn ConstructionScript
  (|CallParentFunction))