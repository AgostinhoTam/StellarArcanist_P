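; Base enemy character that delegates health, damage and healing to BPCDamageSystem and exposes patrol route, combat ranges and speed presets.
; Damage responses stop movement, play a hit montage and switch the AI controller from frozen back to attacking.
; Death ragdolls the mesh, stops AI logic, reports to the player's objective and BP_Colosseum, then destroys the actor after a delay.
; A health bar widget toggles by player distance, rechecked through a delayed Tick.
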(event Custom|Death
  (bind _mesh (Variables|Character|GetMesh))
  (bind _as_bp_third_person_character (Variables|Default|GetAs%20BP%20Third%20Person%20Character)
    (:then
      (Default|CallOnObjectiveIDCalled _as_bp_third_person_character (Variables|Default|GetObjectiveID) 1)
      (Physics|SetSimulatePhysics _mesh true)
      (Collision|SetCollisionEnabled _mesh "QueryAndPhysics")
      (Utilities|FlowControl|Sequence
        (:then_0
          (AI|Logic|StopLogic (Variables|/Script/AIModule.AIController|GetBrainComponent (AI|GetAIController self)) "")
          (Default|SetStateasDead (Variables|Default|GetAs%20AI%20Controller%20Sin))
          (Utilities|FlowControl|Delay 5.0)
          (Actor|DestroyActor))
        (:then_1
          (bind _colosseum (Variables|Default|GetColosseum)
            (:then
              (Default|EnemyCount _colosseum))
            (:else)))))
    (:else)))

(event Custom|Blocked
  (params (CanBeParried :type Boolean))
  (Development|PrintString "Blocked"))

(event Custom|DamageResponse
  (params (DamageRespoonse :type E_DamageResponse%20Enum :default "NewEnumerator0"))
  (Components|Movement|StopMovementImmediately (Variables|Character|GetCharacterMovement))
  (bind _as_ai_controller_sin (Variables|Default|GetAs%20AI%20Controller%20Sin)
    (:then
      (Default|SetStateasFrozen _as_ai_controller_sin)
      (Animation|Montage|PlayMontage (Variables|Character|GetMesh) (Variables|Default|GetHitReactionMontage)
        (:OnCompleted
          _)
        (:OnInterrupted
          _))
      (Default|SetStateasAttacking (Variables|Default|GetAs%20AI%20Controller%20Sin)))
    (:else)))

(event Custom|InitHpSettingEvent
  (if (>= 2.5e+03 (Math|Vector|Distance(Vector) (Transformation|GetActorLocation (Variables|Default|GetAs%20BP%20Third%20Person%20Character)) (Transformation|GetActorLocation)))
    (Rendering|SetVisibility (Variables|Default|GetWidget) true false)
    (else
      (Rendering|SetVisibility (Variables|Default|GetWidget) false false))))

(event EventBeginPlay
  (bind _bpc_damagesystem (Variables|Default|GetBPC_DamageSystem))
  (bind _asbp_third_person_character (Utilities|Casting|CastToBP_ThirdPersonCharacter (Game|GetPlayerCharacter 0)))
  (Variables|Default|SetAs%20BP%20Third%20Person%20Character _asbp_third_person_character)
  (Utilities|FlowControl|Sequence
    (:then_0
      (bind _returnvalue (UserInterface|CreateWidget "/Game/Enemy/Enemy_Sin_Test/Widget/WBP_UserHealthBar.WBP_UserHealthBar_C" 0 self))
      (UserInterface|SetWidget (Variables|Default|GetWidget) _returnvalue)
      (EventDispatchers|BindEventtoOnDeath _bpc_damagesystem (EventDispatchers|CreateEvent :!event Custom|Death))
      (EventDispatchers|BindEventtoOnBlock _bpc_damagesystem (EventDispatchers|CreateEvent :!event Custom|Blocked))
      (EventDispatchers|AssignOnDamageResponse _bpc_damagesystem (EventDispatchers|CreateEvent :!event Custom|DamageResponse))
      (bind _asai_controller_sin (Utilities|Casting|CastToAI_Controller_Sin (AI|GetAIController self)))
      (Variables|Default|SetAs%20AI%20Controller%20Sin _asai_controller_sin))
    (:then_1
      (CallFunction|InitHpSettingEvent))
    (:then_2
      (Utilities|FlowControl|Delay 0.2)
      (Variables|Default|GetColosseum
        (:then)
        (:else
          (bind _returnvalue_2 (Actor|GetActorOfClass "/Game/BluePrints/BP_Colosseum.BP_Colosseum_C"))
          (if (Utilities|IsValid _returnvalue_2)
            (bind _output_get (Variables|Default|SetColosseum _returnvalue_2))
            (Default|AddEnemy _output_get)))))))

(event EventEquipWeapon)

(event EventTick
  (params (DeltaSeconds :type Float%20%28single-precision%29))
  (Utilities|FlowControl|Delay 2.0)
  (if (>= 2.5e+03 (Math|Vector|Distance(Vector) (Transformation|GetActorLocation (Variables|Default|GetAs%20BP%20Third%20Person%20Character)) (Transformation|GetActorLocation)))
    (Rendering|SetVisibility (Variables|Default|GetWidget) true false)
    (else
      (Rendering|SetVisibility (Variables|Default|GetWidget) false false))))

(fn ConstructionScript)

(fn GetCurrentHealth
  (return (Variables|/Game/DamageSystem/BPC_DamageSystem.BPC_DamageSystem_C|GetHealth (Variables|Default|GetBPC_DamageSystem))))

(fn GetIdealRange
  (return 1.5e+02 3.5e+02))

(fn GetMaxHealth
  (return (Variables|/Game/DamageSystem/BPC_DamageSystem.BPC_DamageSystem_C|GetMaxHealth (Variables|Default|GetBPC_DamageSystem))))

(fn GetPatrolRoute
  (return (Variables|AI|GetPatrolRoute)))

(fn Heal
  (params (Heal :type Float%20%28double-precision%29))
  (bind _newhealth (Default|Heal (Variables|Default|GetBPC_DamageSystem) Heal))
  (return _newhealth))

(fn IsDead
  (return (Variables|/Game/DamageSystem/BPC_DamageSystem.BPC_DamageSystem_C|GetIsDead (Variables|Default|GetBPC_DamageSystem))))

(fn SetInitializeHP
  (return (Variables|/Game/DamageSystem/BPC_DamageSystem.BPC_DamageSystem_C|GetMaxHealth (Variables|Default|GetBPC_DamageSystem))))

(fn SetMovementSpeed
  (params (Speed :type E_EnemySpeed%20Enum :default "NewEnumerator0"))
  (bind _output_get (Variables|/Script/Engine.CharacterMovementComponent|SetMaxWalkSpeed (Variables|Character|GetCharacterMovement) (Utilities|Select :Index Speed :NewEnumerator0 0.0 :NewEnumerator1 1e+02 :NewEnumerator2 3e+02 :NewEnumerator3 5e+02)))
  (return _output_get))

(fn TakeDamage
  (params (DamageInfo :type S%20Damage%20Info%20Structure))
  (bind _wasdamaged (Default|TakeDamage (Variables|Default|GetBPC_DamageSystem) DamageInfo))
  (return _wasdamaged))