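; Magic-casting enemy with a long-range attack, a quicker close-range attack and a spawn sequence.
; Montage notifies time each action: both attacks launch fireballs through ACFireBall and place BP_MagicCircle near ground level, while the spawn montage triggers its own actor spawns.
; Overlapping the player calls ApplyDamage on the enemy itself.
; TakeDamage delegates to BPCDamageSystem, alongside functions supplying combat ranges and setting walk speed by movement state.
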(event OnComponentBeginOverlap(CapsuleComponent)
  (params (OverlappedComponent :type Primitive%20Component%20Object%20Reference) (OtherActor :type Actor%20Object%20Reference) (OtherComp :type Primitive%20Component%20Object%20Reference) (OtherBodyIndex :type Integer) (bFromSweep :type Boolean) (SweepResult :type Hit%20Result%20Structure%20%28by%20ref%29))
  ;[1 1 1] ダメージ
  (Utilities|Casting|CastToBP_ThirdPersonCharacter OtherActor)
  (Game|Damage|ApplyDamage self 0.0 0 0))

(event Custom|MagicAttack1
  (bind _returnvalue (Transformation|GetActorTransform))
  ;[1 1 1] 遠距離攻撃
  (bind _notifyname (Animation|Montage|PlayMontage (Variables|Character|GetMesh) "/Game/Enemy/MagicEnemy/Animation/Animation_Montage/AnimM_MagicAttack.AnimM_MagicAttack")
    (:OnNotifyBegin
      (switch name _notifyname
        (:FireBall
          (Default|SpawnFireBall (Variables|Default|GetAC_FireBall)))
        (:Circle
          (Game|SpawnActorfromClass "/Game/Enemy/MagicEnemy/BluePrints/BP_MagicCircle.BP_MagicCircle_C" (Math|Transform|MakeTransform (Math|Vector|MakeVector (.x (.location _returnvalue)) (.y (.location _returnvalue)) -0.01) (.rotation _returnvalue) (.scale _returnvalue)) "Undefined" "MultiplyWithRoot" 0 0))))))

(event Custom|MagicAttack2
  (bind _returnvalue (Transformation|GetActorTransform))
  ;[1 1 1] 近距離攻撃
  (bind _notifyname (Animation|Montage|PlayMontage (Variables|Character|GetMesh) "/Game/Enemy/MagicEnemy/Animation/Animation_Montage/AnimM_QuickMagicAttack.AnimM_QuickMagicAttack")
    (:OnNotifyBegin
      (switch name _notifyname
        (:FireBall
          (Default|SpawnFireBall (Variables|Default|GetAC_FireBall)))
        (:Circle
          (Game|SpawnActorfromClass "/Game/Enemy/MagicEnemy/BluePrints/BP_MagicCircle.BP_MagicCircle_C" (Math|Transform|MakeTransform (Math|Vector|MakeVector (.x (.location _returnvalue)) (.y (.location _returnvalue)) -0.01) (.rotation _returnvalue) (.scale _returnvalue)) "Undefined" "MultiplyWithRoot" 0 0))))))

(event Custom|EnemySpawn
  (bind _returnvalue (Transformation|GetActorTransform))
  (bind _returnvalue_2 (Transformation|GetActorTransform))
  (bind _notifyname (Animation|Montage|PlayMontage (Variables|Character|GetMesh) "/Game/Enemy/MagicEnemy/Animation/Animation_Montage/AnimM_Spawn.AnimM_Spawn")
    (:OnNotifyBegin
      (switch name _notifyname
        (:Spawn
          (Game|SpawnActorfromClass "/Game/Enemy/MagicEnemy/BluePrints/BP_SpawnArea.BP_SpawnArea_C" (Math|Transform|MakeTransform (Math|Vector|MakeVector (.x (.location _returnvalue)) (.y (.location _returnvalue)) 5e+01) (.rotation _returnvalue) (.scale _returnvalue)) "Undefined" "MultiplyWithRoot" 0 0))
        (:Circle
          (Game|SpawnActorfromClass "/Game/Enemy/MagicEnemy/BluePrints/BP_MagicCircle.BP_MagicCircle_C" (Math|Transform|MakeTransform (Math|Vector|MakeVector (.x (.location _returnvalue_2)) (.y (.location _returnvalue_2)) -0.01) (.rotation _returnvalue_2) (.scale _returnvalue_2)) "Undefined" "MultiplyWithRoot" 0 0))))))

(event EventBeginPlay
  (|CallParentFunction))

(fn ConstructionScript
  (|CallParentFunction))

(fn TakeDamage
  (params (DamageInfo :type S%20Damage%20Info%20Structure))
  (bind _wasdamaged (Default|TakeDamage (Variables|Default|GetBPC_DamageSystem) DamageInfo))
  (return _wasdamaged))

(fn GetIdealRange
  (return 2e+03 2e+03))

(fn SetMovementSpeed
  (params (Speed :type E_EnemySpeed%20Enum :default "NewEnumerator0"))
  (bind _output_get (Variables|/Script/Engine.CharacterMovementComponent|SetMaxWalkSpeed (Variables|Character|GetCharacterMovement) (Utilities|Select :Index Speed :NewEnumerator0 0.0 :NewEnumerator1 2e+02 :NewEnumerator2 3e+02 :NewEnumerator3 5e+02)))
  (return _output_get))