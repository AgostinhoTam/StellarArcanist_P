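; Actor component for the magic enemy that manages a spawn area actor used to spawn enemies.
; It caches its owning base enemy, spawns a BP_SpawnArea attached to a mesh socket, and can destroy it.
; SpawnBegin detaches the area and, if the AI controller has a valid attack target, triggers its enemy spawn.
; A visibility trace toward that target runs first, but its result is unused.
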(event Custom|Spawn%20Begin
  (bind _spawnarea_ref (Variables|Default|GetSpawnArea%20Ref)
    (:then
      (Transformation|DetachFromActor _spawnarea_ref "KeepRelative" "KeepRelative" "KeepRelative")
      (bind _asbp_magic_enemy_ai (Utilities|Casting|CastToBP_MagicEnemy_AI (AI|GetAIController (Variables|Default|GetCharactor%20Ref))))
      (bind _attacktarget (Variables|/Game/Enemy/MagicEnemy/BP_MagicEnemy_AI.BP_MagicEnemy_AI_C|GetAttackTarget _asbp_magic_enemy_ai)
        (:then
          (Collision|LineTraceByChannel (Transformation|GetActorLocation (Variables|Default|GetSpawnArea%20Ref)) (Transformation|GetActorLocation _attacktarget) "TraceTypeQuery1" false 0 "None")
          (Default|SpawnEnemy (Variables|Default|GetSpawnArea%20Ref)))
        (:else)))
    (:else)))

(event EventBeginPlay
  (bind _asbp_enemy_base (Utilities|Casting|CastToBP_Enemy_Base (Components|GetOwner)))
  (Variables|Default|SetCharactor%20Ref _asbp_enemy_base))

(fn SpawnSpawnArea
  (bind _returnvalue (Game|SpawnActorfromClass "/Game/Enemy/MagicEnemy/BluePrints/BP_SpawnArea.BP_SpawnArea_C" (Math|Transform|MakeTransform "0.000000,0.000000,500.000000" (Transformation|GetActorRotation (Variables|Default|GetCharactor%20Ref)) "1.000000,1.000000,1.000000") "Undefined" "MultiplyWithRoot" 0 0))
  (bind _output_get (Variables|Default|SetSpawnArea%20Ref _returnvalue))
  (Transformation|AttachComponentToComponent _output_get (Variables|/Script/Engine.Character|GetMesh (Variables|Default|GetCharactor%20Ref)) (Variables|Default|GetSpawnArea%20socketname) "KeepRelative" "KeepRelative" "KeepRelative" true))

(fn DestroySpawnArea
  (bind _spawnarea_ref (Variables|Default|GetSpawnArea%20Ref)
    (:then
      (Actor|DestroyActor _spawnarea_ref))
    (:else)))