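; BP_SpawnArea is a spawn volume that populates itself with three BP_MagicEnemy AI pawns, running BT_SpawnEnemy, at BeginPlay.
; Each spawns at a random point inside the Box component's bounds, copying the player character's rotation.
; Failed spawns retry at new points until a shared MissCount reaches its limit of 50, which resets the counter and abandons that enemy.
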(event EventBeginPlay
  (bind _box (Variables|Default|GetBox))
  (bind (_origin _boxextent) (Collision|GetComponentBounds _box))
  (for _index (range 0 2)
    (bind _returnvalue (AI|SpawnAIFromClass "/Game/Enemy/MagicEnemy/BP_MagicEnemy.BP_MagicEnemy_C" "/Game/Enemy/MagicEnemy/BehaviorTree/BT_SpawnEnemy.BT_SpawnEnemy" (Math|Random|RandomPointinBoundingBox _origin _boxextent) (Transformation|GetActorRotation (Game|GetPlayerCharacter 0)) false 0 :!label _label))
    (Utilities|IsValid _returnvalue
      (:Is%20Not%20Valid
        (bind _result (Math|Integer|IncrementInt (Variables|Default|GetMissCount))
          (:%20%20
            (if (not (>= _result 50))
              (goto _label)
              (else
                (Variables|Default|SetMissCount 0)))))))))

(event Collision|EventActorBeginOverlap
  (params (OtherActor :type Actor%20Object%20Reference))
  (|CallParentFunction OtherActor) ; このノードは無効になっているため呼び出せません。\n機能をビルドするにはピンをドラッグしてください。
)

(event EventTick
  (params (DeltaSeconds :type Float%20%28single-precision%29))
  (|CallParentFunction DeltaSeconds) ; このノードは無効になっているため呼び出せません。\n機能をビルドするにはピンをドラッグしてください。
)

(fn ConstructionScript)