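; AC_FireBall is an actor component that manages the fireball attack of BP_MagicEnemy.
; SpawnFireBall creates a stationary BP_Projectile_FireBall attached to a socket on the enemy's mesh, and DestroyFireBall removes it.
; FireBallBegin detaches the projectile and launches it toward the AI controller's AttackTarget along a unit direction vector.
; A visibility line trace runs before launch, but its result is unused.
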(event Custom|FireBallBegin
  (bind _fireballref (Variables|Default|GetFireBallRef))
  (bind _returnvalue (Transformation|GetActorLocation _fireballref))
  (bind _fireballref_2 (Variables|Default|GetFireBallRef)
    (:then
      (Transformation|DetachFromActor _fireballref_2 "KeepRelative" "KeepRelative" "KeepRelative")
      (bind _asbp_magic_enemy_ai (Utilities|Casting|CastToBP_MagicEnemy_AI (AI|GetAIController (Variables|Default|GetCharactor%20Ref))))
      (bind _attacktarget (Variables|/Game/Enemy/MagicEnemy/BP_MagicEnemy_AI.BP_MagicEnemy_AI_C|GetAttackTarget _asbp_magic_enemy_ai)
        (:then
          (Collision|LineTraceByChannel _returnvalue (Transformation|GetActorLocation _attacktarget) "TraceTypeQuery1" false 0 "None")
          (Default|FireBall (Variables|Default|GetFireBallRef) (Math|Vector|GetUnitDirection(Vector) _returnvalue (Transformation|GetActorLocation _attacktarget))))
        (:else)))
    (:else)))

(event EventBeginPlay
  (bind _asbp_magic_enemy (Utilities|Casting|CastToBP_MagicEnemy (Components|GetOwner)))
  (Variables|Default|SetCharactor%20Ref _asbp_magic_enemy))

(fn SpawnFireBall
  (bind _returnvalue (Game|SpawnActorfromClass "/Game/Enemy/MagicEnemy/BP_Projectile_FireBall.BP_Projectile_FireBall_C" (Math|Transform|MakeTransform "0, 0, 0" "0, 0, 0" "1.000000,1.000000,1.000000") "Undefined" "MultiplyWithRoot" 0 0.0 0.0 0))
  (bind _output_get (Variables|Default|SetFireBallRef _returnvalue))
  (Transformation|AttachComponentToComponent _output_get (Variables|/Script/Engine.Character|GetMesh (Variables|Default|GetCharactor%20Ref)) (Variables|Default|GetFireBall%20socket%20Name) "KeepRelative" "KeepRelative" "KeepRelative" true))

(fn DestroyFireBall
  (bind _fireballref (Variables|Default|GetFireBallRef)
    (:then
      (Actor|DestroyActor _fireballref))
    (:else)))