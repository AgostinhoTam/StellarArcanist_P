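; Prototype enemy AI controller that tracks the player through AI perception.
; On BeginPlay it runs the prototype enemy behavior tree.
; Perception updates for the first player character write it to the TargetActor blackboard key when sensed and clear the key when sensing is lost, ignoring all other actors.
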(event OnTargetPerceptionUpdated(AIPerception)
  (params (Actor :type Actor%20Object%20Reference) (Stimulus :type AI%20Stimulus%20Structure))
  (if (== Actor (Game|GetPlayerCharacter 0))
    (if (.bSuccessfullySensed (Utilities|Struct|BreakAIStimulus Stimulus))
      (AI|Components|Blackboard|SetValueasObject (Variables|Default|GetBlackboard) (Utilities|Name|MakeLiteralName "TargetActor") Actor)
      (else
        (AI|Components|Blackboard|SetValueasObject (Variables|Default|GetBlackboard) (Utilities|Name|MakeLiteralName "TargetActor") 0)))))

(event EventBeginPlay
  (AI|RunBehaviorTree "/Game/Enemy/BT_Enemy_Prototype.BT_Enemy_Prototype"))

(fn ConstructionScript
  (|CallParentFunction))