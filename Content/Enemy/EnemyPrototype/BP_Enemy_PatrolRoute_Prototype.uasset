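; Prototype enemy patrol route actor that serves world-space waypoints from the PatrolRoute spline.
; GetSplinePointAsWorldPosition returns the location of the spline point at PointIndex.
; ImcrementPatrolRoute steps PointIndex by Direction, then sets Direction to -1 at the last point.
; Every other point resets Direction to 1 through an always-true branch, so the index oscillates between the final two points instead of returning to the start.
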(event Custom|ImcrementPatrolRoute
  ;[1 1 1] パtpロールポイントの増減
  (bind _output_get (Variables|Default|SetPointIndex (+ (Variables|Default|GetPointIndex) (Variables|Default|GetDirection))))
  (if (== _output_get (- (Spline|GetNumberOfSplinePoints (Variables|Default|GetPatrolRoute)) 1))
    (Variables|Default|SetDirection -1)
    (elif true
      (Variables|Default|SetDirection 1))))

(fn ConstructionScript)

(fn GetSplinePointasWorldPosition
  ;[1 1 1] ルートの取得
  (return (Spline|GetLocationatSplinePoint (Variables|Default|GetPatrolRoute) (Variables|Default|GetPointIndex) "World")))