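; Test Mountain Dragon enemy creature that attacks with melee montages or fire and supplies range, speed and damage functions.
; Attack uses cascading random rolls to pick one of three claw/bite montages, falling through to a fire montage most often.
; Melee notifies sphere-trace low and forward to deal blockable, parryable damage to BP_ThirdPersonCharacter; fire notifies drive ACFireBallMechanics and toggle a particle.
; Montage completion or interruption signals attack end; incoming damage goes to BPCDamageSystem, while IsDead always returns false.
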(event EventBeginPlay
  (|CallParentFunction))

(event Collision|EventActorBeginOverlap
  (params (OtherActor :type Actor%20Object%20Reference))
  (|CallParentFunction OtherActor))

(event EventTick
  (params (DeltaSeconds :type Float%20%28single-precision%29))
  (|CallParentFunction DeltaSeconds))

(event EventAttack
  (bind _returnvalue (Transformation|GetActorLocation))
  (bind _returnvalue_2 (Transformation|GetActorLocation))
  (bind _returnvalue_3 (Transformation|GetActorLocation))
  (bind _returnvalue_4 (- (.z _returnvalue_2) 2e+02))
  (bind _returnvalue_5 (- (.z _returnvalue_3) 2e+02))
  (bind _returnvalue_6 (- (.z _returnvalue) 2e+02))
  (if (> (Math|Random|RandomInteger 100) 75)
    (bind _notifyname (Animation|Montage|PlayMontage (Variables|Character|GetMesh) "/Game/QuadrapedCreatures/MountainDragon/AM_Dragon_Attack01.AM_Dragon_Attack01")
      (:OnCompleted
        (Default|CallOnAttackEnd :!label _label))
      (:OnInterrupted
        (goto _label))
      (:OnNotifyBegin
        (switch name _notifyname
          (:Claw01
            _)
          (:Claw02
            _))
        (bind (_outhit _returnvalue_7) (Collision|SphereTraceForObjects (Math|Vector|MakeVector (.x _returnvalue_3) (.y _returnvalue_3) _returnvalue_5) (+ (Math|Vector|MakeVector (.x _returnvalue_3) (.y _returnvalue_3) _returnvalue_5) (* (Transformation|GetActorForwardVector) 3.5e+02)) 1e+02 (Utilities|Array|MakeArray "ObjectTypeQuery3") false 0 "ForDuration"))
        (if _returnvalue_7
          (bind _asbp_third_person_character (Utilities|Casting|CastToBP_ThirdPersonCharacter (.HitActor (Collision|BreakHitResult _outhit))))
          (Default|TakeDamage (Variables|/Game/ThirdPerson/Blueprints/BP_ThirdPersonCharacter.BP_ThirdPersonCharacter_C|GetBPC_DamageSystem _asbp_third_person_character) (Utilities|Struct|MakeS_DamageInfo 1e+01 "NewEnumerator0" "NewEnumerator0" false true true false)))))
    (elif (> (Math|Random|RandomInteger 100) 75)
      (bind _notifyname_2 (Animation|Montage|PlayMontage (Variables|Character|GetMesh) "/Game/QuadrapedCreatures/MountainDragon/AM_Dragon_Attack02.AM_Dragon_Attack02")
        (:OnCompleted
          (Default|CallOnAttackEnd :!label _label_2))
        (:OnInterrupted
          (goto _label_2))
        (:OnNotifyBegin
          (switch name _notifyname_2
            (:Bite
              _)
            (:Claw02
              _))
          (bind (_outhit_2 _returnvalue_8) (Collision|SphereTraceForObjects (Math|Vector|MakeVector (.x _returnvalue) (.y _returnvalue) _returnvalue_6) (+ (Math|Vector|MakeVector (.x _returnvalue) (.y _returnvalue) _returnvalue_6) (* (Transformation|GetActorForwardVector) 3.5e+02)) 1e+02 (Utilities|Array|MakeArray "ObjectTypeQuery3") false 0 "ForDuration"))
          (if _returnvalue_8
            (bind _asbp_third_person_character_2 (Utilities|Casting|CastToBP_ThirdPersonCharacter (.HitActor (Collision|BreakHitResult _outhit_2))))
            (Default|TakeDamage (Variables|/Game/ThirdPerson/Blueprints/BP_ThirdPersonCharacter.BP_ThirdPersonCharacter_C|GetBPC_DamageSystem _asbp_third_person_character_2) (Utilities|Struct|MakeS_DamageInfo 1e+01 "NewEnumerator0" "NewEnumerator0" false true true false)))))
      (elif (> (Math|Random|RandomInteger 100) 75)
        (bind _notifyname_3 (Animation|Montage|PlayMontage (Variables|Character|GetMesh) "/Game/QuadrapedCreatures/MountainDragon/AM_Dragon_Attack04.AM_Dragon_Attack04")
          (:OnCompleted
            (Default|CallOnAttackEnd :!label _label_3))
          (:OnInterrupted
            (goto _label_3))
          (:OnNotifyBegin
            (switch name _notifyname_3
              (:Bite
                _)
              (:Claw01
                _)
              (:Claw02
                _))
            (bind (_outhit_3 _returnvalue_9) (Collision|SphereTraceForObjects (Math|Vector|MakeVector (.x _returnvalue_2) (.y _returnvalue_2) _returnvalue_4) (+ (Math|Vector|MakeVector (.x _returnvalue_2) (.y _returnvalue_2) _returnvalue_4) (* (Transformation|GetActorForwardVector) 3.5e+02)) 1e+02 (Utilities|Array|MakeArray "ObjectTypeQuery3") false 0 "ForDuration"))
            (if _returnvalue_9
              (bind _asbp_third_person_character_3 (Utilities|Casting|CastToBP_ThirdPersonCharacter (.HitActor (Collision|BreakHitResult _outhit_3))))
              (Default|TakeDamage (Variables|/Game/ThirdPerson/Blueprints/BP_ThirdPersonCharacter.BP_ThirdPersonCharacter_C|GetBPC_DamageSystem _asbp_third_person_character_3) (Utilities|Struct|MakeS_DamageInfo 1e+01 "NewEnumerator0" "NewEnumerator0" false true true false)))))
        (else
          (bind _notifyname_4 (Animation|Montage|PlayMontage (Variables|Character|GetMesh) "/Game/QuadrapedCreatures/MountainDragon/AM_Dragon_Attack_03.AM_Dragon_Attack_03")
            (:OnCompleted
              (Default|CallOnAttackEnd :!label _label_4))
            (:OnInterrupted
              (goto _label_4))
            (:OnNotifyBegin
              (switch name _notifyname_4
                (:FireBigin
                  (Default|SpawnFire (Variables|Default|GetAC_FireBallMechanics)))
                (:Fire01
                  (Default|FireArrowBegin (Variables|Default|GetAC_FireBallMechanics))
                  (Rendering|ToggleVisibility (Variables|Default|GetParticleSystem) false))
                (:Bigin
                  (Rendering|ToggleVisibility (Variables|Default|GetParticleSystem) false))))))))))

(fn ConstructionScript
  (|CallParentFunction))

(fn IsDead
  (return false))

(fn TakeDamage
  (params (DamageInfo :type S%20Damage%20Info%20Structure))
  (bind _wasdamaged (Default|TakeDamage (Variables|Default|GetBPC_DamageSystem) DamageInfo))
  (return _wasdamaged))

(fn GetIdealRange
  (return 5e+02 2e+03))

(fn SetMovementSpeed
  (params (Speed :type E_EnemySpeed%20Enum :default "NewEnumerator0"))
  (bind _output_get (Variables|/Script/Engine.CharacterMovementComponent|SetMaxWalkSpeed (Variables|Character|GetCharacterMovement) (Utilities|Select :Index Speed :NewEnumerator0 0.0 :NewEnumerator1 2e+02 :NewEnumerator2 3e+02 :NewEnumerator3 5e+02)))
  (return _output_get))