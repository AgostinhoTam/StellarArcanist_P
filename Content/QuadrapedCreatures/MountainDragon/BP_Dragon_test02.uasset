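; Test dragon creature Blueprint that performs melee attacks on the third-person player and takes damage through a damage-system component.
; Attack randomly picks between Attack01 (used by two branches) and Attack04 montages, then signals attack end on completion or interruption.
; Montage notifies trigger a short forward sphere trace that deals blockable, parryable damage to the player.
; TakeDamage forwards to the component, while IsDead always returns false.
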(event EventBeginPlay
  (|CallParentFunction))

(event Collision|EventActorBeginOverlap
  (params (OtherActor :type Actor%20Object%20Reference))
  (|CallParentFunction OtherActor))

(event EventTick
  (params (DeltaSeconds :type Float%20%28single-precision%29))
  (|CallParentFunction DeltaSeconds))

(event EventAttack
  (bind _returnvalue (Transformation|GetActorLocation))
  (bind _returnvalue_2 (Transformation|GetActorLocation))
  (bind _returnvalue_3 (Transformation|GetActorLocation))
  (if (> (Math|Random|RandomInteger 10) 6)
    (bind _notifyname (Animation|Montage|PlayMontage (Variables|Character|GetMesh) "/Game/QuadrapedCreatures/MountainDragon/AM_Dragon_Attack01.AM_Dragon_Attack01")
      (:OnCompleted
        (Default|CallOnAttackEnd :!label _label))
      (:OnInterrupted
        (goto _label))
      (:OnNotifyBegin
        (switch name _notifyname
          (:Claw01
            (bind (_outhit _returnvalue_4) (Collision|SphereTraceForObjects _returnvalue_3 (+ _returnvalue_3 (* (Transformation|GetActorForwardVector) 2e+02)) 0.0 (Utilities|Array|MakeArray "ObjectTypeQuery3") false 0 "None"))
            (if _returnvalue_4
              (bind _asbp_third_person_character (Utilities|Casting|CastToBP_ThirdPersonCharacter (.HitActor (Collision|BreakHitResult _outhit))))
              (Default|TakeDamage (Variables|/Game/ThirdPerson/Blueprints/BP_ThirdPersonCharacter.BP_ThirdPersonCharacter_C|GetBPC_DamageSystem _asbp_third_person_character) (Utilities|Struct|MakeS_DamageInfo 1e+01 "NewEnumerator0" "NewEnumerator0" false true true false)))))))
    (elif (> (Math|Random|RandomInteger 10) 6)
      (bind _notifyname_2 (Animation|Montage|PlayMontage (Variables|Character|GetMesh) "/Game/QuadrapedCreatures/MountainDragon/AM_Dragon_Attack01.AM_Dragon_Attack01")
        (:OnCompleted
          (Default|CallOnAttackEnd :!label _label_2))
        (:OnInterrupted
          (goto _label_2))
        (:OnNotifyBegin
          (switch name _notifyname_2
            (:Bite
              _)
            (:Claw02
              _))
          (bind (_outhit_2 _returnvalue_5) (Collision|SphereTraceForObjects _returnvalue (+ _returnvalue (* (Transformation|GetActorForwardVector) 2e+02)) 0.0 (Utilities|Array|MakeArray "ObjectTypeQuery3") false 0 "None"))
          (if _returnvalue_5
            (bind _asbp_third_person_character_2 (Utilities|Casting|CastToBP_ThirdPersonCharacter (.HitActor (Collision|BreakHitResult _outhit_2))))
            (Default|TakeDamage (Variables|/Game/ThirdPerson/Blueprints/BP_ThirdPersonCharacter.BP_ThirdPersonCharacter_C|GetBPC_DamageSystem _asbp_third_person_character_2) (Utilities|Struct|MakeS_DamageInfo 1e+01 "NewEnumerator0" "NewEnumerator0" false true true false)))))
      (else
        (bind _notifyname_3 (Animation|Montage|PlayMontage (Variables|Character|GetMesh) "/Game/QuadrapedCreatures/MountainDragon/AM_Dragon_Attack04.AM_Dragon_Attack04")
          (:OnCompleted
            (Default|CallOnAttackEnd :!label _label_3))
          (:OnInterrupted
            (goto _label_3))
          (:OnNotifyBegin
            (switch name _notifyname_3
              (:Bite
                _)
              (:Claw01
                _)
              (:Claw02
                _))
            (bind (_outhit_3 _returnvalue_6) (Collision|SphereTraceForObjects _returnvalue_2 (+ _returnvalue_2 (* (Transformation|GetActorForwardVector) 2e+02)) 0.0 (Utilities|Array|MakeArray "ObjectTypeQuery3") false 0 "None"))
            (if _returnvalue_6
              (bind _asbp_third_person_character_3 (Utilities|Casting|CastToBP_ThirdPersonCharacter (.HitActor (Collision|BreakHitResult _outhit_3))))
              (Default|TakeDamage (Variables|/Game/ThirdPerson/Blueprints/BP_ThirdPersonCharacter.BP_ThirdPersonCharacter_C|GetBPC_DamageSystem _asbp_third_person_character_3) (Utilities|Struct|MakeS_DamageInfo 1e+01 "NewEnumerator0" "NewEnumerator0" false true true false)))))))))

(fn ConstructionScript
  (|CallParentFunction))

(fn TakeDamage
  (params (DamageInfo :type S%20Damage%20Info%20Structure))
  (bind _wasdamaged (Default|TakeDamage (Variables|Default|GetBPC_DamageSystem) DamageInfo))
  (return _wasdamaged))

(fn IsDead
  (return false))