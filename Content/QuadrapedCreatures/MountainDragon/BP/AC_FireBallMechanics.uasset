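; Actor component that handles the fireball attack of the mountain dragon (BP_Dragon_Test).
; SpawnFire creates a BP_Dragon_FireBall attached to a socket on the dragon's mesh, and DestroyFire removes it.
; FireArrowBegin detaches the fireball and launches it toward the AttackTarget held by the dragon's AI controller.
; A visibility line trace runs before launch, but its result is unused.
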(event Custom|FireArrowBegin
  (bind _fireref (Variables|Default|GetFireRef))
  (bind _returnvalue (Transformation|GetActorLocation _fireref))
  (bind _fireref_2 (Variables|Default|GetFireRef)
    (:then
      (Transformation|DetachFromActor _fireref_2 "KeepWorld" "KeepWorld" "KeepWorld")
      (bind _asai_controller_dragon (Utilities|Casting|CastToAI_Controller_Dragon (AI|GetAIController (Variables|Default|GetCharacterRef))))
      (bind _attack_target (Variables|/Game/QuadrapedCreatures/MountainDragon/AI/AI_Controller_Dragon.AI_Controller_Dragon_C|GetAttack%20Target _asai_controller_dragon)
        (:then
          (Collision|LineTraceByChannel _returnvalue (Transformation|GetActorLocation _attack_target) "TraceTypeQuery1" false 0 "None")
          (Default|Fire (Variables|Default|GetFireRef) (Math|Vector|GetUnitDirection(Vector) _returnvalue (Transformation|GetActorLocation _attack_target))))
        (:else)))
    (:else)))

(event EventBeginPlay
  (bind _asbp_dragon_test (Utilities|Casting|CastToBP_Dragon_Test (Components|GetOwner)))
  (Variables|Default|SetCharacterRef _asbp_dragon_test))

(fn SpawnFire
  (bind _returnvalue (Game|SpawnActorfromClass "/Game/QuadrapedCreatures/MountainDragon/BP/BP_Dragon_FireBall.BP_Dragon_FireBall_C" (Math|Transform|MakeTransform "0, 0, 0" (Transformation|GetActorRotation (Variables|Default|GetCharacterRef)) "1.000000,1.000000,1.000000") "Undefined" "MultiplyWithRoot" 0 0.0 0.0 0))
  (bind _output_get (Variables|Default|SetFireRef _returnvalue))
  (Transformation|AttachComponentToComponent _output_get (Variables|/Script/Engine.Character|GetMesh (Variables|Default|GetCharacterRef)) (Variables|Default|GetFireBollSocketName) "SnapToTarget" "SnapToTarget" "SnapToTarget" true))

(fn DestroyFire
  (bind _fireref (Variables|Default|GetFireRef)
    (:then
      (Actor|DestroyActor _fireref))
    (:else)))