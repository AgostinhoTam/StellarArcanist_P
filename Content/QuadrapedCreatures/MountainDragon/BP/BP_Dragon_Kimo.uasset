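; Mountain dragon enemy character that fights with water ball, blade and pillar attacks.
; Attack randomly picks montages, switching to airborne volleys and two-claw blades once Tick sees health at or below half.
; Montage notifies drive ACWaterBallMechanics or spawn a pillar at the player's location, and montage end calls OnAttackEnd.
; CreateField spawns a single BP_Field, removed by IsDead; an older sphere-trace attack chain remains disconnected.
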(event Custom|CreateField
  (bind _returnvalue (Transformation|GetActorLocation))
  (bind _returnvalue_2 (Transformation|GetActorScale3D))
  ;[1 1 1] DOKUMUMA★
  (Variables|Default|GetField
    (:then
      (Default|CallOnAttackEnd :!label _label))
    (:else
      (bind _notifyname (Animation|Montage|PlayMontage (Variables|Character|GetMesh) "/Game/QuadrapedCreatures/MountainDragon/AM/AM_Dragon_Attack_03.AM_Dragon_Attack_03")
        (:OnCompleted
          (goto _label))
        (:OnInterrupted
          (goto _label))
        (:OnNotifyBegin
          (switch name _notifyname
            (:Fire01
              (bind _returnvalue_3 (Game|SpawnActorfromClass "/Game/QuadrapedCreatures/MountainDragon/BP/BP_Field.BP_Field_C" (Math|Transform|MakeTransform (Math|Vector|MakeVector (.x _returnvalue) (.y _returnvalue) (.z _returnvalue)) "0, 0, 0" (Math|Vector|MakeVector (* (.x _returnvalue_2) 4.0) (* (.y _returnvalue_2) 4.0) 1.0)) "Undefined" "MultiplyWithRoot" 0 0))
              (Variables|Default|SetField _returnvalue_3))))))))

(event EventBeginPlay
  (|CallParentFunction))

(event Collision|EventActorBeginOverlap
  (params (OtherActor :type Actor%20Object%20Reference))
  (|CallParentFunction OtherActor))

(event EventTick
  (params (DeltaSeconds :type Float%20%28single-precision%29))
  (bind _bpc_damagesystem (Variables|Default|GetBPC_DamageSystem))
  (|CallParentFunction DeltaSeconds)
  (CallFunction|GetCurrentHealth)
  (if (<= (/ (Variables|/Game/DamageSystem/BPC_DamageSystem.BPC_DamageSystem_C|GetHealth _bpc_damagesystem) (Variables|/Game/DamageSystem/BPC_DamageSystem.BPC_DamageSystem_C|GetMaxHealth _bpc_damagesystem)) 0.5)
    (Variables|Default|SetUnder50 true)))

(event EventAttack
  (bind _returnvalue (Transformation|GetActorScale3D))
  (bind _returnvalue_2 (Transformation|GetActorScale3D))
  (bind _mesh (Variables|Character|GetMesh))
  (bind _mesh_2 (Variables|Character|GetMesh))
  (bind _ac_waterballmechanics (Variables|Default|GetAC_WaterBallMechanics))
  (bind _ac_waterballmechanics_2 (Variables|Default|GetAC_WaterBallMechanics))
  (bind _ac_waterballmechanics_3 (Variables|Default|GetAC_WaterBallMechanics))
  ;[1 1 1] 攻撃
  (if (Variables|Default|GetUnder50)
    (if (> (Math|Random|RandomInteger 100) 66)
      (bind _notifyname (Animation|Montage|PlayMontage (Variables|Character|GetMesh) "/Game/QuadrapedCreatures/MountainDragon/AM/AM_Dragon_Attack_06.AM_Dragon_Attack_06")
        (:OnCompleted
          (Default|CallOnAttackEnd :!label _label))
        (:OnInterrupted
          (goto _label))
        (:OnNotifyBegin
          (switch name _notifyname
            (:Takeoff
              (Transformation|SetRelativeLocation _mesh_2 (Math|Vector|MakeVector 0.0 0.0 (* (.z _returnvalue_2) 1e+02)) false false))
            (:Begin
              (Default|SpawnPillar (Variables|Default|GetAC_WaterBallMechanics) "None"))
            (:Attack
              (Default|PillarFareBegin (Variables|Default|GetAC_WaterBallMechanics)))
            (:Takeon
              (Transformation|SetRelativeLocation _mesh_2 (Math|Vector|MakeVector 0.0 0.0 (* (.z _returnvalue_2) -3e+02)) false false)))))
      (elif (> (Math|Random|RandomInteger 100) 66)
        (bind _notifyname_2 (Animation|Montage|PlayMontage (Variables|Character|GetMesh) "/Game/QuadrapedCreatures/MountainDragon/AM/AM_Dragon_Attack01.AM_Dragon_Attack01")
          (:OnCompleted
            (Default|CallOnAttackEnd :!label _label_2))
          (:OnInterrupted
            (goto _label_2))
          (:OnNotifyBegin
            (switch name _notifyname_2
              (:Begin01
                (Default|SpawnBlade (Variables|Default|GetAC_WaterBallMechanics) (Variables|Default|GetRclaw_Soket)))
              (:Begin02
                (Default|SpawnBlade (Variables|Default|GetAC_WaterBallMechanics) (Variables|Default|GetLclaw_Soket)))
              (:Claw01
                (Default|BladeFireBegin (Variables|Default|GetAC_WaterBallMechanics) :!label _label_3))
              (:Claw02
                (goto _label_3)))))
        (else
          (bind _notifyname_3 (Animation|Montage|PlayMontage (Variables|Character|GetMesh) "/Game/QuadrapedCreatures/MountainDragon/AM/AM_Dragon_Attack_05.AM_Dragon_Attack_05")
            (:OnCompleted
              (Default|CallOnAttackEnd :!label _label_4))
            (:OnInterrupted
              (goto _label_4))
            (:OnNotifyBegin
              (switch name _notifyname_3
                (:Begin
                  (Transformation|SetRelativeLocation _mesh (Math|Vector|MakeVector 0.0 0.0 (* (.z _returnvalue) 1e+02)) false false))
                (:Spawn
                  (Default|SpawnBall _ac_waterballmechanics (Variables|Default|GetFireboll_Soket))
                  (Default|SpawnBlade _ac_waterballmechanics_2 (Variables|Default|GetLwing_Soket))
                  (Default|SpawnPillar _ac_waterballmechanics_3 (Variables|Default|GetRwing_Soket)))
                (:Fire
                  (Default|BallFireBegin _ac_waterballmechanics)
                  (Default|BladeFireBegin _ac_waterballmechanics_2)
                  (Default|PillarFareBegin _ac_waterballmechanics_3))
                (:Takeon
                  (Transformation|SetRelativeLocation _mesh (Math|Vector|MakeVector 0.0 0.0 (* (.z _returnvalue) -3e+02)) false false))))))))
    (elif (> (Math|Random|RandomInteger 100) 75)
      (bind _notifyname_4 (Animation|Montage|PlayMontage (Variables|Character|GetMesh) "/Game/QuadrapedCreatures/MountainDragon/AM/AM_Dragon_Attack_03.AM_Dragon_Attack_03")
        (:OnCompleted
          (Default|CallOnAttackEnd :!label _label_5))
        (:OnInterrupted
          (goto _label_5))
        (:OnNotifyBegin
          (switch name _notifyname_4
            (:FireBigin
              (Default|SpawnBall (Variables|Default|GetAC_WaterBallMechanics) (Variables|Default|GetFireboll_Soket)))
            (:Fire01
              (Default|BallFireBegin (Variables|Default|GetAC_WaterBallMechanics))
              (Rendering|ToggleVisibility (Variables|Default|GetParticleSystem) false))
            (:Bigin
              (Rendering|ToggleVisibility (Variables|Default|GetParticleSystem) false)))))
      (elif (> (Math|Random|RandomInteger 100) 75)
        (bind _notifyname_5 (Animation|Montage|PlayMontage (Variables|Character|GetMesh) "/Game/QuadrapedCreatures/MountainDragon/AM/AM_DragonAttack09.AM_DragonAttack09")
          (:OnCompleted
            (Default|CallOnAttackEnd :!label _label_6))
          (:OnInterrupted
            (goto _label_6))
          (:OnNotifyBegin
            (switch name _notifyname_5
              (:Begin
                (Default|SpawnBlade (Variables|Default|GetAC_WaterBallMechanics) (Variables|Default|GetRclaw_Soket)))
              (:Claw
                (Default|BladeFireBegin (Variables|Default|GetAC_WaterBallMechanics))))))
        (elif (> (Math|Random|RandomInteger 100) 75)
          (bind _notifyname_6 (Animation|Montage|PlayMontage (Variables|Character|GetMesh) "/Game/QuadrapedCreatures/MountainDragon/AM/AM_DragonAttack08.AM_DragonAttack08")
            (:OnCompleted
              (Default|CallOnAttackEnd :!label _label_7))
            (:OnInterrupted
              (goto _label_7))
            (:OnNotifyBegin
              (switch name _notifyname_6
                (:Begin
                  (Default|SpawnBlade (Variables|Default|GetAC_WaterBallMechanics) (Variables|Default|GetLclaw_Soket)))
                (:Claw
                  (Default|BladeFireBegin (Variables|Default|GetAC_WaterBallMechanics))))))
          (else
            (bind _notifyname_7 (Animation|Montage|PlayMontage (Variables|Character|GetMesh) "/Game/QuadrapedCreatures/MountainDragon/AM/AM_Dragon_Attack_03.AM_Dragon_Attack_03")
              (:OnCompleted
                (Default|CallOnAttackEnd :!label _label_8))
              (:OnInterrupted
                (goto _label_8))
              (:OnNotifyBegin
                (switch name _notifyname_7
                  (:Fire01
                    (Default|Fire (stale _returnvalue_3))
                    (Utilities|FlowControl|Delay 1.0)
                    (Actor|DestroyActor (stale _returnvalue_3)))
                  (:Bigin
                    (bind _output_get (Variables|Default|SetPlayerLocation (Transformation|GetActorLocation (Game|GetPlayerCharacter 0))))
                    (bind _returnvalue_3 (Game|SpawnActorfromClass "/Game/QuadrapedCreatures/MountainDragon/BP/BP_Dragon_WaterPillar02.BP_Dragon_WaterPillar02_C" (Math|Transform|MakeTransform _output_get "0, 0, 0" "1.000000,1.000000,1.000000") "Undefined" "MultiplyWithRoot" 0 0))))))))))))

(fn ConstructionScript
  (|CallParentFunction))

(fn IsDead
  (Actor|DestroyActor (Variables|Default|GetField))
  (return true))

(fn TakeDamage
  (params (DamageInfo :type S%20Damage%20Info%20Structure))
  (bind _wasdamaged (Default|TakeDamage (Variables|Default|GetBPC_DamageSystem) DamageInfo))
  (return _wasdamaged))

(fn GetIdealRange
  (return 2e+03 2.5e+03))

(fn SetMovementSpeed
  (params (Speed :type E_EnemySpeed%20Enum :default "NewEnumerator0"))
  (bind _output_get (Variables|/Script/Engine.CharacterMovementComponent|SetMaxWalkSpeed (Variables|Character|GetCharacterMovement) (Utilities|Select :Index Speed :NewEnumerator0 0.0 :NewEnumerator1 2e+02 :NewEnumerator2 3e+02 :NewEnumerator3 5e+02)))
  (return _output_get))