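; Actor component that handles the water ball, pillar and blade projectile attacks of the BP_Dragon_Kimo dragon.
; Spawn functions create each projectile attached to a socket on the dragon's mesh, and matching Destroy functions remove it.
; Fire events detach the projectile and, if the dragon AI controller's AttackTarget is valid, launch it toward that target's current location.
; Each launch also runs a visibility line trace whose result is unused.
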(event Custom|BladeFireBegin
  (bind _bladeref (Variables|Default|GetBladeRef))
  (bind _returnvalue (Transformation|GetActorLocation _bladeref))
  (bind _bladeref_2 (Variables|Default|GetBladeRef)
    (:then
      (Transformation|DetachFromActor _bladeref_2 "KeepWorld" "KeepRelative" "KeepRelative")
      (bind _asai_controller_dragon (Utilities|Casting|CastToAI_Controller_Dragon (AI|GetAIController (Variables|Default|GetCharacterRef))))
      (bind _attack_target (Variables|/Game/QuadrapedCreatures/MountainDragon/AI/AI_Controller_Dragon.AI_Controller_Dragon_C|GetAttack%20Target _asai_controller_dragon)
        (:then
          (Collision|LineTraceByChannel _returnvalue (Transformation|GetActorLocation _attack_target) "TraceTypeQuery1" false 0 "None")
          (Default|Fire (Variables|Default|GetBladeRef) (Math|Vector|GetUnitDirection(Vector) _returnvalue (Transformation|GetActorLocation _attack_target))))
        (:else)))
    (:else)))

(event Custom|BallFireBegin
  (bind _ballref (Variables|Default|GetBallRef))
  (bind _returnvalue (Transformation|GetActorLocation _ballref))
  (bind _ballref_2 (Variables|Default|GetBallRef)
    (:then
      (Transformation|DetachFromActor _ballref_2 "KeepWorld" "KeepWorld" "KeepWorld")
      (bind _asai_controller_dragon (Utilities|Casting|CastToAI_Controller_Dragon (AI|GetAIController (Variables|Default|GetCharacterRef))))
      (bind _attack_target (Variables|/Game/QuadrapedCreatures/MountainDragon/AI/AI_Controller_Dragon.AI_Controller_Dragon_C|GetAttack%20Target _asai_controller_dragon)
        (:then
          (Collision|LineTraceByChannel _returnvalue (Transformation|GetActorLocation _attack_target) "TraceTypeQuery1" false 0 "None")
          (Default|Fire (Variables|Default|GetBallRef) (Math|Vector|GetUnitDirection(Vector) _returnvalue (Transformation|GetActorLocation _attack_target))))
        (:else)))
    (:else)))

(event Custom|PillarFareBegin
  (bind _pillarref (Variables|Default|GetPillarRef))
  (bind _returnvalue (Transformation|GetActorLocation _pillarref))
  (bind _pillarref_2 (Variables|Default|GetPillarRef)
    (:then
      (Transformation|DetachFromActor _pillarref_2 "KeepWorld" "KeepRelative" "KeepRelative")
      (bind _asai_controller_dragon (Utilities|Casting|CastToAI_Controller_Dragon (AI|GetAIController (Variables|Default|GetCharacterRef))))
      (bind _attack_target (Variables|/Game/QuadrapedCreatures/MountainDragon/AI/AI_Controller_Dragon.AI_Controller_Dragon_C|GetAttack%20Target _asai_controller_dragon)
        (:then
          (Collision|LineTraceByChannel _returnvalue (Transformation|GetActorLocation _attack_target) "TraceTypeQuery1" false 0 "None")
          (Default|Fire (Variables|Default|GetPillarRef) (Math|Vector|GetUnitDirection(Vector) _returnvalue (Transformation|GetActorLocation _attack_target))))
        (:else)))
    (:else)))

(event EventBeginPlay
  (bind _asbp_dragon_kimo (Utilities|Casting|CastToBP_Dragon_Kimo (Components|GetOwner)))
  (Variables|Default|SetCharacterRef _asbp_dragon_kimo))

(fn SpawnBall
  (bind _returnvalue (Game|SpawnActorfromClass "/Game/QuadrapedCreatures/MountainDragon/BP/BP_Dragon_WaterBall.BP_Dragon_WaterBall_C" (Math|Transform|MakeTransform "0, 0, 0" (Transformation|GetActorRotation (Variables|Default|GetCharacterRef)) "1.000000,1.000000,1.000000") "Undefined" "MultiplyWithRoot" 0 0.0 0.0 0))
  (bind _output_get (Variables|Default|SetBallRef _returnvalue))
  (Transformation|AttachComponentToComponent _output_get (Variables|/Script/Engine.Character|GetMesh (Variables|Default|GetCharacterRef)) (Variables|Default|GetBollSocketName) "SnapToTarget" "SnapToTarget" "SnapToTarget" true))

(fn DestroyBall
  (bind _ballref (Variables|Default|GetBallRef)
    (:then
      (Actor|DestroyActor _ballref))
    (:else)))

(fn SpawnPillar
  (bind _returnvalue (Game|SpawnActorfromClass "/Game/QuadrapedCreatures/MountainDragon/BP/BP_Dragon_WaterPillar.BP_Dragon_WaterPillar_C" (Math|Transform|MakeTransform "0, 0, 0" (Transformation|GetActorRotation (Variables|Default|GetCharacterRef)) "1.000000,1.000000,0.500000") "Undefined" "MultiplyWithRoot" 0 0.0 0.0 0))
  (bind _output_get (Variables|Default|SetPillarRef _returnvalue))
  (Transformation|AttachComponentToComponent _output_get (Variables|/Script/Engine.Character|GetMesh (Variables|Default|GetCharacterRef)) (Variables|Default|GetPillarSocketName) "SnapToTarget" "SnapToTarget" "KeepWorld" true))

(fn SpawnBlade
  (bind _returnvalue (Game|SpawnActorfromClass "/Game/QuadrapedCreatures/MountainDragon/BP/BP_Dragon_WaterBlade.BP_Dragon_WaterBlade_C" (Math|Transform|MakeTransform "0, 0, 0" (Transformation|GetActorRotation (Variables|Default|GetCharacterRef)) "1.000000,1.000000,1.000000") "Undefined" "MultiplyWithRoot" 0 0.0 0.0 0))
  (bind _output_get (Variables|Default|SetBladeRef _returnvalue))
  (Transformation|AttachComponentToComponent _output_get (Variables|/Script/Engine.Character|GetMesh (Variables|Default|GetCharacterRef)) (Variables|Default|GetBladeSocketName) "SnapToTarget" "KeepRelative" "KeepRelative" true))

(fn DestroyPillar
  (bind _pillarref (Variables|Default|GetPillarRef)
    (:then
      (Actor|DestroyActor _pillarref))
    (:else)))

(fn DestroyBlade
  (bind _bladeref (Variables|Default|GetBladeRef)
    (:then
      (Actor|DestroyActor _bladeref))
    (:else)))