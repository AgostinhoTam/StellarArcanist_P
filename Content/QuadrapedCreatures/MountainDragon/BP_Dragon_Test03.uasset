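; Test variant of the Mountain Dragon creature that performs a montage-driven ranged attack.
; The Attack event plays a dragon attack montage on the mesh and calls OnAttackEnd when it completes or is interrupted.
; Montage notifies drive the reused ACBowMechanics component, spawning an arrow on the fire-begin notify and starting its launch on the following one.
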(event EventBeginPlay
  (|CallParentFunction) ; このノードは無効になっているため呼び出せません。\n機能をビルドするにはピンをドラッグしてください。
)

(event Collision|EventActorBeginOverlap
  (params (OtherActor :type Actor%20Object%20Reference))
  (|CallParentFunction OtherActor) ; このノードは無効になっているため呼び出せません。\n機能をビルドするにはピンをドラッグしてください。
)

(event EventTick
  (params (DeltaSeconds :type Float%20%28single-precision%29))
  (|CallParentFunction DeltaSeconds) ; このノードは無効になっているため呼び出せません。\n機能をビルドするにはピンをドラッグしてください。
)

(event EventAttack
  (bind _notifyname (Animation|Montage|PlayMontage (Variables|Character|GetMesh) "/Game/QuadrapedCreatures/MountainDragon/AM_Dragon_Attack_03.AM_Dragon_Attack_03")
    (:OnCompleted
      (Default|CallOnAttackEnd :!label _label))
    (:OnInterrupted
      (goto _label))
    (:OnNotifyBegin
      (switch name _notifyname
        (:FireBigin
          (Default|SpawnArrow (Variables|Default|GetAC_BowMechanics)))
        (:Fire01
          (Default|FireArrowBegin (Variables|Default|GetAC_BowMechanics)))))))

(fn ConstructionScript
  (|CallParentFunction))