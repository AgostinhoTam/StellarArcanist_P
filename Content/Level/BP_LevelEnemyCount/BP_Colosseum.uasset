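; BP_Colosseum is an actor that tracks the remaining enemies and opens the Clear1_Bar level once all are gone.
; On BeginPlay it stores the number of BP_Enemy_Base actors in the level as AllEnemy.
; Each call to its EnemyCount event decrements that total and loads the next level when it reaches zero or below.
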(event Custom|EnemyCount
  (Variables|Default|SetAllEnemy (- (Variables|Default|GetAllEnemy) 1))
  (if (<= (Variables|Default|GetAllEnemy) 0)
    (Game|OpenLevel(byObjectReference) "/Game/Level/Clear1_Bar.Clear1_Bar")))

(event EventBeginPlay
  (bind _outactors (Actor|GetAllActorsOfClass "/Game/Enemy/Enemy_Sin_Test/BP_Enemy_Base.BP_Enemy_Base_C"))
  (bind _output_get (Variables|Default|SetOut%20Actors _outactors))
  (Variables|Default|SetAllEnemy (Utilities|Array|Length _output_get)))

(fn ConstructionScript)