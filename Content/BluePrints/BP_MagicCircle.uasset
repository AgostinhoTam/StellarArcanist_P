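; Magic circle for setting up a spell's initial components: shape, attribute, spawn, attack and compression.
; Selecting a component highlights its icon and opens a chip or charge widget.
; Loaded chips refresh icon materials by type, while slider values from BP_MagicGameInstance rebuild the shape, attribute and spawn chip structs.
; Stamina cost combines a per-variant data table base with the shape slider scaled by the chip's increment, even for non-shape chips.
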(event Custom|Select_InitComponentEvent
  (Variables|Default|GetInitSelectComponent_Used
    (:then
      (bind _widgetref (Variables|Default|GetWidgetRef)
        (:then
          (Widget|RemovefromParent _widgetref))
        (:else
          _))
      (CallFunction|SetInitMaterial)
      (if (== (Variables|Default|GetInitSelect_Shape) (Variables|Default|GetInitSelectComponent_Used))
        (Variables|Default|SetSelect_InitComponentNumber 1)
        (Rendering|Material|SetMaterial (Variables|Default|GetInitMagicIcon2) 0 "/Engine/MapTemplates/Materials/BasicAsset03.BasicAsset03")
        (CallFunction|CreateWidget "NewEnumerator0")
        (Variables|Default|SetIsShow? true)
        (elif (== (Variables|Default|GetInitSelect_Spawn) (Variables|Default|GetInitSelectComponent_Used))
          (Variables|Default|SetSelect_InitComponentNumber 2)
          (Rendering|Material|SetMaterial (Variables|Default|GetInitMagicIcon1) 0 "/Engine/MapTemplates/Materials/BasicAsset03.BasicAsset03")
          (CallFunction|CreateWidget "NewEnumerator6")
          (Variables|Default|SetIsShow? true)
          (elif (== (Variables|Default|GetInitSelect_Damege) (Variables|Default|GetInitSelectComponent_Used))
            (Variables|Default|SetSelect_InitComponentNumber 3)
            (Rendering|Material|SetMaterial (Variables|Default|GetInitMagicIcon5) 0 "/Engine/MapTemplates/Materials/BasicAsset03.BasicAsset03")
            (CallFunction|CreateWidget "NewEnumerator9")
            (Variables|Default|SetIsShow? true)
            (elif (== (Variables|Default|GetInitSelect_Compression) (Variables|Default|GetInitSelectComponent_Used))
              (Variables|Default|SetSelect_InitComponentNumber 4)
              (Rendering|Material|SetMaterial (Variables|Default|GetInitMagicIcon4) 0 "/Engine/MapTemplates/Materials/BasicAsset03.BasicAsset03")
              (CallFunction|CreateWidgetforAtkCom "NewEnumerator1")
              (Variables|Default|SetIsShow? true)
              (elif (== (Variables|Default|GetInitSelect_Attribute) (Variables|Default|GetInitSelectComponent_Used))
                (Variables|Default|SetSelect_InitComponentNumber 5)
                (Rendering|Material|SetMaterial (Variables|Default|GetInitMagicIcon3) 0 "/Engine/MapTemplates/Materials/BasicAsset03.BasicAsset03")
                (CallFunction|CreateWidgetforAtkCom "NewEnumerator0")
                (Variables|Default|SetIsShow? true)))))))
    (:else)))

(event Custom|LoadInitData
  (params (LoadMagicChipInfo :type S%20Magic%20Chip%20Info%20Ver%202%20Structure))
  (bind (_chipstatas _chipshape _chipmove _chipspecial _chipcondition _chipattribute _chipend _chipspawn) (Utilities|Struct|BreakS_MagicChipInfo_Ver2 LoadMagicChipInfo))
  ;[1 1 1] 初期化チップのマテリアルとか設定
  (Variables|Default|SetMagicChipInfo LoadMagicChipInfo)
  (CallFunction|SetInitMaterial)
  (switch Utilities|FlowControl|Switch|SwitchonE_ChipType_Ver2 (.ChipType (Utilities|Struct|BreakS_ChipStatas_Ver2 _chipstatas))
    (:NewEnumerator0
      (Variables|/Game/Scene/BP_MagicGameInstance.BP_MagicGameInstance_C|SetInitSliderValue_Shape (Variables|Default|GetAsBPMagicGameInstance) (/ (.size (Utilities|Struct|BreakS_ChipShape_Ver2 _chipshape)) (Variables|/Game/BluePrints/BP_Chip.BP_Chip_C|GetSize (Variables|Default|GetChipSample))))
      (Variables|Default|SetMagicChipInfo_Shape (Variables|Default|GetMagicChipInfo)))
    (:NewEnumerator6
      (Variables|/Game/Scene/BP_MagicGameInstance.BP_MagicGameInstance_C|SetInitSliderValue_Attribute (Variables|Default|GetAsBPMagicGameInstance) (/ (.AttributeDamege (Utilities|Struct|BreakS_ChipAttribute_Ver2 _chipattribute)) (Variables|/Game/BluePrints/BP_Chip.BP_Chip_C|GetAttributeDamege (Variables|Default|GetChipSample))))
      (Variables|Default|SetMagicChipInfo_Attribute (Variables|Default|GetMagicChipInfo)))
    (:NewEnumerator9
      (Variables|/Game/Scene/BP_MagicGameInstance.BP_MagicGameInstance_C|SetInitSliderValue_Attribute (Variables|Default|GetAsBPMagicGameInstance) (/ (.SpawnDistance (Utilities|Struct|BreakS_ChipSpawn_Ver2 _chipspawn)) (Variables|/Game/BluePrints/BP_Chip.BP_Chip_C|GetDistance (Variables|Default|GetChipSample))))
      (Variables|Default|SetMagicChipInfo_Spawn (Variables|Default|GetMagicChipInfo)))))

(event Custom|SetInitMaterial
  ;[1 1 1] マテリアルの初期化
  (CallFunction|SetMaterialShape)
  (CallFunction|SetMaterialAttribute)
  (Rendering|Material|SetMaterial (Variables|Default|GetInitMagicIcon4) 0 "/Engine/BasicShapes/BasicShapeMaterial.BasicShapeMaterial")
  (CallFunction|SetMaterialSpawn)
  (bind _widgetref (Variables|Default|GetWidgetRef)
    (:then
      (Widget|RemovefromParent _widgetref)
      (Variables|Default|SetIsShow? false))
    (:else)))

(event Custom|ChengeValue_Chip
  ;[1 1 1] スライダーを動かした時のチップの値の設定
  (switch Utilities|FlowControl|Switch|SwitchonE_ChipType_Ver2 (.ChipType (Utilities|Struct|BreakS_ChipStatas_Ver2 (.ChipStatas (Utilities|Struct|BreakS_MagicChipInfo_Ver2 (Variables|Default|GetMagicChipInfo)))))
    (:NewEnumerator0
      (CallFunction|SetChipValueShape))
    (:NewEnumerator6
      (CallFunction|SetChipValueAttribte))
    (:NewEnumerator9
      (CallFunction|SetChipValueSpawn))))

(event Custom|ChengeValue_Statas
  (params (MagicStatasType :type E_MagicAtkCom%20Enum :default "NewEnumerator0"))
  ;[1 1 1] 攻撃力や耐久を設定
  (switch Utilities|FlowControl|Switch|SwitchonE_MagicAtkCom MagicStatasType
    (:NewEnumerator0
      (Variables|Default|SetAttackValue (Variables|/Game/Scene/BP_MagicGameInstance.BP_MagicGameInstance_C|GetAttackValue (Variables|Default|GetAsBPMagicGameInstance))))
    (:NewEnumerator1
      (Variables|Default|SetCompositionValue (Variables|/Game/Scene/BP_MagicGameInstance.BP_MagicGameInstance_C|GetCompositionValue (Variables|Default|GetAsBPMagicGameInstance))))))

(event EventBeginPlay
  ;[1 1 1] 最初にインスタンスのポインタを取得
  (bind _asbp_magic_game_instance (Utilities|Casting|CastToBP_MagicGameInstance (Game|GetGameInstance)))
  (Variables|Default|SetAsBPMagicGameInstance _asbp_magic_game_instance))

(fn ConstructionScript)

(fn CreateWidget
  (params (SelectedType :type E_ChipType_Ver2%20Enum :default "NewEnumerator0"))
  (bind _returnvalue (UserInterface|CreateWidget "/Game/Widget/DefaultUI/WBP_MagicTitleView.WBP_MagicTitleView_C" 0 SelectedType))
  (UserInterface|Viewport|AddtoViewport _returnvalue 0)
  (Variables|Default|SetWidgetRef _returnvalue))

(fn CreateWidgetforAtkCom
  (params (MagicAtkCom :type E_MagicAtkCom%20Enum :default "NewEnumerator0"))
  (switch Utilities|FlowControl|Switch|SwitchonE_MagicAtkCom MagicAtkCom
    (:NewEnumerator0
      (bind _returnvalue (UserInterface|CreateWidget "/Game/Widget/DefaultUI/WBP_AtkComCharge.WBP_AtkComCharge_C" 0 MagicAtkCom))
      (bind _output_get (Variables|Default|SetWidgetRef _returnvalue)))
    (:NewEnumerator1
      (bind _returnvalue_2 (UserInterface|CreateWidget "/Game/Widget/DefaultUI/WBP_AtkComCharge.WBP_AtkComCharge_C" 0 MagicAtkCom))
      (bind _output_get_2 (Variables|Default|SetWidgetRef _returnvalue_2))))
  (UserInterface|Viewport|AddtoViewport _output_get_2 0)
  (Class|UserWidget|SetPositioninViewport _output_get_2 "(X=760.000000,Y=400.000000)" true))

(fn SetChipValueShape
  (bind _magicchipinfo (Variables|Default|GetMagicChipInfo))
  (bind (_chipstatas _chipshape _chipmove _chipspecial _chipcondition _chipattribute _chipend _chipspawn) (Utilities|Struct|BreakS_MagicChipInfo_Ver2 _magicchipinfo))
  (bind (_chipshapetype _3dtexture _isused_) (Utilities|Struct|BreakS_ChipShape_Ver2 _chipshape))
  (switch Utilities|FlowControl|Switch|SwitchonE_ChipShapeType_Ver2 _chipshapetype
    (:NewEnumerator1
      (Variables|Default|SetDTRowName "Shape_Cube"))
    (:NewEnumerator2
      (Variables|Default|SetDTRowName "Shape_Sphere"))
    (:NewEnumerator3
      (Variables|Default|SetDTRowName "Shape_Wall")))
  (bind _stamina (Class|BPIGetMagicChipDT|GetDTStamina(Message) (Variables|Default|GetChipSample) (Variables|Default|GetDTRowName)))
  (Variables|Default|SetInitStamina _stamina)
  (CallFunction|SetStamina)
  (Variables|Default|SetMagicChipInfo_Shape (Utilities|Struct|MakeS_MagicChipInfo_Ver2 _chipstatas (Utilities|Struct|MakeS_ChipShape_Ver2 _chipshapetype _3dtexture _isused_ (* (Variables|/Game/Scene/BP_MagicGameInstance.BP_MagicGameInstance_C|GetInitSliderValue_Shape (Variables|Default|GetAsBPMagicGameInstance)) (Variables|/Game/BluePrints/BP_Chip.BP_Chip_C|GetSize (Variables|Default|GetChipSample)))) _chipmove _chipspecial _chipcondition _chipattribute _chipend _chipspawn)))

(fn SetMaterialShape
  (bind _initmagicicon2 (Variables|Default|GetInitMagicIcon2))
  (bind _magicchipinfo (Variables|Default|GetMagicChipInfo))
  (bind (_chipstatas _chipshape) (Utilities|Struct|BreakS_MagicChipInfo_Ver2 _magicchipinfo))
  (if (<= (.TimeStart (Utilities|Struct|BreakS_ChipStatas_Ver2 _chipstatas)) -1.0)
    (switch Utilities|FlowControl|Switch|SwitchonE_ChipShapeType_Ver2 (.ChipShapeType (Utilities|Struct|BreakS_ChipShape_Ver2 _chipshape))
      (:NewEnumerator1
        (Rendering|Material|SetMaterial _initmagicicon2 0 "/Game/MagicChipTexstures/MagicChipIcon/M_BUILDSQUARE_Mat.M_BUILDSQUARE_Mat"))
      (:NewEnumerator2
        (Rendering|Material|SetMaterial _initmagicicon2 0 "/Game/MagicChipTexstures/MagicChipIcon/M_BUILDBALL_Mat.M_BUILDBALL_Mat"))
      (:NewEnumerator3
        (Rendering|Material|SetMaterial _initmagicicon2 0 "/Game/MagicChipTexstures/MagicChipIcon/M_BUILDWALL_Mat.M_BUILDWALL_Mat")))
    (else
      (Rendering|Material|SetMaterial (Variables|Default|GetInitMagicIcon2) 0 "/Engine/BasicShapes/BasicShapeMaterial.BasicShapeMaterial"))))

(fn SetStamina
  (Variables|Default|SetMagicChipInfo (Utilities|Struct|MakeS_MagicChipInfo_Ver2 (Utilities|Struct|MakeS_ChipStatas_Ver2 (.ChipName (Utilities|Struct|BreakS_ChipStatas_Ver2 (.ChipStatas (Utilities|Struct|BreakS_MagicChipInfo_Ver2 (Variables|Default|GetMagicChipInfo))))) (.ChipDescription (Utilities|Struct|BreakS_ChipStatas_Ver2 (.ChipStatas (Utilities|Struct|BreakS_MagicChipInfo_Ver2 (Variables|Default|GetMagicChipInfo))))) (.ChipIcon (Utilities|Struct|BreakS_ChipStatas_Ver2 (.ChipStatas (Utilities|Struct|BreakS_MagicChipInfo_Ver2 (Variables|Default|GetMagicChipInfo))))) (.CastTime (Utilities|Struct|BreakS_ChipStatas_Ver2 (.ChipStatas (Utilities|Struct|BreakS_MagicChipInfo_Ver2 (Variables|Default|GetMagicChipInfo))))) (.ChipDamege (Utilities|Struct|BreakS_ChipStatas_Ver2 (.ChipStatas (Utilities|Struct|BreakS_MagicChipInfo_Ver2 (Variables|Default|GetMagicChipInfo))))) (.ChipType (Utilities|Struct|BreakS_ChipStatas_Ver2 (.ChipStatas (Utilities|Struct|BreakS_MagicChipInfo_Ver2 (Variables|Default|GetMagicChipInfo))))) (.IsBad? (Utilities|Struct|BreakS_ChipStatas_Ver2 (.ChipStatas (Utilities|Struct|BreakS_MagicChipInfo_Ver2 (Variables|Default|GetMagicChipInfo))))) (.ChipNumber (Utilities|Struct|BreakS_ChipStatas_Ver2 (.ChipStatas (Utilities|Struct|BreakS_MagicChipInfo_Ver2 (Variables|Default|GetMagicChipInfo))))) (.ActorLocation (Utilities|Struct|BreakS_ChipStatas_Ver2 (.ChipStatas (Utilities|Struct|BreakS_MagicChipInfo_Ver2 (Variables|Default|GetMagicChipInfo))))) (.TimeStart (Utilities|Struct|BreakS_ChipStatas_Ver2 (.ChipStatas (Utilities|Struct|BreakS_MagicChipInfo_Ver2 (Variables|Default|GetMagicChipInfo))))) (.TimeEnd (Utilities|Struct|BreakS_ChipStatas_Ver2 (.ChipStatas (Utilities|Struct|BreakS_MagicChipInfo_Ver2 (Variables|Default|GetMagicChipInfo))))) (+ (* (Variables|/Game/Scene/BP_MagicGameInstance.BP_MagicGameInstance_C|GetInitSliderValue_Shape (Variables|Default|GetAsBPMagicGameInstance)) (.UpStaminaValue (Utilities|Struct|BreakS_ChipStatas_Ver2 (.ChipStatas (Utilities|Struct|BreakS_MagicChipInfo_Ver2 (Variables|Default|GetMagicChipInfo)))))) (Variables|Default|GetInitStamina)) (.UI_ChipIcon (Utilities|Struct|BreakS_ChipStatas_Ver2 (.ChipStatas (Utilities|Struct|BreakS_MagicChipInfo_Ver2 (Variables|Default|GetMagicChipInfo))))) (.hardness (Utilities|Struct|BreakS_ChipStatas_Ver2 (.ChipStatas (Utilities|Struct|BreakS_MagicChipInfo_Ver2 (Variables|Default|GetMagicChipInfo))))) (.UpStaminaValue (Utilities|Struct|BreakS_ChipStatas_Ver2 (.ChipStatas (Utilities|Struct|BreakS_MagicChipInfo_Ver2 (Variables|Default|GetMagicChipInfo))))) (.UpCastValue (Utilities|Struct|BreakS_ChipStatas_Ver2 (.ChipStatas (Utilities|Struct|BreakS_MagicChipInfo_Ver2 (Variables|Default|GetMagicChipInfo)))))) (.ChipShape (Utilities|Struct|BreakS_MagicChipInfo_Ver2 (Variables|Default|GetMagicChipInfo))) (.ChipMove (Utilities|Struct|BreakS_MagicChipInfo_Ver2 (Variables|Default|GetMagicChipInfo))) (.ChipSpecial (Utilities|Struct|BreakS_MagicChipInfo_Ver2 (Variables|Default|GetMagicChipInfo))) (.ChipCondition (Utilities|Struct|BreakS_MagicChipInfo_Ver2 (Variables|Default|GetMagicChipInfo))) (.ChipAttribute (Utilities|Struct|BreakS_MagicChipInfo_Ver2 (Variables|Default|GetMagicChipInfo))) (.ChipEnd (Utilities|Struct|BreakS_MagicChipInfo_Ver2 (Variables|Default|GetMagicChipInfo))) (.ChipSpawn (Utilities|Struct|BreakS_MagicChipInfo_Ver2 (Variables|Default|GetMagicChipInfo))))))

(fn SetMaterialAttribute
  (bind _magicchipinfo (Variables|Default|GetMagicChipInfo))
  (bind (_chipstatas _chipshape _chipmove _chipspecial _chipcondition _chipattribute) (Utilities|Struct|BreakS_MagicChipInfo_Ver2 _magicchipinfo))
  (if (<= (.TimeStart (Utilities|Struct|BreakS_ChipStatas_Ver2 _chipstatas)) -1.0)
    (switch Utilities|FlowControl|Switch|SwitchonE_ChipAttributeType_Ver2 (.ChipAttributeType (Utilities|Struct|BreakS_ChipAttribute_Ver2 _chipattribute))
      (:NewEnumerator0
        (Rendering|Material|SetMaterial (Variables|Default|GetInitMagicIcon1) 0 "/Game/MagicChipTexstures/MagicChipIcon/M_ATTRIBUTEFIRE_Mat.M_ATTRIBUTEFIRE_Mat"))
      (:NewEnumerator1
        (Rendering|Material|SetMaterial (Variables|Default|GetInitMagicIcon1) 0 "/Game/MagicChipTexstures/MagicChipIcon/M_ATTRIBUTEWATER_Mat.M_ATTRIBUTEWATER_Mat"))
      (:NewEnumerator3
        (Rendering|Material|SetMaterial (Variables|Default|GetInitMagicIcon1) 0 "/Game/MagicChipTexstures/MagicChipIcon/M_ATTRIBUTETHUNDER_Mat.M_ATTRIBUTETHUNDER_Mat"))
      (:NewEnumerator4
        (Rendering|Material|SetMaterial (Variables|Default|GetInitMagicIcon1) 0 "/Game/MagicChipTexstures/MagicChipIcon/M_ATTRIBUTESOIL_Mat.M_ATTRIBUTESOIL_Mat")))
    (else
      (Rendering|Material|SetMaterial (Variables|Default|GetInitMagicIcon1) 0 "/Engine/BasicShapes/BasicShapeMaterial.BasicShapeMaterial"))))

(fn SetMaterialSpawn
  (bind _magicchipinfo (Variables|Default|GetMagicChipInfo))
  (bind _initmagicicon5 (Variables|Default|GetInitMagicIcon5))
  (bind (_chipstatas _chipshape _chipmove _chipspecial _chipcondition _chipattribute _chipend _chipspawn) (Utilities|Struct|BreakS_MagicChipInfo_Ver2 _magicchipinfo))
  (bind (_spawntype _spawndirection) (Utilities|Struct|BreakS_ChipSpawn_Ver2 _chipspawn))
  (if (<= (.TimeStart (Utilities|Struct|BreakS_ChipStatas_Ver2 _chipstatas)) -1.0)
    (switch Utilities|FlowControl|Switch|SwitchonE_ChipSpawnType_Ver2 _spawntype
      (:NewEnumerator1
        (switch Utilities|FlowControl|Switch|SwitchonE_ChipSpawnDirectionType_Ver2 _spawndirection
          (:NewEnumerator1
            (Rendering|Material|SetMaterial _initmagicicon5 0 "/Game/MagicChipTexstures/MagicChipIcon/M_SPAWNFORWARD_Mat.M_SPAWNFORWARD_Mat"))
          (:NewEnumerator2
            (Rendering|Material|SetMaterial _initmagicicon5 0 "/Game/MagicChipTexstures/MagicChipIcon/M_SPAWNBACK_Mat.M_SPAWNBACK_Mat"))
          (:NewEnumerator3
            (Rendering|Material|SetMaterial _initmagicicon5 0 "/Game/MagicChipTexstures/MagicChipIcon/M_SPAWNLEFT_Mat.M_SPAWNLEFT_Mat"))
          (:NewEnumerator4
            (Rendering|Material|SetMaterial _initmagicicon5 0 "/Game/MagicChipTexstures/MagicChipIcon/M_SPAWNRIGHT_Mat.M_SPAWNRIGHT_Mat"))
          (:NewEnumerator5
            (Rendering|Material|SetMaterial _initmagicicon5 0 "/Game/MagicChipTexstures/MagicChipIcon/M_SPAWNUP_Mat.M_SPAWNUP_Mat"))
          (:NewEnumerator6
            (Rendering|Material|SetMaterial _initmagicicon5 0 "/Game/MagicChipTexstures/MagicChipIcon/M_SPAWNDOWN_Mat.M_SPAWNDOWN_Mat"))
          (:NewEnumerator7
            (Rendering|Material|SetMaterial _initmagicicon5 0 "/Game/MagicChipTexstures/MagicChipIcon/M_SPAWNRANDOM_Mat.M_SPAWNRANDOM_Mat")))))
    (else
      (Rendering|Material|SetMaterial (Variables|Default|GetInitMagicIcon5) 0 "/Engine/BasicShapes/BasicShapeMaterial.BasicShapeMaterial"))))

(fn SetChipValueSpawn
  (bind _magicchipinfo (Variables|Default|GetMagicChipInfo))
  (bind (_chipstatas _chipshape _chipmove _chipspecial _chipcondition _chipattribute _chipend _chipspawn) (Utilities|Struct|BreakS_MagicChipInfo_Ver2 _magicchipinfo))
  (bind (_spawntype _spawndirection) (Utilities|Struct|BreakS_ChipSpawn_Ver2 _chipspawn))
  (switch Utilities|FlowControl|Switch|SwitchonE_ChipSpawnDirectionType_Ver2 _spawndirection
    (:NewEnumerator1
      (Variables|Default|SetDTRowName "Spawn_Player_Front"))
    (:NewEnumerator2
      (Variables|Default|SetDTRowName "Spawn_Player_Back"))
    (:NewEnumerator3
      (Variables|Default|SetDTRowName "Spawn_Player_Left"))
    (:NewEnumerator4
      (Variables|Default|SetDTRowName "Spawn_Player_Front"))
    (:NewEnumerator5
      (Variables|Default|SetDTRowName "Spawn_Player_Top"))
    (:NewEnumerator6
      (Variables|Default|SetDTRowName "Spawn_Player_Under"))
    (:NewEnumerator7
      (Variables|Default|SetDTRowName "Spawn_Player_Random")))
  (bind _stamina (Class|BPIGetMagicChipDT|GetDTStamina(Message) (Variables|Default|GetChipSample) (Variables|Default|GetDTRowName)))
  (Variables|Default|SetInitStamina _stamina)
  (CallFunction|SetStamina)
  (Variables|Default|SetMagicChipInfo_Spawn (Utilities|Struct|MakeS_MagicChipInfo_Ver2 _chipstatas _chipshape _chipmove _chipspecial _chipcondition _chipattribute _chipend (Utilities|Struct|MakeS_ChipSpawn_Ver2 _spawntype _spawndirection (* (Variables|/Game/Scene/BP_MagicGameInstance.BP_MagicGameInstance_C|GetInitSliderValue_Spawn (Variables|Default|GetAsBPMagicGameInstance)) (Variables|/Game/BluePrints/BP_Chip.BP_Chip_C|GetDistance (Variables|Default|GetChipSample)))))))

(fn SetChipValueAttribte
  (bind _magicchipinfo (Variables|Default|GetMagicChipInfo))
  (bind (_chipstatas _chipshape _chipmove _chipspecial _chipcondition _chipattribute _chipend _chipspawn) (Utilities|Struct|BreakS_MagicChipInfo_Ver2 _magicchipinfo))
  (bind (_chipattributetype _attributedamege _isused_) (Utilities|Struct|BreakS_ChipAttribute_Ver2 _chipattribute))
  (switch Utilities|FlowControl|Switch|SwitchonE_ChipAttributeType_Ver2 _chipattributetype
    (:NewEnumerator0
      (Variables|Default|SetDTRowName "Attribute_Fire"))
    (:NewEnumerator1
      (Variables|Default|SetDTRowName "Attribute_Water"))
    (:NewEnumerator3
      (Variables|Default|SetDTRowName "Attribute_Lightning"))
    (:NewEnumerator4
      (Variables|Default|SetDTRowName "Attribute_Rock")))
  (bind _stamina (Class|BPIGetMagicChipDT|GetDTStamina(Message) (Variables|Default|GetChipSample) (Variables|Default|GetDTRowName)))
  (Variables|Default|SetInitStamina _stamina)
  (CallFunction|SetStamina)
  (Variables|Default|SetMagicChipInfo_Attribute (Utilities|Struct|MakeS_MagicChipInfo_Ver2 _chipstatas _chipshape _chipmove _chipspecial _chipcondition (Utilities|Struct|MakeS_ChipAttribute_Ver2 _chipattributetype (* (Variables|/Game/Scene/BP_MagicGameInstance.BP_MagicGameInstance_C|GetInitSliderValue_Attribute (Variables|Default|GetAsBPMagicGameInstance)) (Variables|/Game/BluePrints/BP_Chip.BP_Chip_C|GetAttributeDamege (Variables|Default|GetChipSample))) _isused_) _chipend _chipspawn)))

(fn GetWidget
  (bind _widgetref (Variables|Default|GetWidgetRef)
    (:then
      (return _widgetref))
    (:else)))