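; BP_ChipNone is the "none" variant of a magic chip actor, shown in the world as a billboard sprite.
; The SetChipNoneTexture event swaps the billboard sprite to the ChipNone texture.
; SetChipLocation rebuilds the ChipInfoVer2 struct, writing the actor's current location into its status data and carrying all other fields over unchanged.
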(event Custom|SetChipNoneTexture
  (Rendering|Components|Sprite|SetSprite (Variables|Default|GetBillboard) (Variables|Default|GetChipNoneTexture)))

(fn ConstructionScript)

(fn SetChipLocation
  (Variables|Default|SetChipInfo_Ver2 (Utilities|Struct|MakeS_MagicChipInfo_Ver2 (Utilities|Struct|MakeS_ChipStatas_Ver2 (.ChipName (Utilities|Struct|BreakS_ChipStatas_Ver2 (.ChipStatas (Utilities|Struct|BreakS_MagicChipInfo_Ver2 (Variables|Default|GetChipInfo_Ver2))))) (.ChipDescription (Utilities|Struct|BreakS_ChipStatas_Ver2 (.ChipStatas (Utilities|Struct|BreakS_MagicChipInfo_Ver2 (Variables|Default|GetChipInfo_Ver2))))) (.ChipIcon (Utilities|Struct|BreakS_ChipStatas_Ver2 (.ChipStatas (Utilities|Struct|BreakS_MagicChipInfo_Ver2 (Variables|Default|GetChipInfo_Ver2))))) (.CastTime (Utilities|Struct|BreakS_ChipStatas_Ver2 (.ChipStatas (Utilities|Struct|BreakS_MagicChipInfo_Ver2 (Variables|Default|GetChipInfo_Ver2))))) (.ChipDamege (Utilities|Struct|BreakS_ChipStatas_Ver2 (.ChipStatas (Utilities|Struct|BreakS_MagicChipInfo_Ver2 (Variables|Default|GetChipInfo_Ver2))))) (.ChipType (Utilities|Struct|BreakS_ChipStatas_Ver2 (.ChipStatas (Utilities|Struct|BreakS_MagicChipInfo_Ver2 (Variables|Default|GetChipInfo_Ver2))))) (.IsBad? (Utilities|Struct|BreakS_ChipStatas_Ver2 (.ChipStatas (Utilities|Struct|BreakS_MagicChipInfo_Ver2 (Variables|Default|GetChipInfo_Ver2))))) (.ChipNumber (Utilities|Struct|BreakS_ChipStatas_Ver2 (.ChipStatas (Utilities|Struct|BreakS_MagicChipInfo_Ver2 (Variables|Default|GetChipInfo_Ver2))))) (Transformation|GetActorLocation)) (.ChipShape (Utilities|Struct|BreakS_MagicChipInfo_Ver2 (Variables|Default|GetChipInfo_Ver2))) (.ChipMove (Utilities|Struct|BreakS_MagicChipInfo_Ver2 (Variables|Default|GetChipInfo_Ver2))) (.ChipSpecial (Utilities|Struct|BreakS_MagicChipInfo_Ver2 (Variables|Default|GetChipInfo_Ver2))) (.ChipIf (Utilities|Struct|BreakS_MagicChipInfo_Ver2 (Variables|Default|GetChipInfo_Ver2))) (.ChipCondition (Utilities|Struct|BreakS_MagicChipInfo_Ver2 (Variables|Default|GetChipInfo_Ver2))) (.ChipAttribute (Utilities|Struct|BreakS_MagicChipInfo_Ver2 (Variables|Default|GetChipInfo_Ver2))) (.ChipEnd (Utilities|Struct|BreakS_MagicChipInfo_Ver2 (Variables|Default|GetChipInfo_Ver2))) (.ChipSpawn (Utilities|Struct|BreakS_MagicChipInfo_Ver2 (Variables|Default|GetChipInfo_Ver2))) (.ChipValue (Utilities|Struct|BreakS_MagicChipInfo_Ver2 (Variables|Default|GetChipInfo_Ver2))))))