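; BP_Colosseum manages a combat stage, tracking remaining enemies and loading the Clear1_Bar level once all are defeated.
; On BeginPlay it hands itself to every BP_Enemy_Base, counts them, and stores the level name in BP_MagicGameInstance.
; EnemyCount and AddEnemy adjust the count; reaching zero triggers brief slow motion via global time dilation before the delayed level change.
; A NotPaused function unpauses the game.
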(event Custom|EnemyCount
  (Variables|Default|SetAllEnemy (- (Variables|Default|GetAllEnemy) 1))
  (if (<= (Variables|Default|GetAllEnemy) 0)
    (Utilities|FlowControl|Sequence
      (:then_0
        (Utilities|FlowControl|Delay 3.0)
        (Game|OpenLevel(byObjectReference) "/Game/Level/Clear1_Bar.Clear1_Bar"))
      (:then_1
        (Utilities|Time|SetGlobalTimeDilation 0.2))
      (:then_2
        (Utilities|FlowControl|Delay 0.5)
        (Utilities|Time|SetGlobalTimeDilation 1.0)))))

(event Custom|AddEnemy
  (Variables|Default|SetAllEnemy (+ (Variables|Default|GetAllEnemy) 1)))

(event EventBeginPlay
  (Utilities|FlowControl|Sequence
    (:then_0
      (bind _outactors (Actor|GetAllActorsOfClass "/Game/Enemy/Enemy_Sin_Test/BP_Enemy_Base.BP_Enemy_Base_C"))
      (for _array_element _outactors
        (Variables|/Game/Enemy/Enemy_Sin_Test/BP_Enemy_Base.BP_Enemy_Base_C|SetColosseum _array_element self))
      (bind _output_get (Variables|Default|SetOut%20Actors _outactors))
      (Variables|Default|SetAllEnemy (Utilities|Array|Length _output_get)))
    (:then_1
      (bind _returnvalue (Game|GetCurrentLevelName true))
      (bind _asbp_magic_game_instance (Utilities|Casting|CastToBP_MagicGameInstance (Game|GetGameInstance)))
      (Variables|/Game/Scene/BP_MagicGameInstance.BP_MagicGameInstance_C|Setstagename _asbp_magic_game_instance _returnvalue))))

(fn ConstructionScript)

(fn NotPaused
  (Game|SetGamePaused false))