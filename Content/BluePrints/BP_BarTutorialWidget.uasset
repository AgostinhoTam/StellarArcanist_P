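; Tutorial trigger actor that shows a tutorial widget while something overlaps its box, likely for a bar area given the asset name.
; On BeginPlay it creates its own WBP_Tutorial for the first player controller and adds it to the viewport.
; Overlap start clears the widget held by WidgetConnection, then switches its own to TutorialWidget; overlap end clears its own.
; The overlap events do not filter which actor triggers them.
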(event OnComponentBeginOverlap(Box)
  (params (OverlappedComponent :type Primitive%20Component%20Object%20Reference) (OtherActor :type Actor%20Object%20Reference) (OtherComp :type Primitive%20Component%20Object%20Reference) (OtherBodyIndex :type Integer) (bFromSweep :type Boolean) (SweepResult :type Hit%20Result%20Structure%20%28by%20ref%29))
  (Default|ClearWidget (Variables|BP_BarTutorialWidget_C|GetWidgetRef (Variables|Default|GetWidgetConnection)))
  (Default|SwitchWidget (Variables|Default|GetWidgetRef) (Variables|Default|GetTutorialWidget)))

(event OnComponentEndOverlap(Box)
  (params (OverlappedComponent :type Primitive%20Component%20Object%20Reference) (OtherActor :type Actor%20Object%20Reference) (OtherComp :type Primitive%20Component%20Object%20Reference) (OtherBodyIndex :type Integer))
  (Default|ClearWidget (Variables|Default|GetWidgetRef)))

(event EventBeginPlay
  (bind _returnvalue (UserInterface|CreateWidget "/Game/Widget/Tutorial/WBP_Tutorial.WBP_Tutorial_C" (Game|GetPlayerController 0)))
  (bind _output_get (Variables|Default|SetWidgetRef _returnvalue))
  (UserInterface|Viewport|AddtoViewport _output_get 0))

(fn ConstructionScript)