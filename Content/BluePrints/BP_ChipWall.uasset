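; BP_ChipWall is a board that turns the BP_Chip actors fitted on it into an ordered magic sequence with total cast time and stamina cost.
; ChipQuickSave gathers fitted chips overlapping its Box.
; ChipSave orders their info by Row, then TimeStart, and sums both costs.
; The ordering is a selection sort that flags each picked chip with IsSetMagicInfo, clearing all flags before each run.
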(event OnComponentBeginOverlap(Box)
  (params (OverlappedComponent :type Primitive%20Component%20Object%20Reference) (OtherActor :type Actor%20Object%20Reference) (OtherComp :type Primitive%20Component%20Object%20Reference) (OtherBodyIndex :type Integer) (bFromSweep :type Boolean) (SweepResult :type Hit%20Result%20Structure%20%28by%20ref%29)))

(event OnComponentEndOverlap(Box)
  (params (OverlappedComponent :type Primitive%20Component%20Object%20Reference) (OtherActor :type Actor%20Object%20Reference) (OtherComp :type Primitive%20Component%20Object%20Reference) (OtherBodyIndex :type Integer)))

(event OnComponentHit(Box)
  (params (HitComponent :type Primitive%20Component%20Object%20Reference) (OtherActor :type Actor%20Object%20Reference) (OtherComp :type Primitive%20Component%20Object%20Reference) (NormalImpulse :type Vector :default "0, 0, 0") (Hit :type Hit%20Result%20Structure%20%28by%20ref%29)))

(event Custom|ChipQuickSave
  (Utilities|Array|Clear (Variables|Default|GetChipActor))
  (for _array_element (Collision|GetOverlappingActors (Variables|Default|GetBox) "/Game/BluePrints/BP_Chip.BP_Chip_C" :!class /Script/Engine.PrimitiveComponent)
    (bind _asbp_chip (Utilities|Casting|CastToBP_Chip _array_element))
    (if (Variables|/Game/BluePrints/BP_Chip.BP_Chip_C|GetisFit? _asbp_chip)
      (Utilities|Array|Add (Variables|Default|GetChipActor) _asbp_chip))))

(event Custom|ChipSave
  (CallFunction|SetChipOrderRow&Time)
  (Variables|Default|SetCastTime 0.0)
  (Variables|Default|SetStaminaCost 0.0)
  (for _array_element (Variables|Default|GetChipInfo_Ver2_Order)
    (Variables|Default|SetCastTime (+ (Variables|Default|GetCastTime) (.CastTime (Utilities|Struct|BreakS_ChipStatas_Ver2 (.ChipStatas (Utilities|Struct|BreakS_MagicChipInfo_Ver2 _array_element))))))
    (Variables|Default|SetStaminaCost (+ (Variables|Default|GetStaminaCost) (.Staminaconsumed (Utilities|Struct|BreakS_ChipStatas_Ver2 (.ChipStatas (Utilities|Struct|BreakS_MagicChipInfo_Ver2 _array_element))))))))

(event EventTick
  (params (DeltaSeconds :type Float%20%28single-precision%29)))

(fn ConstructionScript)

(fn SetChipOrderRow&Time
  (Utilities|Array|Clear (Variables|Default|GetChipInfo_Ver2_Order))
  (for _array_element (Variables|Default|GetChipActor)
    (Variables|/Game/BluePrints/BP_Chip.BP_Chip_C|SetisSetMagicInfo? _array_element false))
  (for _array_element_2 (Variables|Default|GetChipActor)
    (for (_array_element_3 _array_index) (Variables|Default|GetChipActor)
      (LocalVariables|SetArrayIndex_Origin _array_index)
      (LocalVariables|SetChipActorArrayIndex _array_element_3)
      (if (not (Variables|/Game/BluePrints/BP_Chip.BP_Chip_C|GetisSetMagicInfo? (LocalVariables|GetChipActorArrayIndex)))
        (Variables|Default|GetChipActor_OnceSave
          (:then
            (if (== (Variables|/Game/BluePrints/BP_Chip.BP_Chip_C|GetRow (LocalVariables|GetChipActorArrayIndex)) (Variables|/Game/BluePrints/BP_Chip.BP_Chip_C|GetRow (Variables|Default|GetChipActor_OnceSave)))
              (if (< (Variables|/Game/BluePrints/BP_Chip.BP_Chip_C|GetTime_Start (LocalVariables|GetChipActorArrayIndex)) (Variables|/Game/BluePrints/BP_Chip.BP_Chip_C|GetTime_Start (Variables|Default|GetChipActor_OnceSave)))
                (Variables|Default|SetChipActor_OnceSave (LocalVariables|GetChipActorArrayIndex)))
              (elif (< (Variables|/Game/BluePrints/BP_Chip.BP_Chip_C|GetRow (LocalVariables|GetChipActorArrayIndex)) (Variables|/Game/BluePrints/BP_Chip.BP_Chip_C|GetRow (Variables|Default|GetChipActor_OnceSave)))
                (Variables|Default|SetChipActor_OnceSave (LocalVariables|GetChipActorArrayIndex)))))
          (:else
            (Variables|Default|SetChipActor_OnceSave (LocalVariables|GetChipActorArrayIndex))))))
    (Variables|Default|GetChipActor_OnceSave
      (:then
        (Variables|/Game/BluePrints/BP_Chip.BP_Chip_C|SetisSetMagicInfo? (Variables|Default|GetChipActor_OnceSave) true)
        (Utilities|Array|Add (Variables|Default|GetChipInfo_Ver2_Order) (Variables|/Game/BluePrints/BP_Chip.BP_Chip_C|GetChipInfo_Ver2 (Variables|Default|GetChipActor_OnceSave)))
        (Variables|Default|SetChipActor_OnceSave 0))
      (:else))))