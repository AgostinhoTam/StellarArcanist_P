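; Magic actor built from an array of chips that define its mesh and behavior, destroying itself about six seconds after it starts ticking.
; SetChipInfo takes the mesh from the first chip and converts movement chips into offsets along the player controller's forward or right vector, scaled by speed.
; Tick walks the chips in order, applying movement offsets, while unfinished Delay chips count frames and break the loop to hold back later chips.
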(event Custom|SetChipInfo
  (params (ChipInfo :type Array%20of%20S%20Magic%20Chip%20Info%20Structures))
  ;[1 1 1] メッシュ入れてる
  (Variables|Default|SetChipInfo ChipInfo)
  (if (Math|Conversions|ToBoolean(Integer) (Utilities|Array|Length (Variables|Default|GetChipInfo)))
    (Components|StaticMesh|SetStaticMesh (Variables|Default|GetStaticMesh) (.3dtexture (Utilities|Array|Get(acopy) (Variables|Default|GetChipInfo))))
    (bind (_array_element _array_index) (Utilities|Array|ForEachLoopwithBreak (Variables|Default|GetChipInfo))
      (:LoopBody
        (switch Utilities|FlowControl|Switch|SwitchonE_ChipType (.chiptype _array_element)
          (:NewEnumerator1
            (CallFunction|SetMoveDirectoion (.movedirection _array_element) _array_index (.chiptype _array_element) (.movespeed _array_element))))))))

(event EventTick
  (params (DeltaSeconds :type Float%20%28single-precision%29))
  (bind (_array_element _array_index) (Utilities|Array|ForEachLoopwithBreak (Variables|Default|GetChipInfo) :!label _label)
    (:LoopBody
      (switch Utilities|FlowControl|Switch|SwitchonE_ChipType (.chiptype _array_element)
        (:NewEnumerator1
          (Transformation|SetActorLocation (+ (Transformation|GetActorLocation) (.movelocation _array_element)) false false))
        (:NewEnumerator3
          (switch Utilities|FlowControl|Switch|SwitchonE_ChipSpecial (.chipspecial _array_element)
            (:NewEnumerator1
              (if (not (.isused? _array_element))
                (Utilities|Array|SetArrayElem (Variables|Default|GetChipInfo) _array_index (Utilities|Struct|MakeS_MagicChipInfo "None" "" (.chiptype _array_element) "NewEnumerator2" 0 0.0 0.0 0 "NewEnumerator0" false true 0.0 "0.000000,0.000000,0.000000" "NewEnumerator0" (.chipspecial _array_element) (.chipspecialvalue _array_element) (.isused? _array_element) (stale _result)))
                (if (== (.delaycount (Utilities|Array|Get(acopy) (Variables|Default|GetChipInfo) _array_index)) (.chipspecialvalue (Utilities|Array|Get(acopy) (Variables|Default|GetChipInfo) _array_index)))
                  (Utilities|Array|SetArrayElem (Variables|Default|GetChipInfo) _array_index (Utilities|Struct|MakeS_MagicChipInfo "None" "" (.chiptype _array_element) "NewEnumerator2" 0 0.0 0.0 0 "NewEnumerator0" false true 0.0 "0.000000,0.000000,0.000000" "NewEnumerator0" (.chipspecial _array_element) (.chipspecialvalue _array_element) true (.delaycount _array_element)))
                  (else
                    (bind _result (Math|Integer|IncrementInt (.delaycount (Utilities|Array|Get(acopy) (Variables|Default|GetChipInfo) _array_index)))
                      (:%20%20
                        (goto _label Break)))))))))))
    (:Completed
      (Utilities|FlowControl|Delay 1.0)
      (CallFunction|PrintStructureNum)
      (Utilities|FlowControl|Delay 5.0)
      (Actor|DestroyActor))))

(event EventBeginPlay)

(fn ConstructionScript)

(fn PrintStructureNum
  (Development|PrintString (Utilities|String|ToString(Integer) (Utilities|Array|Length (Variables|Default|GetChipInfo))) true true "(R=0.000000,G=0.660000,B=1.000000,A=1.000000)" 1.0)
  (Development|PrintString "-----------要素数----------" true true "(R=0.000000,G=0.660000,B=1.000000,A=1.000000)" 1.0))

(fn SetMoveDirectoion
  (params (MoveDirection :type E_ChipMoveDirection%20Enum :default "NewEnumerator0") (ChipIndex :type Integer) (Type :type E_ChipType%20Enum :default "NewEnumerator0") (MoveSpeed :type Float%20%28double-precision%29))
  (switch Utilities|FlowControl|Switch|SwitchonE_ChipMoveDirection MoveDirection
    (:NewEnumerator0
      ;[1 1 1] 前方処理
      (Utilities|Array|SetArrayElem (Variables|Default|GetChipInfo) ChipIndex (Utilities|Struct|MakeS_MagicChipInfo "None" "" Type "NewEnumerator2" 0 0.0 0.0 0 "NewEnumerator0" false true 0.0 (* (Transformation|GetActorForwardVector (Game|GetPlayerController 0)) MoveSpeed) "NewEnumerator1" "NewEnumerator0" 0.0 false 0)))
    (:NewEnumerator3
      ;[1 1 1] 右方向処理
      (Utilities|Array|SetArrayElem (Variables|Default|GetChipInfo) ChipIndex (Utilities|Struct|MakeS_MagicChipInfo "None" "" Type "NewEnumerator2" 0 0.0 0.0 0 "NewEnumerator0" false true 0.0 (* (Transformation|GetActorRightVector (Game|GetPlayerController 0)) MoveSpeed) "NewEnumerator4" "NewEnumerator0" 0.0 false 0)))))

(fn ActionSpecial
  (params (ChipSpecial :type E_ChipSpecial%20Enum :default "NewEnumerator0") (ChipIndex :type Integer) (ChipType :type E_ChipType%20Enum :default "NewEnumerator0"))
  (switch Utilities|FlowControl|Switch|SwitchonE_ChipSpecial ChipSpecial))

(fn ActionSpecialDelay
  (params (DelayTime :type Float%20%28double-precision%29) (IsUsed? :type Boolean) (ChipIndex :type Integer) (Type :type E_ChipType%20Enum :default "NewEnumerator0") (Special :type E_ChipSpecial%20Enum :default "NewEnumerator0"))
  (Utilities|Array|SetArrayElem (Variables|Default|GetChipInfo) ChipIndex (Utilities|Struct|MakeS_MagicChipInfo "None" "" Type "NewEnumerator2" 0 0.0 0.0 0 "NewEnumerator0" false true 0.0 "0.000000,0.000000,0.000000" "NewEnumerator4" Special 0.0 true 0))
  (return))