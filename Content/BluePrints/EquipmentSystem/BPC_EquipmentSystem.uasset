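; Equipment system component that lets the player pick up items and stores their data.
; On IA_Interact, it sphere-traces WorldDynamic objects from player character 0 toward a point ahead of and below it.
; A hit BP_Item has its ItemData appended to ItemSlots through AddWeapon, then the actor is destroyed.
; AddWeapon is a plain array add, with no slot limit or equip logic.
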(event Input|EnhancedActionEvents|EnhancedInputActionIA_Interact
  (params (ActionValue :type Boolean) (ElapsedSeconds :type Float%20%28double-precision%29) (TriggeredSeconds :type Float%20%28double-precision%29) (InputAction :type Input%20Action%20Object%20Reference :default "/Game/ThirdPerson/Input/Actions/IA_Interact.IA_Interact"))
  (bind _returnvalue (Game|GetPlayerCharacter 0))
  (bind _rootcomponent (Variables|/Script/Engine.Actor|GetRootComponent _returnvalue))
  (bind _returnvalue_2 (Transformation|GetWorldLocation _rootcomponent))
  (:Started
    (bind (_outhit _returnvalue_3) (Collision|SphereTraceForObjects _returnvalue_2 (- (+ _returnvalue_2 (* (Math|Vector|GetForwardVector (Transformation|GetWorldRotation _rootcomponent)) 1e+02)) "0.000000,0.000000,100.000000") 5e+01 (Utilities|Array|MakeArray "ObjectTypeQuery2") false 0 "None"))
    (if _returnvalue_3
      (bind _asbp_item (Utilities|Casting|CastToBP_Item (.HitActor (Collision|BreakHitResult _outhit))))
      (CallFunction|AddWeapon (Variables|/Game/BluePrints/EquipmentSystem/BP_Item.BP_Item_C|GetItemData _asbp_item))
      (Actor|DestroyActor _asbp_item))))

(event EventBeginPlay)

(event EventTick
  (params (DeltaSeconds :type Float%20%28single-precision%29)))

(fn AddWeapon
  (params (NewItem :type S%20Slots%20Structure%20%28by%20ref%29))
  (Utilities|Array|Add (Variables|Default|GetItemSlots) NewItem))