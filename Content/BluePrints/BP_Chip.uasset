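; BP_Chip is a placeable magic chip actor that holds one spell component's data and shows its icon, value and option sprites.
; Fitting it into a BP_ChipFrame, also via overlap, records its row and start time.
; Changing the time index on Movement or Homing chips stacks or removes BP_ChipNone actors along Z, which follow the chip.
; Edits to value, timing or position rebuild the chip's info struct, scaling size, speed or distance by type.
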(event OnComponentBeginOverlap(TachBox)
  (params (OverlappedComponent :type Primitive%20Component%20Object%20Reference) (OtherActor :type Actor%20Object%20Reference) (OtherComp :type Primitive%20Component%20Object%20Reference) (OtherBodyIndex :type Integer) (bFromSweep :type Boolean) (SweepResult :type Hit%20Result%20Structure%20%28by%20ref%29))
  ;[1 1 1] チップがロードで再展開された後にフレームにはめる処理
  (bind _asbp_chip_frame (Utilities|Casting|CastToBP_ChipFrame OtherActor))
  (CallFunction|SetChipinFrame _asbp_chip_frame))

(event Custom|SetChipData
  (params (MagicChipInfo :type S%20Magic%20Chip%20Info%20Ver%202%20Structure))
  ;[1 1 1] チップをActorとして作成
  (Variables|Default|SetChipInfo_Ver2 MagicChipInfo)
  (bind _returnvalue (Rendering|Material|CreateDynamicMaterialInstance (Variables|Default|GetChip) 0 "/Game/MagicChipMaterial/M_ChipMaterial.M_ChipMaterial" "M_MoveBack" :!class /Script/Engine.PrimitiveComponent))
  (Rendering|Material|SetTextureParameterValue _returnvalue "ChipTexture" (.ChipIcon (Utilities|Struct|BreakS_ChipStatas_Ver2 (.ChipStatas (Utilities|Struct|BreakS_MagicChipInfo_Ver2 (Variables|Default|GetChipInfo_Ver2))))))
  (CallFunction|SetChipValueOption)
  (bind _output_get (Variables|Default|SetTimeIndex (.TimeEnd (Utilities|Struct|BreakS_ChipStatas_Ver2 (.ChipStatas (Utilities|Struct|BreakS_MagicChipInfo_Ver2 (Variables|Default|GetChipInfo_Ver2)))))))
  (for _index (range 0 (Math|Float|Truncate _output_get))
    (CallFunction|SetSpawnChipNeneEvent)
    (CallFunction|SetChipValueEvent))
  (switch Utilities|FlowControl|Switch|SwitchonE_ChipType_Ver2 (.ChipType (Utilities|Struct|BreakS_ChipStatas_Ver2 (.ChipStatas (Utilities|Struct|BreakS_MagicChipInfo_Ver2 (Variables|Default|GetChipInfo_Ver2)))))
    (:NewEnumerator4
      _)
    (:NewEnumerator6
      _)
    (:NewEnumerator10
      _))
  (Development|SetHiddeninGame (Variables|Default|GetValueText) true false))

(event Custom|SetTimeStart
  (params (ChipFrame :type Actor%20Object%20Reference))
  ;[1 1 1] TimeStartの設定
  (bind _asbp_chip_frame (Utilities|Casting|CastToBP_ChipFrame ChipFrame))
  (Variables|Default|SetTime_Start (Variables|/Game/BluePrints/BP_ChipFrame.BP_ChipFrame_C|GetTime _asbp_chip_frame))
  (CallFunction|SetChipTimeMoveStart&End))

(event Custom|SetRow
  (params (ChipFrame :type Actor%20Object%20Reference))
  ;[1 1 1] Rowの設定
  (bind _asbp_chip_frame (Utilities|Casting|CastToBP_ChipFrame ChipFrame))
  (Variables|Default|SetRow (Variables|/Game/BluePrints/BP_ChipFrame.BP_ChipFrame_C|GetRow _asbp_chip_frame)))

(event Custom|SetDestory_ChipNone
  ;[1 1 1] Noneチップを削除
  (for _array_element (Variables|Default|GetChipNone)
    (Actor|DestroyActor _array_element)))

(event Custom|SetChipValueEvent
  ;[1 1 1] 数値を変更した時に呼ばれる
  (CallFunction|SetChipValue))

(event Custom|SetSpawnChipNeneEvent
  ;[1 1 1] 時間を変更した時に呼ばれる
  (CallFunction|SpawnChipNone)
  (CallFunction|SetChipTimeMoveStart&End))

(event Custom|SetPlusTimeIndexEvent
  (bind _chipinfo_ver2 (Variables|Default|GetChipInfo_Ver2))
  (bind (_chipstatas _chipshape _chipmove _chipspecial) (Utilities|Struct|BreakS_MagicChipInfo_Ver2 _chipinfo_ver2))
  ;[1 1 1] ChipのIndexを設定
  (switch Utilities|FlowControl|Switch|SwitchonE_ChipType_Ver2 (.ChipType (Utilities|Struct|BreakS_ChipStatas_Ver2 _chipstatas))
    (:NewEnumerator1
      _)
    (:NewEnumerator3
      (switch Utilities|FlowControl|Switch|SwitchonE_ChipSpecialType_Ver2 (.ChipSpecialType (Utilities|Struct|BreakS_ChipSpecial_Ver2 _chipspecial))
        (:NewEnumerator3
          _))))
  (if (> (Variables|Default|GetTimeIndex) 1.0)
    (Variables|Default|SetTimeIndex (+ (Variables|Default|GetTimeIndex) -1.0))
    (CallFunction|SetSpawnChipNeneEvent)))

(event Custom|SetMinasTimeIndexEvent
  (bind _chipinfo_ver2 (Variables|Default|GetChipInfo_Ver2))
  (bind (_chipstatas _chipshape _chipmove _chipspecial) (Utilities|Struct|BreakS_MagicChipInfo_Ver2 _chipinfo_ver2))
  ;[1 1 1] ChipのIndexを設定
  (switch Utilities|FlowControl|Switch|SwitchonE_ChipType_Ver2 (.ChipType (Utilities|Struct|BreakS_ChipStatas_Ver2 _chipstatas))
    (:NewEnumerator1
      _)
    (:NewEnumerator3
      (switch Utilities|FlowControl|Switch|SwitchonE_ChipSpecialType_Ver2 (.ChipSpecialType (Utilities|Struct|BreakS_ChipSpecial_Ver2 _chipspecial))
        (:NewEnumerator3
          _))))
  (if (< (Variables|Default|GetTimeIndex) 11.0)
    (Variables|Default|SetTimeIndex (+ (Variables|Default|GetTimeIndex) 1.0))
    (CallFunction|SetSpawnChipNeneEvent)))

(event EventSetChipinFrame
  (params (ChipFrameActor :type Actor%20Object%20Reference))
  ;[1 1 1] チップを枠にはめたときの処理
  (Variables|Default|SetisFit? true)
  (CallFunction|SetTimeStart ChipFrameActor)
  (CallFunction|SetRow ChipFrameActor))

(event EventTick
  (params (DeltaSeconds :type Float%20%28single-precision%29))
  (if (not (Class|KismetMathLibrary|EqualExactlyVectorVector (.ActorLocation (Utilities|Struct|BreakS_ChipStatas_Ver2 (.ChipStatas (Utilities|Struct|BreakS_MagicChipInfo_Ver2 (Variables|Default|GetChipInfo_Ver2))))) (Transformation|GetActorLocation)))
    (CallFunction|SetChipLocation)
    (CallFunction|SetChipLocationChipNone)))

(event EventSetChipOutFrame
  ;[1 1 1] チップを枠から取り出した時の処理
  (Variables|Default|SetisFit? false))

(event EventChipSelect
  ;[1 1 1] Deleteアイコンを表示
  (Rendering|SetVisibility (Variables|Default|GetDeleteIcon) true false))

(event EventChipNoSelect
  ;[1 1 1] Deleteアイコンを非表示
  (Rendering|SetVisibility (Variables|Default|GetDeleteIcon) false false))

(fn ConstructionScript)

(fn SetChipLocation
  (Variables|Default|SetChipInfo_Ver2 (Utilities|Struct|MakeS_MagicChipInfo_Ver2 (Utilities|Struct|MakeS_ChipStatas_Ver2 (.ChipName (Utilities|Struct|BreakS_ChipStatas_Ver2 (.ChipStatas (Utilities|Struct|BreakS_MagicChipInfo_Ver2 (Variables|Default|GetChipInfo_Ver2))))) (.ChipDescription (Utilities|Struct|BreakS_ChipStatas_Ver2 (.ChipStatas (Utilities|Struct|BreakS_MagicChipInfo_Ver2 (Variables|Default|GetChipInfo_Ver2))))) (.ChipIcon (Utilities|Struct|BreakS_ChipStatas_Ver2 (.ChipStatas (Utilities|Struct|BreakS_MagicChipInfo_Ver2 (Variables|Default|GetChipInfo_Ver2))))) (.CastTime (Utilities|Struct|BreakS_ChipStatas_Ver2 (.ChipStatas (Utilities|Struct|BreakS_MagicChipInfo_Ver2 (Variables|Default|GetChipInfo_Ver2))))) (.ChipDamege (Utilities|Struct|BreakS_ChipStatas_Ver2 (.ChipStatas (Utilities|Struct|BreakS_MagicChipInfo_Ver2 (Variables|Default|GetChipInfo_Ver2))))) (.ChipType (Utilities|Struct|BreakS_ChipStatas_Ver2 (.ChipStatas (Utilities|Struct|BreakS_MagicChipInfo_Ver2 (Variables|Default|GetChipInfo_Ver2))))) (.IsBad? (Utilities|Struct|BreakS_ChipStatas_Ver2 (.ChipStatas (Utilities|Struct|BreakS_MagicChipInfo_Ver2 (Variables|Default|GetChipInfo_Ver2))))) (.ChipNumber (Utilities|Struct|BreakS_ChipStatas_Ver2 (.ChipStatas (Utilities|Struct|BreakS_MagicChipInfo_Ver2 (Variables|Default|GetChipInfo_Ver2))))) (Transformation|GetActorLocation) (.TimeStart (Utilities|Struct|BreakS_ChipStatas_Ver2 (.ChipStatas (Utilities|Struct|BreakS_MagicChipInfo_Ver2 (Variables|Default|GetChipInfo_Ver2))))) (.TimeEnd (Utilities|Struct|BreakS_ChipStatas_Ver2 (.ChipStatas (Utilities|Struct|BreakS_MagicChipInfo_Ver2 (Variables|Default|GetChipInfo_Ver2))))) (.Staminaconsumed (Utilities|Struct|BreakS_ChipStatas_Ver2 (.ChipStatas (Utilities|Struct|BreakS_MagicChipInfo_Ver2 (Variables|Default|GetChipInfo_Ver2)))))) (.ChipShape (Utilities|Struct|BreakS_MagicChipInfo_Ver2 (Variables|Default|GetChipInfo_Ver2))) (.ChipMove (Utilities|Struct|BreakS_MagicChipInfo_Ver2 (Variables|Default|GetChipInfo_Ver2))) (.ChipSpecial (Utilities|Struct|BreakS_MagicChipInfo_Ver2 (Variables|Default|GetChipInfo_Ver2))) (.ChipCondition (Utilities|Struct|BreakS_MagicChipInfo_Ver2 (Variables|Default|GetChipInfo_Ver2))) (.ChipAttribute (Utilities|Struct|BreakS_MagicChipInfo_Ver2 (Variables|Default|GetChipInfo_Ver2))) (.ChipEnd (Utilities|Struct|BreakS_MagicChipInfo_Ver2 (Variables|Default|GetChipInfo_Ver2))) (.ChipSpawn (Utilities|Struct|BreakS_MagicChipInfo_Ver2 (Variables|Default|GetChipInfo_Ver2))))))

(fn SpawnChipNone
  (bind _returnvalue (Transformation|GetActorLocation))
  (bind _chipinfo_ver2 (Variables|Default|GetChipInfo_Ver2))
  (bind _chipnone (Variables|Default|GetChipNone))
  (bind _chipnone_2 (Variables|Default|GetChipNone))
  (bind (_chipstatas _chipshape _chipmove _chipspecial) (Utilities|Struct|BreakS_MagicChipInfo_Ver2 _chipinfo_ver2))
  (bind (_x _y _z) (Math|Vector|BreakVector _returnvalue))
  (if (!= (Variables|Default|GetTimeIndex) (Variables|Default|GetSpawnChipNoneIndex))
    (if (> (Variables|Default|GetTimeIndex) (Variables|Default|GetSpawnChipNoneIndex))
      (switch Utilities|FlowControl|Switch|SwitchonE_ChipType_Ver2 (.ChipType (Utilities|Struct|BreakS_ChipStatas_Ver2 _chipstatas))
        (:NewEnumerator1
          _)
        (:NewEnumerator3
          (switch Utilities|FlowControl|Switch|SwitchonE_ChipSpecialType_Ver2 (.ChipSpecialType (Utilities|Struct|BreakS_ChipSpecial_Ver2 _chipspecial))
            (:NewEnumerator3
              _))))
      (bind _returnvalue_2 (Game|SpawnActorfromClass :Class "/Game/BluePrints/BP_ChipNone.BP_ChipNone_C" :SpawnTransform (Math|Transform|MakeTransform (Math|Vector|MakeVector _x _y (+ _z (* (+ (Variables|Default|GetSpawnChipNoneIndex) 1.0) (Variables|Default|GetChipNoneDistance)))) "0, 0, 0" "1.000000,1.000000,1.000000") :CollisionHandlingOverride "Undefined" :TransformScaleMethod "MultiplyWithRoot" :Instigator 0))
      (Utilities|Array|Add (Variables|Default|GetChipNone) _returnvalue_2)
      (Variables|/Game/BluePrints/BP_ChipNone.BP_ChipNone_C|SetChipNoneTexture _returnvalue_2 "/Game/MagicChipTexstures/T_Move.T_Move")
      (Default|SetChipNoneTexture _returnvalue_2)
      (Variables|Default|SetSpawnChipNoneIndex (+ (Variables|Default|GetSpawnChipNoneIndex) 1.0))
      (else
        (Actor|DestroyActor (Utilities|Array|Get(acopy) _chipnone (- (Utilities|Array|Length _chipnone) 1)))
        (Utilities|Array|RemoveIndex _chipnone_2 (- (Utilities|Array|Length _chipnone_2) 1))
        (Variables|Default|SetSpawnChipNoneIndex (- (Variables|Default|GetSpawnChipNoneIndex) 1.0))))))

(fn SetChipLocationChipNone
  (bind _returnvalue (Transformation|GetActorLocation))
  (bind (_x _y _z) (Math|Vector|BreakVector _returnvalue))
  (for (_array_element _array_index) (Variables|Default|GetChipNone)
    (Transformation|SetActorLocation _array_element (Math|Vector|MakeVector _x _y (+ _z (* (+ _array_index 1) (Variables|Default|GetChipNoneDistance)))) false false)))

(fn SetChipValue
  (if (!= (Variables|Default|GetChipValue) (Variables|Default|GetChipValue_Record))
    (if (not (Variables|/Script/Engine.SceneComponent|GetbHiddenInGame (Variables|Default|GetValueText)))
      (Variables|Default|SetChipValue_Record (Variables|Default|GetChipValue))
      (switch Utilities|FlowControl|Switch|SwitchonE_ChipType_Ver2 (.ChipType (Utilities|Struct|BreakS_ChipStatas_Ver2 (.ChipStatas (Utilities|Struct|BreakS_MagicChipInfo_Ver2 (Variables|Default|GetChipInfo_Ver2)))))
        (:NewEnumerator0
          (CallFunction|SetChipValueShapeSize))
        (:NewEnumerator1
          (CallFunction|SetChipValueMoveSpeed))
        (:NewEnumerator3
          (CallFunction|SetChipValueSpecial))
        (:NewEnumerator9
          (CallFunction|SetChipValueSpawnDistance)))
      (CallFunction|SetChipValueTexture))))

(fn SetChipValueTexture
  (if (>= (Variables|Default|GetChipValue) 5.0)
    (if (== 5.0 (Variables|Default|GetChipValue)) :!label _label
      (Rendering|Components|Sprite|SetSprite (Variables|Default|GetValueText) "/Game/Textures/T_Number_05.T_Number_05")
      (elif (== 6.0 (Variables|Default|GetChipValue))
        (Rendering|Components|Sprite|SetSprite (Variables|Default|GetValueText) "/Game/Textures/T_Number_06.T_Number_06")
        (elif (== 7.0 (Variables|Default|GetChipValue))
          (Rendering|Components|Sprite|SetSprite (Variables|Default|GetValueText) "/Game/Textures/T_Number_07.T_Number_07")
          (elif (== 8.0 (Variables|Default|GetChipValue))
            (Rendering|Components|Sprite|SetSprite (Variables|Default|GetValueText) "/Game/Textures/T_Number_08.T_Number_08")
            (elif (== 9.0 (Variables|Default|GetChipValue))
              (Rendering|Components|Sprite|SetSprite (Variables|Default|GetValueText) "/Game/Textures/T_Number_09.T_Number_09")
              (elif (== 1e+01 (Variables|Default|GetChipValue))
                (Rendering|Components|Sprite|SetSprite (Variables|Default|GetValueText) "/Game/Textures/T_Number_10.T_Number_10")))))))
    (elif (== 0.0 (Variables|Default|GetChipValue))
      (Rendering|Components|Sprite|SetSprite (Variables|Default|GetValueText) "/Game/Textures/T_Number_0.T_Number_0")
      (elif (== 1.0 (Variables|Default|GetChipValue))
        (Rendering|Components|Sprite|SetSprite (Variables|Default|GetValueText) "/Game/Textures/T_Number_01.T_Number_01")
        (elif (== 2.0 (Variables|Default|GetChipValue))
          (Rendering|Components|Sprite|SetSprite (Variables|Default|GetValueText) "/Game/Textures/T_Number_02.T_Number_02")
          (elif (== 3.0 (Variables|Default|GetChipValue))
            (Rendering|Components|Sprite|SetSprite (Variables|Default|GetValueText) "/Game/Textures/T_Number_03.T_Number_03")
            (elif (== 4.0 (Variables|Default|GetChipValue))
              (Rendering|Components|Sprite|SetSprite (Variables|Default|GetValueText) "/Game/Textures/T_Number_04.T_Number_04")
              (else
                (goto _label)))))))))

(fn SetChipValueMoveSpeed
  (Variables|Default|SetChipInfo_Ver2 (Utilities|Struct|MakeS_MagicChipInfo_Ver2 (.ChipStatas (Utilities|Struct|BreakS_MagicChipInfo_Ver2 (Variables|Default|GetChipInfo_Ver2))) "(ChipShapeType_7_D0A7429B4E46D1984142D6AC1C6C09FC=NewEnumerator0,3DTexture_6_CB930A80470CAD92277DEA8DDF15240A=None,IsUsed?_9_A2720F424C1C437CA1F843921FF30AA5=False,size_13_6650CE4F43784BB2B0FF8381D09A033E=0.000000)" (Utilities|Struct|MakeS_ChipMove_Ver2 (.ChipMoveDirectionType (Utilities|Struct|BreakS_ChipMove_Ver2 (.ChipMove (Utilities|Struct|BreakS_MagicChipInfo_Ver2 (Variables|Default|GetChipInfo_Ver2))))) (* (Variables|Default|GetChipValue) (LocalVariables|GetSpeed)) (.MoveLocation (Utilities|Struct|BreakS_ChipMove_Ver2 (.ChipMove (Utilities|Struct|BreakS_MagicChipInfo_Ver2 (Variables|Default|GetChipInfo_Ver2)))))))))

(fn SetChipValueShapeSize
  (Variables|Default|SetChipInfo_Ver2 (Utilities|Struct|MakeS_MagicChipInfo_Ver2 (.ChipStatas (Utilities|Struct|BreakS_MagicChipInfo_Ver2 (Variables|Default|GetChipInfo_Ver2))) (Utilities|Struct|MakeS_ChipShape_Ver2 (.ChipShapeType (Utilities|Struct|BreakS_ChipShape_Ver2 (.ChipShape (Utilities|Struct|BreakS_MagicChipInfo_Ver2 (Variables|Default|GetChipInfo_Ver2))))) (.3DTexture (Utilities|Struct|BreakS_ChipShape_Ver2 (.ChipShape (Utilities|Struct|BreakS_MagicChipInfo_Ver2 (Variables|Default|GetChipInfo_Ver2))))) (.IsUsed? (Utilities|Struct|BreakS_ChipShape_Ver2 (.ChipShape (Utilities|Struct|BreakS_MagicChipInfo_Ver2 (Variables|Default|GetChipInfo_Ver2))))) (* (Variables|Default|GetChipValue) (Variables|Default|GetSize))))))

(fn SetChipValueSpawnDistance
  (Variables|Default|SetChipInfo_Ver2 (Utilities|Struct|MakeS_MagicChipInfo_Ver2 (.ChipStatas (Utilities|Struct|BreakS_MagicChipInfo_Ver2 (Variables|Default|GetChipInfo_Ver2))) "(ChipShapeType_7_D0A7429B4E46D1984142D6AC1C6C09FC=NewEnumerator0,3DTexture_6_CB930A80470CAD92277DEA8DDF15240A=None,IsUsed?_9_A2720F424C1C437CA1F843921FF30AA5=False,size_13_6650CE4F43784BB2B0FF8381D09A033E=0.000000)" "(ChipMoveDirectionType_10_4915AED94BCCB891B5A92BB92579A3AF=NewEnumerator0,MoveSpeed_5_78DA1AA94C4F84822D5877A8B97AD4FE=0.000000,MoveLocation_9_2809D0F64AB7CC2C411F049EBE2CC596=(X=0.000000,Y=0.000000,Z=0.000000))" "(ChipSpecialType_6_3B5EDCAA4D8FDA68DA74278DC55901C0=NewEnumerator0,ChipDelayTime_5_08E108864A90A42763E241AD80C519F0=(IsUsed?_1_9980ABC845E4CA130FCA5EB9BE1951E7=False,DelayTime_8_0308187F448978D8B3719C94E9EC06C6=0.000000,DelayCount_7_58DA77354FFB2DDC46B2898A19F6431D=0.000000),ChipHoming_17_A06A411141D02181C89CCC9557946E9D=(speed_2_A88FF88E431ED5AA8156C79F784BE226=0.000000,TargetActor_7_E3E1496B48DF1345A9251EB7C05C3A43=None,IsTargeted_9_52A0CFB6426CB83EB3D75FA70E4E117C=False,Location_13_1C6534A44DDD63FA4B9BA2B6D8E284AA=(X=0.000000,Y=0.000000,Z=0.000000)))" "(ConditionType_24_56697AE94C44CAB4EF60EF922AC8031D=NewEnumerator0,ConditionTime_32_3D353E9249536E9E44540FA5590C1303=(ConditionTimeType_9_3768C87E4CC6EA067621ADA414EF3E88=NewEnumerator0,TimeValue_5_9AA4464A488A3DD1A90FB381F75542D0=0.000000,TimeCount_12_26311640481FD74B385D83992938FB04=0.000000),IsUsed?_36_43BA177A46243C9315CA41AB6EAB9D2C=False,FlagChenged?_38_D4CFEC824F7999E2558252AB5BCC8FE7=False,ConditionHit_43_3A3F0AB24EBCB50B2DA8A39D3D517925=(ConditionHitType_19_3768C87E4CC6EA067621ADA414EF3E88=NewEnumerator0,KeepHit?_17_26311640481FD74B385D83992938FB04=False))" "(ChipAttributeType_2_CEDC4CEE443A86AD18D5FF82B0B73117=NewEnumerator2,AttributeDamege_5_DD56E1F94F4524348E86A698B49CDE2E=0.000000,IsUsed?_10_D986B5AC470A6AC0C0757B818FB141F0=False)" "(TypeEnd_3_A19BA0F14C23C24F8855CEB69952F3FB=NewEnumerator0,IsEnd?_6_D1C203774EC68415949859987A4209C2=False,Explosion_11_463CAF064194C8C6E7FA65928086DE1D=(Size_2_C0A98C40497D32613C183E870A236DA2=0.000000))" (Utilities|Struct|MakeS_ChipSpawn_Ver2 (.SpawnType (Utilities|Struct|BreakS_ChipSpawn_Ver2 (.ChipSpawn (Utilities|Struct|BreakS_MagicChipInfo_Ver2 (Variables|Default|GetChipInfo_Ver2))))) (.SpawnDirection (Utilities|Struct|BreakS_ChipSpawn_Ver2 (.ChipSpawn (Utilities|Struct|BreakS_MagicChipInfo_Ver2 (Variables|Default|GetChipInfo_Ver2))))) (* (Variables|Default|GetChipValue) (LocalVariables|Getdistance))))))

(fn SetChipTimeMoveStart&End
  (Variables|Default|SetChipInfo_Ver2 (Utilities|Struct|MakeS_MagicChipInfo_Ver2 (Utilities|Struct|MakeS_ChipStatas_Ver2 (.ChipName (Utilities|Struct|BreakS_ChipStatas_Ver2 (.ChipStatas (Utilities|Struct|BreakS_MagicChipInfo_Ver2 (Variables|Default|GetChipInfo_Ver2))))) (.ChipDescription (Utilities|Struct|BreakS_ChipStatas_Ver2 (.ChipStatas (Utilities|Struct|BreakS_MagicChipInfo_Ver2 (Variables|Default|GetChipInfo_Ver2))))) (.ChipIcon (Utilities|Struct|BreakS_ChipStatas_Ver2 (.ChipStatas (Utilities|Struct|BreakS_MagicChipInfo_Ver2 (Variables|Default|GetChipInfo_Ver2))))) (.CastTime (Utilities|Struct|BreakS_ChipStatas_Ver2 (.ChipStatas (Utilities|Struct|BreakS_MagicChipInfo_Ver2 (Variables|Default|GetChipInfo_Ver2))))) (.ChipDamege (Utilities|Struct|BreakS_ChipStatas_Ver2 (.ChipStatas (Utilities|Struct|BreakS_MagicChipInfo_Ver2 (Variables|Default|GetChipInfo_Ver2))))) (.ChipType (Utilities|Struct|BreakS_ChipStatas_Ver2 (.ChipStatas (Utilities|Struct|BreakS_MagicChipInfo_Ver2 (Variables|Default|GetChipInfo_Ver2))))) (.IsBad? (Utilities|Struct|BreakS_ChipStatas_Ver2 (.ChipStatas (Utilities|Struct|BreakS_MagicChipInfo_Ver2 (Variables|Default|GetChipInfo_Ver2))))) (.ChipNumber (Utilities|Struct|BreakS_ChipStatas_Ver2 (.ChipStatas (Utilities|Struct|BreakS_MagicChipInfo_Ver2 (Variables|Default|GetChipInfo_Ver2))))) (.ActorLocation (Utilities|Struct|BreakS_ChipStatas_Ver2 (.ChipStatas (Utilities|Struct|BreakS_MagicChipInfo_Ver2 (Variables|Default|GetChipInfo_Ver2))))) (Variables|Default|GetTime_Start) (+ (Variables|Default|GetTime_Start) (Variables|Default|GetTimeIndex)) (.Staminaconsumed (Utilities|Struct|BreakS_ChipStatas_Ver2 (.ChipStatas (Utilities|Struct|BreakS_MagicChipInfo_Ver2 (Variables|Default|GetChipInfo_Ver2)))))) (.ChipShape (Utilities|Struct|BreakS_MagicChipInfo_Ver2 (Variables|Default|GetChipInfo_Ver2))) (.ChipMove (Utilities|Struct|BreakS_MagicChipInfo_Ver2 (Variables|Default|GetChipInfo_Ver2))) (.ChipSpecial (Utilities|Struct|BreakS_MagicChipInfo_Ver2 (Variables|Default|GetChipInfo_Ver2))) (.ChipCondition (Utilities|Struct|BreakS_MagicChipInfo_Ver2 (Variables|Default|GetChipInfo_Ver2))) (.ChipAttribute (Utilities|Struct|BreakS_MagicChipInfo_Ver2 (Variables|Default|GetChipInfo_Ver2))) (.ChipEnd (Utilities|Struct|BreakS_MagicChipInfo_Ver2 (Variables|Default|GetChipInfo_Ver2))) (.ChipSpawn (Utilities|Struct|BreakS_MagicChipInfo_Ver2 (Variables|Default|GetChipInfo_Ver2))))))

(fn SetChipValueOption
  (bind _chipinfo_ver2 (Variables|Default|GetChipInfo_Ver2))
  (bind (_chipstatas _chipshape _chipmove _chipspecial) (Utilities|Struct|BreakS_MagicChipInfo_Ver2 _chipinfo_ver2))
  (switch Utilities|FlowControl|Switch|SwitchonE_ChipType_Ver2 (.ChipType (Utilities|Struct|BreakS_ChipStatas_Ver2 _chipstatas))
    (:NewEnumerator0
      (Rendering|Components|Sprite|SetSprite (Variables|Default|GetValueDataText) "/Game/Textures/T_SIZE.T_SIZE"))
    (:NewEnumerator1
      (Rendering|Components|Sprite|SetSprite (Variables|Default|GetValueDataText) "/Game/Textures/T_SPEED.T_SPEED" :!label _label))
    (:NewEnumerator3
      (switch Utilities|FlowControl|Switch|SwitchonE_ChipSpecialType_Ver2 (.ChipSpecialType (Utilities|Struct|BreakS_ChipSpecial_Ver2 _chipspecial))
        (:NewEnumerator3
          (goto _label))))
    (:NewEnumerator4
      (Development|SetHiddeninGame (Variables|Default|GetValueDataText) true false :!label _label_2))
    (:NewEnumerator5
      (goto _label_2))
    (:NewEnumerator6
      (goto _label_2))
    (:NewEnumerator7
      (goto _label_2))
    (:NewEnumerator9
      (Rendering|Components|Sprite|SetSprite (Variables|Default|GetValueDataText) "/Game/Textures/T_DISTANCE.T_DISTANCE"))
    (:NewEnumerator10
      (goto _label_2))))

(fn SetChipValueSpecial
  (switch Utilities|FlowControl|Switch|SwitchonE_ChipSpecialType_Ver2 (.ChipSpecialType (Utilities|Struct|BreakS_ChipSpecial_Ver2 (.ChipSpecial (Utilities|Struct|BreakS_MagicChipInfo_Ver2 (Variables|Default|GetChipInfo_Ver2)))))
    (:NewEnumerator3
      (CallFunction|SetChipValueSpecialHomingSpeed))))

(fn SetChipValueSpecialHomingSpeed
  (Variables|Default|SetChipInfo_Ver2 (Utilities|Struct|MakeS_MagicChipInfo_Ver2 (.ChipStatas (Utilities|Struct|BreakS_MagicChipInfo_Ver2 (Variables|Default|GetChipInfo_Ver2))) "(ChipShapeType_7_D0A7429B4E46D1984142D6AC1C6C09FC=NewEnumerator0,3DTexture_6_CB930A80470CAD92277DEA8DDF15240A=None,IsUsed?_9_A2720F424C1C437CA1F843921FF30AA5=False,size_13_6650CE4F43784BB2B0FF8381D09A033E=0.000000)" "(ChipMoveDirectionType_10_4915AED94BCCB891B5A92BB92579A3AF=NewEnumerator0,MoveSpeed_5_78DA1AA94C4F84822D5877A8B97AD4FE=0.000000,MoveLocation_9_2809D0F64AB7CC2C411F049EBE2CC596=(X=0.000000,Y=0.000000,Z=0.000000))" (Utilities|Struct|MakeS_ChipSpecial_Ver2 (.ChipSpecialType (Utilities|Struct|BreakS_ChipSpecial_Ver2 (.ChipSpecial (Utilities|Struct|BreakS_MagicChipInfo_Ver2 (Variables|Default|GetChipInfo_Ver2))))) "(IsUsed?_1_9980ABC845E4CA130FCA5EB9BE1951E7=False,DelayTime_8_0308187F448978D8B3719C94E9EC06C6=0.000000,DelayCount_7_58DA77354FFB2DDC46B2898A19F6431D=0.000000)" (Utilities|Struct|MakeS_Special_Homing_Ver2 (* (Variables|Default|GetChipValue) (LocalVariables|GetSpeed)) (.TargetActor (Utilities|Struct|BreakS_Special_Homing_Ver2 (.ChipHoming (Utilities|Struct|BreakS_ChipSpecial_Ver2 (.ChipSpecial (Utilities|Struct|BreakS_MagicChipInfo_Ver2 (Variables|Default|GetChipInfo_Ver2))))))) (.IsTargeted (Utilities|Struct|BreakS_Special_Homing_Ver2 (.ChipHoming (Utilities|Struct|BreakS_ChipSpecial_Ver2 (.ChipSpecial (Utilities|Struct|BreakS_MagicChipInfo_Ver2 (Variables|Default|GetChipInfo_Ver2))))))) (.Location (Utilities|Struct|BreakS_Special_Homing_Ver2 (.ChipHoming (Utilities|Struct|BreakS_ChipSpecial_Ver2 (.ChipSpecial (Utilities|Struct|BreakS_MagicChipInfo_Ver2 (Variables|Default|GetChipInfo_Ver2))))))))))))