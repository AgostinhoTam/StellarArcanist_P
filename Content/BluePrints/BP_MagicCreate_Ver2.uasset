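; Spell projectile actor that runs a player spell defined as an array of chips, with the first Shape chip supplying its mesh.
; SetChipInfo bakes movement chips into velocities from the player controller's axes or world up.
; Each Tick interprets enabled chips: movement shifts the actor, timed If conditions toggle IsBad on chips through End if, and End can spawn an explosion before destruction.
; A ten-second delay forces destruction; spawn positioning is stubbed.
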(event Custom|SetChipInfo
  (params (ChipInfo_Ver2 :type Array%20of%20S%20Magic%20Chip%20Info%20Ver%202%20Structures))
  (Variables|Default|SetChipInfo_Ver2 ChipInfo_Ver2)
  ;[1 1 1] メッシュの格納
  (switch Utilities|FlowControl|Switch|SwitchonE_ChipType_Ver2 (.ChipType (Utilities|Struct|BreakS_ChipStatas_Ver2 (.chipstatas (Utilities|Array|Get(acopy) (Variables|Default|GetChipInfo_Ver2)))))
    (:NewEnumerator0
      (Components|StaticMesh|SetStaticMesh (Variables|Default|GetStaticMesh) (.3DTexture (Utilities|Struct|BreakS_ChipShape_Ver2 (.chipshape (Utilities|Array|Get(acopy) (Variables|Default|GetChipInfo_Ver2))))))
      (for (_ _array_index) (Variables|Default|GetChipInfo_Ver2)
        (Variables|Default|SetSettingChipData_ArrayIndex _array_index)
        (switch Utilities|FlowControl|Switch|SwitchonE_ChipType_Ver2 (.ChipType (Utilities|Struct|BreakS_ChipStatas_Ver2 (.chipstatas (Utilities|Array|Get(acopy) (Variables|Default|GetChipInfo_Ver2) (Variables|Default|GetSettingChipData_ArrayIndex)))))
          (:NewEnumerator1
            ;[1 1 1] 方向の設定
            (CallFunction|SetMoveDirection (Variables|Default|GetSettingChipData_ArrayIndex)))
          (:NewEnumerator9
            ;[1 1 1] 生成場所の設定
            (CallFunction|SetSpawnPosition (Variables|Default|GetSettingChipData_ArrayIndex))))))
    (:NewEnumerator1
      (Development|PrintString "弾が設定されていません！" true true "(R=1.000000,G=0.000000,B=0.053420,A=1.000000)" :!label _label))
    (:NewEnumerator3
      (goto _label))
    (:NewEnumerator4
      (goto _label))
    (:NewEnumerator5
      (goto _label))
    (:NewEnumerator6
      (goto _label))
    (:NewEnumerator7
      (goto _label))))

(event EventTick
  (params (DeltaSeconds :type Float%20%28single-precision%29))
  (Variables|Default|SetDeltaSeconds DeltaSeconds)
  ;[1 1 1] 魔術の制御【Prt～α】
  (CallFunction|MagicControlaVer2)
  ;[1 1 1] 強制削除
  (Utilities|FlowControl|Delay 1e+01)
  (Actor|DestroyActor))

(event EventBeginPlay)

(fn ConstructionScript)

(fn ActionSpecial
  (params (ChipSpecial :type E_ChipSpecial%20Enum :default "NewEnumerator0") (ChipIndex :type Integer) (ChipType :type E_ChipType%20Enum :default "NewEnumerator0"))
  (switch Utilities|FlowControl|Switch|SwitchonE_ChipSpecial ChipSpecial))

(fn SetMoveDirection
  (params (LocalArrayIndex :type Integer))
  (LocalVariables|SetArrayIndex_move LocalArrayIndex)
  (switch Utilities|FlowControl|Switch|SwitchonE_ChipMoveDirectionType_Ver2 (.ChipMoveDirectionType (Utilities|Struct|BreakS_ChipMove_Ver2 (.chipmove (Utilities|Array|Get(acopy) (Variables|Default|GetChipInfo_Ver2) (LocalVariables|GetArrayIndex_move)))))
    (:NewEnumerator1
      (Utilities|Array|SetArrayElem (Variables|Default|GetChipInfo_Ver2) (LocalVariables|GetArrayIndex_move) (Utilities|Struct|MakeS_MagicChipInfo_Ver2 (.chipstatas (Utilities|Array|Get(acopy) (Variables|Default|GetChipInfo_Ver2) (LocalVariables|GetArrayIndex_move))) "(ChipShapeType_7_D0A7429B4E46D1984142D6AC1C6C09FC=NewEnumerator0,3DTexture_6_CB930A80470CAD92277DEA8DDF15240A=None,IsUsed?_9_A2720F424C1C437CA1F843921FF30AA5=False)" (Utilities|Struct|MakeS_ChipMove_Ver2 (.ChipMoveDirectionType (Utilities|Struct|BreakS_ChipMove_Ver2 (.chipmove (Utilities|Array|Get(acopy) (Variables|Default|GetChipInfo_Ver2) (LocalVariables|GetArrayIndex_move))))) (.MoveSpeed (Utilities|Struct|BreakS_ChipMove_Ver2 (.chipmove (Utilities|Array|Get(acopy) (Variables|Default|GetChipInfo_Ver2) (LocalVariables|GetArrayIndex_move))))) (* (Transformation|GetActorForwardVector (Game|GetPlayerController 0)) (.MoveSpeed (Utilities|Struct|BreakS_ChipMove_Ver2 (.chipmove (Utilities|Array|Get(acopy) (Variables|Default|GetChipInfo_Ver2) (LocalVariables|GetArrayIndex_move))))))) "(ChipSpecialType_6_3B5EDCAA4D8FDA68DA74278DC55901C0=NewEnumerator0,ChipDelayTime_5_08E108864A90A42763E241AD80C519F0=(IsUsed?_1_9980ABC845E4CA130FCA5EB9BE1951E7=False,DelayTime_8_0308187F448978D8B3719C94E9EC06C6=0.000000,DelayCount_7_58DA77354FFB2DDC46B2898A19F6431D=0.000000))" "(TypeIf_5_66B94DDD4D78BDA355B03BB5CE781A3D=NewEnumerator0,True_or_False_6_E087641342F38E88B7B6F6BDD7CC07F0=False,IfNumber_12_D3DBE6CD469D99947208E09CD0FC35CD=0)" "(ConditionType_24_56697AE94C44CAB4EF60EF922AC8031D=NewEnumerator0,ConditionTime_32_3D353E9249536E9E44540FA5590C1303=(ConditionTimeType_9_3768C87E4CC6EA067621ADA414EF3E88=NewEnumerator0,TimeValue_5_9AA4464A488A3DD1A90FB381F75542D0=0.000000,TimeCount_12_26311640481FD74B385D83992938FB04=0.000000),IsUsed?_36_43BA177A46243C9315CA41AB6EAB9D2C=False,FlagChenged?_38_D4CFEC824F7999E2558252AB5BCC8FE7=False)" "(ChipAttributeType_2_CEDC4CEE443A86AD18D5FF82B0B73117=NewEnumerator2,AttributeDamege_5_DD56E1F94F4524348E86A698B49CDE2E=0.000000)" "(TypeEnd_3_A19BA0F14C23C24F8855CEB69952F3FB=NewEnumerator0,IsEnd?_6_D1C203774EC68415949859987A4209C2=False,Explosion_11_463CAF064194C8C6E7FA65928086DE1D=(Size_2_C0A98C40497D32613C183E870A236DA2=0.000000))" "(SpawnType_10_52107B4A4259D2CA42227BB68313A4FA=NewEnumerator0,SpawnDirection_12_0B7D96A54317A03644B11A832E18C4CC=NewEnumerator0,SpawnDistance_8_41B3E582417D993B1C9B4880249F8A0C=0.000000)" "(Value_2_D93B6B5D4295A64E0FDBDFA847A9E7D8=0.000000)")))
    (:NewEnumerator4
      (Utilities|Array|SetArrayElem (Variables|Default|GetChipInfo_Ver2) (LocalVariables|GetArrayIndex_move) (Utilities|Struct|MakeS_MagicChipInfo_Ver2 (.chipstatas (Utilities|Array|Get(acopy) (Variables|Default|GetChipInfo_Ver2) (LocalVariables|GetArrayIndex_move))) "(ChipShapeType_7_D0A7429B4E46D1984142D6AC1C6C09FC=NewEnumerator0,3DTexture_6_CB930A80470CAD92277DEA8DDF15240A=None,IsUsed?_9_A2720F424C1C437CA1F843921FF30AA5=False)" (Utilities|Struct|MakeS_ChipMove_Ver2 (.ChipMoveDirectionType (Utilities|Struct|BreakS_ChipMove_Ver2 (.chipmove (Utilities|Array|Get(acopy) (Variables|Default|GetChipInfo_Ver2) (LocalVariables|GetArrayIndex_move))))) (.MoveSpeed (Utilities|Struct|BreakS_ChipMove_Ver2 (.chipmove (Utilities|Array|Get(acopy) (Variables|Default|GetChipInfo_Ver2) (LocalVariables|GetArrayIndex_move))))) (* (Transformation|GetActorRightVector (Game|GetPlayerController 0)) (.MoveSpeed (Utilities|Struct|BreakS_ChipMove_Ver2 (.chipmove (Utilities|Array|Get(acopy) (Variables|Default|GetChipInfo_Ver2) (LocalVariables|GetArrayIndex_move))))))) "(ChipSpecialType_6_3B5EDCAA4D8FDA68DA74278DC55901C0=NewEnumerator0,ChipDelayTime_5_08E108864A90A42763E241AD80C519F0=(IsUsed?_1_9980ABC845E4CA130FCA5EB9BE1951E7=False,DelayTime_8_0308187F448978D8B3719C94E9EC06C6=0.000000,DelayCount_7_58DA77354FFB2DDC46B2898A19F6431D=0.000000))" "(TypeIf_5_66B94DDD4D78BDA355B03BB5CE781A3D=NewEnumerator0,True_or_False_6_E087641342F38E88B7B6F6BDD7CC07F0=False,IfNumber_12_D3DBE6CD469D99947208E09CD0FC35CD=0)" "(ConditionType_24_56697AE94C44CAB4EF60EF922AC8031D=NewEnumerator0,ConditionTime_32_3D353E9249536E9E44540FA5590C1303=(ConditionTimeType_9_3768C87E4CC6EA067621ADA414EF3E88=NewEnumerator0,TimeValue_5_9AA4464A488A3DD1A90FB381F75542D0=0.000000,TimeCount_12_26311640481FD74B385D83992938FB04=0.000000),IsUsed?_36_43BA177A46243C9315CA41AB6EAB9D2C=False,FlagChenged?_38_D4CFEC824F7999E2558252AB5BCC8FE7=False)" "(ChipAttributeType_2_CEDC4CEE443A86AD18D5FF82B0B73117=NewEnumerator2,AttributeDamege_5_DD56E1F94F4524348E86A698B49CDE2E=0.000000)" "(TypeEnd_3_A19BA0F14C23C24F8855CEB69952F3FB=NewEnumerator0,IsEnd?_6_D1C203774EC68415949859987A4209C2=False,Explosion_11_463CAF064194C8C6E7FA65928086DE1D=(Size_2_C0A98C40497D32613C183E870A236DA2=0.000000))" "(SpawnType_10_52107B4A4259D2CA42227BB68313A4FA=NewEnumerator0,SpawnDirection_12_0B7D96A54317A03644B11A832E18C4CC=NewEnumerator0,SpawnDistance_8_41B3E582417D993B1C9B4880249F8A0C=0.000000)" "(Value_2_D93B6B5D4295A64E0FDBDFA847A9E7D8=0.000000)")))
    (:NewEnumerator5
      (bind _output_get (LocalVariables|SetUpVector "0.000000,0.000000,1.000000"))
      (Utilities|Array|SetArrayElem (Variables|Default|GetChipInfo_Ver2) (LocalVariables|GetArrayIndex_move) (Utilities|Struct|MakeS_MagicChipInfo_Ver2 (.chipstatas (Utilities|Array|Get(acopy) (Variables|Default|GetChipInfo_Ver2) (LocalVariables|GetArrayIndex_move))) "(ChipShapeType_7_D0A7429B4E46D1984142D6AC1C6C09FC=NewEnumerator0,3DTexture_6_CB930A80470CAD92277DEA8DDF15240A=None,IsUsed?_9_A2720F424C1C437CA1F843921FF30AA5=False)" (Utilities|Struct|MakeS_ChipMove_Ver2 (.ChipMoveDirectionType (Utilities|Struct|BreakS_ChipMove_Ver2 (.chipmove (Utilities|Array|Get(acopy) (Variables|Default|GetChipInfo_Ver2) (LocalVariables|GetArrayIndex_move))))) (.MoveSpeed (Utilities|Struct|BreakS_ChipMove_Ver2 (.chipmove (Utilities|Array|Get(acopy) (Variables|Default|GetChipInfo_Ver2) (LocalVariables|GetArrayIndex_move))))) (* (.MoveSpeed (Utilities|Struct|BreakS_ChipMove_Ver2 (.chipmove (Utilities|Array|Get(acopy) (Variables|Default|GetChipInfo_Ver2) (LocalVariables|GetArrayIndex_move))))) _output_get)) "(ChipSpecialType_6_3B5EDCAA4D8FDA68DA74278DC55901C0=NewEnumerator0,ChipDelayTime_5_08E108864A90A42763E241AD80C519F0=(IsUsed?_1_9980ABC845E4CA130FCA5EB9BE1951E7=False,DelayTime_8_0308187F448978D8B3719C94E9EC06C6=0.000000,DelayCount_7_58DA77354FFB2DDC46B2898A19F6431D=0.000000))" "(TypeIf_5_66B94DDD4D78BDA355B03BB5CE781A3D=NewEnumerator0,True_or_False_6_E087641342F38E88B7B6F6BDD7CC07F0=False,IfNumber_12_D3DBE6CD469D99947208E09CD0FC35CD=0)" "(ConditionType_24_56697AE94C44CAB4EF60EF922AC8031D=NewEnumerator0,ConditionTime_32_3D353E9249536E9E44540FA5590C1303=(ConditionTimeType_9_3768C87E4CC6EA067621ADA414EF3E88=NewEnumerator0,TimeValue_5_9AA4464A488A3DD1A90FB381F75542D0=0.000000,TimeCount_12_26311640481FD74B385D83992938FB04=0.000000),IsUsed?_36_43BA177A46243C9315CA41AB6EAB9D2C=False,FlagChenged?_38_D4CFEC824F7999E2558252AB5BCC8FE7=False)" "(ChipAttributeType_2_CEDC4CEE443A86AD18D5FF82B0B73117=NewEnumerator2,AttributeDamege_5_DD56E1F94F4524348E86A698B49CDE2E=0.000000)" "(TypeEnd_3_A19BA0F14C23C24F8855CEB69952F3FB=NewEnumerator0,IsEnd?_6_D1C203774EC68415949859987A4209C2=False,Explosion_11_463CAF064194C8C6E7FA65928086DE1D=(Size_2_C0A98C40497D32613C183E870A236DA2=0.000000))" "(SpawnType_10_52107B4A4259D2CA42227BB68313A4FA=NewEnumerator0,SpawnDirection_12_0B7D96A54317A03644B11A832E18C4CC=NewEnumerator0,SpawnDistance_8_41B3E582417D993B1C9B4880249F8A0C=0.000000)" "(Value_2_D93B6B5D4295A64E0FDBDFA847A9E7D8=0.000000)")))))

(fn MagicControl
  (bind _array_index (Utilities|Array|ForEachLoopwithBreak (Variables|Default|GetChipInfo_Ver2) :!label _label)
    (:LoopBody
      (LocalVariables|SetArrayIndex _array_index)
      (switch Utilities|FlowControl|Switch|SwitchonE_ChipType_Ver2 (.ChipType (Utilities|Struct|BreakS_ChipStatas_Ver2 (.chipstatas (Utilities|Array|Get(acopy) (Variables|Default|GetChipInfo_Ver2) (LocalVariables|GetArrayIndex)))))
        (:NewEnumerator1
          (Transformation|SetActorLocation (+ (Transformation|GetActorLocation) (* (Variables|Default|GetDeltaSeconds) (.MoveLocation (Utilities|Struct|BreakS_ChipMove_Ver2 (.chipmove (Utilities|Array|Get(acopy) (Variables|Default|GetChipInfo_Ver2) (LocalVariables|GetArrayIndex))))))) false false))
        (:NewEnumerator3
          (switch Utilities|FlowControl|Switch|SwitchonE_ChipSpecialType_Ver2 (.ChipSpecialType (Utilities|Struct|BreakS_ChipSpecial_Ver2 (.chipspecial (Utilities|Array|Get(acopy) (Variables|Default|GetChipInfo_Ver2) (LocalVariables|GetArrayIndex)))))
            (:NewEnumerator1
              (bind _isused_ (CallFunction|SpecialDelayControl (LocalVariables|GetArrayIndex)))
              (if (not _isused_)
                (goto _label Break)))))))))

(fn SpecialDelayControl
  (params (ArrayIndex :type Integer))
  (LocalVariables|SetLocalArrayIndex ArrayIndex)
  (if (.isused? (.ChipDelayTime (Utilities|Struct|BreakS_ChipSpecial_Ver2 (.chipspecial (Utilities|Array|Get(acopy) (Variables|Default|GetChipInfo_Ver2) (LocalVariables|GetLocalArrayIndex))))))
    (bind _output_get (LocalVariables|SetIsUsedFlag true))
    (else
      (Utilities|Array|SetArrayElem (Variables|Default|GetChipInfo_Ver2) (LocalVariables|GetLocalArrayIndex) (Utilities|Struct|MakeS_MagicChipInfo_Ver2 (.chipstatas (Utilities|Array|Get(acopy) (Variables|Default|GetChipInfo_Ver2) (LocalVariables|GetLocalArrayIndex))) "(ChipShapeType_7_D0A7429B4E46D1984142D6AC1C6C09FC=NewEnumerator0,3DTexture_6_CB930A80470CAD92277DEA8DDF15240A=None,IsUsed?_9_A2720F424C1C437CA1F843921FF30AA5=False)" "(ChipMoveDirectionType_10_4915AED94BCCB891B5A92BB92579A3AF=NewEnumerator0,MoveSpeed_5_78DA1AA94C4F84822D5877A8B97AD4FE=0.000000,MoveLocation_9_2809D0F64AB7CC2C411F049EBE2CC596=(X=0.000000,Y=0.000000,Z=0.000000))" (Utilities|Struct|MakeS_ChipSpecial_Ver2 (.ChipSpecialType (Utilities|Struct|BreakS_ChipSpecial_Ver2 (.chipspecial (Utilities|Array|Get(acopy) (Variables|Default|GetChipInfo_Ver2) (LocalVariables|GetLocalArrayIndex))))) (Utilities|Struct|MakeS_Special_Delay (<= (.delaytime (.ChipDelayTime (Utilities|Struct|BreakS_ChipSpecial_Ver2 (.chipspecial (Utilities|Array|Get(acopy) (Variables|Default|GetChipInfo_Ver2) (LocalVariables|GetLocalArrayIndex)))))) (.delaycount (.ChipDelayTime (Utilities|Struct|BreakS_ChipSpecial_Ver2 (.chipspecial (Utilities|Array|Get(acopy) (Variables|Default|GetChipInfo_Ver2) (LocalVariables|GetLocalArrayIndex))))))) (.delaytime (.ChipDelayTime (Utilities|Struct|BreakS_ChipSpecial_Ver2 (.chipspecial (Utilities|Array|Get(acopy) (Variables|Default|GetChipInfo_Ver2) (LocalVariables|GetLocalArrayIndex)))))) (+ (.delaycount (.ChipDelayTime (Utilities|Struct|BreakS_ChipSpecial_Ver2 (.chipspecial (Utilities|Array|Get(acopy) (Variables|Default|GetChipInfo_Ver2) (LocalVariables|GetLocalArrayIndex)))))) (Variables|Default|GetDeltaSeconds)))) "(TypeIf_5_66B94DDD4D78BDA355B03BB5CE781A3D=NewEnumerator0,True_or_False_6_E087641342F38E88B7B6F6BDD7CC07F0=False,IfNumber_12_D3DBE6CD469D99947208E09CD0FC35CD=0)" "(ConditionType_24_56697AE94C44CAB4EF60EF922AC8031D=NewEnumerator0,ConditionTime_32_3D353E9249536E9E44540FA5590C1303=(ConditionTimeType_9_3768C87E4CC6EA067621ADA414EF3E88=NewEnumerator0,TimeValue_5_9AA4464A488A3DD1A90FB381F75542D0=0.000000,TimeCount_12_26311640481FD74B385D83992938FB04=0.000000),IsUsed?_36_43BA177A46243C9315CA41AB6EAB9D2C=False,FlagChenged?_38_D4CFEC824F7999E2558252AB5BCC8FE7=False)" "(ChipAttributeType_2_CEDC4CEE443A86AD18D5FF82B0B73117=NewEnumerator2,AttributeDamege_5_DD56E1F94F4524348E86A698B49CDE2E=0.000000)" "(TypeEnd_3_A19BA0F14C23C24F8855CEB69952F3FB=NewEnumerator0,IsEnd?_6_D1C203774EC68415949859987A4209C2=False,Explosion_11_463CAF064194C8C6E7FA65928086DE1D=(Size_2_C0A98C40497D32613C183E870A236DA2=0.000000))" "(SpawnType_10_52107B4A4259D2CA42227BB68313A4FA=NewEnumerator0,SpawnDirection_12_0B7D96A54317A03644B11A832E18C4CC=NewEnumerator0,SpawnDistance_8_41B3E582417D993B1C9B4880249F8A0C=0.000000)" "(Value_2_D93B6B5D4295A64E0FDBDFA847A9E7D8=0.000000)"))
      (LocalVariables|SetIsUsedFlag false)))
  (return _output_get))

(fn MagicControlaVer2
  (bind _array_index (Utilities|Array|ForEachLoopwithBreak (Variables|Default|GetChipInfo_Ver2))
    (:LoopBody
      (LocalVariables|SetLocalArrayIndex _array_index)
      (if (not (.IsBad? (Utilities|Struct|BreakS_ChipStatas_Ver2 (.chipstatas (Utilities|Array|Get(acopy) (Variables|Default|GetChipInfo_Ver2) (LocalVariables|GetLocalArrayIndex))))))
        (switch Utilities|FlowControl|Switch|SwitchonE_ChipType_Ver2 (.ChipType (Utilities|Struct|BreakS_ChipStatas_Ver2 (.chipstatas (Utilities|Array|Get(acopy) (Variables|Default|GetChipInfo_Ver2) (LocalVariables|GetLocalArrayIndex)))))
          (:NewEnumerator1
            (Transformation|SetActorLocation (+ (Transformation|GetActorLocation) (* (Variables|Default|GetDeltaSeconds) (.MoveLocation (Utilities|Struct|BreakS_ChipMove_Ver2 (.chipmove (Utilities|Array|Get(acopy) (Variables|Default|GetChipInfo_Ver2) (LocalVariables|GetLocalArrayIndex))))))) false false))
          (:NewEnumerator4
            (switch Utilities|FlowControl|Switch|SwitchonE_ChipIfType_Ver2 (.TypeIf (Utilities|Struct|BreakS_ChipIf_Ver2 (.chipif (Utilities|Array|Get(acopy) (Variables|Default|GetChipInfo_Ver2) (LocalVariables|GetLocalArrayIndex)))))
              (:NewEnumerator1
                (LocalVariables|SetConditionCount 0)
                (bind _index (Utilities|FlowControl|ForLoopwithBreak (LocalVariables|GetLocalArrayIndex) (Utilities|Array|Length (Variables|Default|GetChipInfo_Ver2)))
                  (:LoopBody
                    (LocalVariables|SetIfArrayIndex _index)
                    (if (< (LocalVariables|GetConditionCount) 1)
                      (if (not (.IsBad? (Utilities|Struct|BreakS_ChipStatas_Ver2 (.chipstatas (Utilities|Array|Get(acopy) (Variables|Default|GetChipInfo_Ver2) (LocalVariables|GetIfArrayIndex))))))
                        (switch Utilities|FlowControl|Switch|SwitchonE_ChipType_Ver2 (.ChipType (Utilities|Struct|BreakS_ChipStatas_Ver2 (.chipstatas (Utilities|Array|Get(acopy) (Variables|Default|GetChipInfo_Ver2) (LocalVariables|GetIfArrayIndex)))))
                          (:NewEnumerator5
                            (LocalVariables|SetConditionCount (+ 1 (LocalVariables|GetConditionCount)))
                            (CallFunction|ConditionControl (LocalVariables|GetIfArrayIndex)))))))))))
          (:NewEnumerator7
            (CallFunction|EndControl (LocalVariables|GetLocalArrayIndex))
            (Actor|DestroyActor)))))))

(fn ConditionTypeTime
  (params (IfArrayIndex :type Integer))
  (LocalVariables|SetIfLocalArrayIndex IfArrayIndex)
  (Utilities|Array|SetArrayElem (Variables|Default|GetChipInfo_Ver2) (LocalVariables|GetIfLocalArrayIndex) (Utilities|Struct|MakeS_MagicChipInfo_Ver2 (.chipstatas (Utilities|Array|Get(acopy) (Variables|Default|GetChipInfo_Ver2) (LocalVariables|GetIfLocalArrayIndex))) "(ChipShapeType_7_D0A7429B4E46D1984142D6AC1C6C09FC=NewEnumerator0,3DTexture_6_CB930A80470CAD92277DEA8DDF15240A=None,IsUsed?_9_A2720F424C1C437CA1F843921FF30AA5=False)" "(ChipMoveDirectionType_10_4915AED94BCCB891B5A92BB92579A3AF=NewEnumerator0,MoveSpeed_5_78DA1AA94C4F84822D5877A8B97AD4FE=0.000000,MoveLocation_9_2809D0F64AB7CC2C411F049EBE2CC596=(X=0.000000,Y=0.000000,Z=0.000000))" "(ChipSpecialType_6_3B5EDCAA4D8FDA68DA74278DC55901C0=NewEnumerator0,ChipDelayTime_5_08E108864A90A42763E241AD80C519F0=(IsUsed?_1_9980ABC845E4CA130FCA5EB9BE1951E7=False,DelayTime_8_0308187F448978D8B3719C94E9EC06C6=0.000000,DelayCount_7_58DA77354FFB2DDC46B2898A19F6431D=0.000000))" "(TypeIf_5_66B94DDD4D78BDA355B03BB5CE781A3D=NewEnumerator0,True_or_False_6_E087641342F38E88B7B6F6BDD7CC07F0=False,IfNumber_12_D3DBE6CD469D99947208E09CD0FC35CD=0)" (Utilities|Struct|MakeS_ChipCondition_Ver2 (.ConditionType (Utilities|Struct|BreakS_ChipCondition_Ver2 (.chipcondition (Utilities|Array|Get(acopy) (Variables|Default|GetChipInfo_Ver2) (LocalVariables|GetIfLocalArrayIndex))))) (Utilities|Struct|MakeS_ChipCondition_Time_Ver2 (.ConditionTimeType (Utilities|Struct|BreakS_ChipCondition_Time_Ver2 (.ConditionTime (Utilities|Struct|BreakS_ChipCondition_Ver2 (.chipcondition (Utilities|Array|Get(acopy) (Variables|Default|GetChipInfo_Ver2) (LocalVariables|GetIfLocalArrayIndex))))))) (.TimeValue (Utilities|Struct|BreakS_ChipCondition_Time_Ver2 (.ConditionTime (Utilities|Struct|BreakS_ChipCondition_Ver2 (.chipcondition (Utilities|Array|Get(acopy) (Variables|Default|GetChipInfo_Ver2) (LocalVariables|GetIfLocalArrayIndex))))))) (+ (.TimeCount (Utilities|Struct|BreakS_ChipCondition_Time_Ver2 (.ConditionTime (Utilities|Struct|BreakS_ChipCondition_Ver2 (.chipcondition (Utilities|Array|Get(acopy) (Variables|Default|GetChipInfo_Ver2) (LocalVariables|GetIfLocalArrayIndex))))))) (Variables|Default|GetDeltaSeconds))) (.IsUsed? (Utilities|Struct|BreakS_ChipCondition_Ver2 (.chipcondition (Utilities|Array|Get(acopy) (Variables|Default|GetChipInfo_Ver2) (LocalVariables|GetIfLocalArrayIndex))))) (.FlagChenged? (Utilities|Struct|BreakS_ChipCondition_Ver2 (.chipcondition (Utilities|Array|Get(acopy) (Variables|Default|GetChipInfo_Ver2) (LocalVariables|GetIfLocalArrayIndex)))))) "(ChipAttributeType_2_CEDC4CEE443A86AD18D5FF82B0B73117=NewEnumerator2,AttributeDamege_5_DD56E1F94F4524348E86A698B49CDE2E=0.000000)" "(TypeEnd_3_A19BA0F14C23C24F8855CEB69952F3FB=NewEnumerator0,IsEnd?_6_D1C203774EC68415949859987A4209C2=False,Explosion_11_463CAF064194C8C6E7FA65928086DE1D=(Size_2_C0A98C40497D32613C183E870A236DA2=0.000000))" "(SpawnType_10_52107B4A4259D2CA42227BB68313A4FA=NewEnumerator0,SpawnDirection_12_0B7D96A54317A03644B11A832E18C4CC=NewEnumerator0,SpawnDistance_8_41B3E582417D993B1C9B4880249F8A0C=0.000000)" "(Value_2_D93B6B5D4295A64E0FDBDFA847A9E7D8=0.000000)"))
  (switch Utilities|FlowControl|Switch|SwitchonE_ChipCondition_Time_Ver2 (.ConditionTimeType (Utilities|Struct|BreakS_ChipCondition_Time_Ver2 (.ConditionTime (Utilities|Struct|BreakS_ChipCondition_Ver2 (.chipcondition (Utilities|Array|Get(acopy) (Variables|Default|GetChipInfo_Ver2) (LocalVariables|GetIfLocalArrayIndex)))))))
    (:NewEnumerator1
      (if (<= (.TimeValue (Utilities|Struct|BreakS_ChipCondition_Time_Ver2 (.ConditionTime (Utilities|Struct|BreakS_ChipCondition_Ver2 (.chipcondition (Utilities|Array|Get(acopy) (Variables|Default|GetChipInfo_Ver2) (LocalVariables|GetIfLocalArrayIndex))))))) (.TimeCount (Utilities|Struct|BreakS_ChipCondition_Time_Ver2 (.ConditionTime (Utilities|Struct|BreakS_ChipCondition_Ver2 (.chipcondition (Utilities|Array|Get(acopy) (Variables|Default|GetChipInfo_Ver2) (LocalVariables|GetIfLocalArrayIndex))))))))
        _
        (else
          (return true))))
    (:NewEnumerator3
      (if (>= (.TimeValue (Utilities|Struct|BreakS_ChipCondition_Time_Ver2 (.ConditionTime (Utilities|Struct|BreakS_ChipCondition_Ver2 (.chipcondition (Utilities|Array|Get(acopy) (Variables|Default|GetChipInfo_Ver2) (LocalVariables|GetIfLocalArrayIndex))))))) (.TimeCount (Utilities|Struct|BreakS_ChipCondition_Time_Ver2 (.ConditionTime (Utilities|Struct|BreakS_ChipCondition_Ver2 (.chipcondition (Utilities|Array|Get(acopy) (Variables|Default|GetChipInfo_Ver2) (LocalVariables|GetIfLocalArrayIndex))))))))
        _
        (else
          (return true)))))
  (return false))

(fn ConditionControl
  (params (IfArrayIndex :type Integer))
  (LocalVariables|SetIfArrayIndex_Local IfArrayIndex)
  (switch Utilities|FlowControl|Switch|SwitchonE_ChipConditionType_Ver2 (.ConditionType (Utilities|Struct|BreakS_ChipCondition_Ver2 (.chipcondition (Utilities|Array|Get(acopy) (Variables|Default|GetChipInfo_Ver2) (LocalVariables|GetIfArrayIndex_Local)))))
    (:NewEnumerator1
      (bind _isbad_ (CallFunction|ConditionTypeTime (LocalVariables|GetIfArrayIndex_Local)))
      (LocalVariables|SetIsBad?_ConditionTypeTime _isbad_)
      (if (.FlagChenged? (Utilities|Struct|BreakS_ChipCondition_Ver2 (.chipcondition (Utilities|Array|Get(acopy) (Variables|Default|GetChipInfo_Ver2) (LocalVariables|GetIfArrayIndex_Local)))))
        (if (not (== (.IsUsed? (Utilities|Struct|BreakS_ChipCondition_Ver2 (.chipcondition (Utilities|Array|Get(acopy) (Variables|Default|GetChipInfo_Ver2) (LocalVariables|GetIfArrayIndex_Local))))) (!= (LocalVariables|GetIsBad?_ConditionTypeTime) true)))
          (Utilities|Array|SetArrayElem (Variables|Default|GetChipInfo_Ver2) (LocalVariables|GetIfArrayIndex_Local) (Utilities|Struct|MakeS_MagicChipInfo_Ver2 (.chipstatas (Utilities|Array|Get(acopy) (Variables|Default|GetChipInfo_Ver2) (LocalVariables|GetIfArrayIndex_Local))) "(ChipShapeType_7_D0A7429B4E46D1984142D6AC1C6C09FC=NewEnumerator0,3DTexture_6_CB930A80470CAD92277DEA8DDF15240A=None,IsUsed?_9_A2720F424C1C437CA1F843921FF30AA5=False)" "(ChipMoveDirectionType_10_4915AED94BCCB891B5A92BB92579A3AF=NewEnumerator0,MoveSpeed_5_78DA1AA94C4F84822D5877A8B97AD4FE=0.000000,MoveLocation_9_2809D0F64AB7CC2C411F049EBE2CC596=(X=0.000000,Y=0.000000,Z=0.000000))" "(ChipSpecialType_6_3B5EDCAA4D8FDA68DA74278DC55901C0=NewEnumerator0,ChipDelayTime_5_08E108864A90A42763E241AD80C519F0=(IsUsed?_1_9980ABC845E4CA130FCA5EB9BE1951E7=False,DelayTime_8_0308187F448978D8B3719C94E9EC06C6=0.000000,DelayCount_7_58DA77354FFB2DDC46B2898A19F6431D=0.000000))" "(TypeIf_5_66B94DDD4D78BDA355B03BB5CE781A3D=NewEnumerator0,True_or_False_6_E087641342F38E88B7B6F6BDD7CC07F0=False,IfNumber_12_D3DBE6CD469D99947208E09CD0FC35CD=0)" (Utilities|Struct|MakeS_ChipCondition_Ver2 (.ConditionType (Utilities|Struct|BreakS_ChipCondition_Ver2 (.chipcondition (Utilities|Array|Get(acopy) (Variables|Default|GetChipInfo_Ver2) (LocalVariables|GetIfArrayIndex_Local))))) (.ConditionTime (Utilities|Struct|BreakS_ChipCondition_Ver2 (.chipcondition (Utilities|Array|Get(acopy) (Variables|Default|GetChipInfo_Ver2) (LocalVariables|GetIfArrayIndex_Local))))) (!= (LocalVariables|GetIsBad?_ConditionTypeTime) true) (.FlagChenged? (Utilities|Struct|BreakS_ChipCondition_Ver2 (.chipcondition (Utilities|Array|Get(acopy) (Variables|Default|GetChipInfo_Ver2) (LocalVariables|GetIfArrayIndex_Local))))))))
          (if (LocalVariables|GetIsBad?_ConditionTypeTime) :!label _label
            (bind _index (Utilities|FlowControl|ForLoopwithBreak (+ (LocalVariables|GetIfArrayIndex_Local) 1) (Utilities|Array|Length (Variables|Default|GetChipInfo_Ver2)) :!label _label_2)
              (:LoopBody
                (LocalVariables|SetConditionArrayIndex _index)
                (Utilities|Array|SetArrayElem (Variables|Default|GetChipInfo_Ver2) (LocalVariables|GetConditionArrayIndex) (Utilities|Struct|MakeS_MagicChipInfo_Ver2 (Utilities|Struct|MakeS_ChipStatas_Ver2 (.ChipName (Utilities|Struct|BreakS_ChipStatas_Ver2 (.chipstatas (Utilities|Array|Get(acopy) (Variables|Default|GetChipInfo_Ver2) (LocalVariables|GetConditionArrayIndex))))) (.ChipDescription (Utilities|Struct|BreakS_ChipStatas_Ver2 (.chipstatas (Utilities|Array|Get(acopy) (Variables|Default|GetChipInfo_Ver2) (LocalVariables|GetConditionArrayIndex))))) (.ChipIcon (Utilities|Struct|BreakS_ChipStatas_Ver2 (.chipstatas (Utilities|Array|Get(acopy) (Variables|Default|GetChipInfo_Ver2) (LocalVariables|GetConditionArrayIndex))))) (.CastTime (Utilities|Struct|BreakS_ChipStatas_Ver2 (.chipstatas (Utilities|Array|Get(acopy) (Variables|Default|GetChipInfo_Ver2) (LocalVariables|GetConditionArrayIndex))))) (.ChipDamege (Utilities|Struct|BreakS_ChipStatas_Ver2 (.chipstatas (Utilities|Array|Get(acopy) (Variables|Default|GetChipInfo_Ver2) (LocalVariables|GetConditionArrayIndex))))) (.ChipType (Utilities|Struct|BreakS_ChipStatas_Ver2 (.chipstatas (Utilities|Array|Get(acopy) (Variables|Default|GetChipInfo_Ver2) (LocalVariables|GetConditionArrayIndex)))))) (.chipshape (Utilities|Array|Get(acopy) (Variables|Default|GetChipInfo_Ver2) (LocalVariables|GetConditionArrayIndex))) (.chipmove (Utilities|Array|Get(acopy) (Variables|Default|GetChipInfo_Ver2) (LocalVariables|GetConditionArrayIndex))) (.chipspecial (Utilities|Array|Get(acopy) (Variables|Default|GetChipInfo_Ver2) (LocalVariables|GetConditionArrayIndex))) (.chipif (Utilities|Array|Get(acopy) (Variables|Default|GetChipInfo_Ver2) (LocalVariables|GetConditionArrayIndex))) (.chipcondition (Utilities|Array|Get(acopy) (Variables|Default|GetChipInfo_Ver2) (LocalVariables|GetConditionArrayIndex))) (.chipattribute (Utilities|Array|Get(acopy) (Variables|Default|GetChipInfo_Ver2) (LocalVariables|GetConditionArrayIndex))) (.chipend (Utilities|Array|Get(acopy) (Variables|Default|GetChipInfo_Ver2) (LocalVariables|GetConditionArrayIndex))) "(SpawnType_10_52107B4A4259D2CA42227BB68313A4FA=NewEnumerator0,SpawnDirection_12_0B7D96A54317A03644B11A832E18C4CC=NewEnumerator0,SpawnDistance_8_41B3E582417D993B1C9B4880249F8A0C=0.000000)" "(Value_2_D93B6B5D4295A64E0FDBDFA847A9E7D8=0.000000)"))
                (switch Utilities|FlowControl|Switch|SwitchonE_ChipType_Ver2 (.ChipType (Utilities|Struct|BreakS_ChipStatas_Ver2 (.chipstatas (Utilities|Array|Get(acopy) (Variables|Default|GetChipInfo_Ver2) (LocalVariables|GetConditionArrayIndex)))))
                  (:NewEnumerator4
                    (switch Utilities|FlowControl|Switch|SwitchonE_ChipIfType_Ver2 (.TypeIf (Utilities|Struct|BreakS_ChipIf_Ver2 (.chipif (Utilities|Array|Get(acopy) (Variables|Default|GetChipInfo_Ver2) (LocalVariables|GetConditionArrayIndex)))))
                      (:NewEnumerator2
                        (if (== (.IfNumber (Utilities|Struct|BreakS_ChipIf_Ver2 (.chipif (Utilities|Array|Get(acopy) (Variables|Default|GetChipInfo_Ver2) (LocalVariables|GetConditionArrayIndex))))) (.IfNumber (Utilities|Struct|BreakS_ChipIf_Ver2 (.chipif (Utilities|Array|Get(acopy) (Variables|Default|GetChipInfo_Ver2) (- (LocalVariables|GetIfArrayIndex_Local) 1))))))
                          (goto _label_2 Break))))))))
            (else
              (bind _index_2 (Utilities|FlowControl|ForLoopwithBreak (+ (LocalVariables|GetIfArrayIndex_Local) 1) (Utilities|Array|Length (Variables|Default|GetChipInfo_Ver2)) :!label _label_3)
                (:LoopBody
                  (LocalVariables|SetConditionArrayIndex _index_2)
                  (Utilities|Array|SetArrayElem (Variables|Default|GetChipInfo_Ver2) (LocalVariables|GetConditionArrayIndex) (Utilities|Struct|MakeS_MagicChipInfo_Ver2 (Utilities|Struct|MakeS_ChipStatas_Ver2 (.ChipName (Utilities|Struct|BreakS_ChipStatas_Ver2 (.chipstatas (Utilities|Array|Get(acopy) (Variables|Default|GetChipInfo_Ver2) (LocalVariables|GetConditionArrayIndex))))) (.ChipDescription (Utilities|Struct|BreakS_ChipStatas_Ver2 (.chipstatas (Utilities|Array|Get(acopy) (Variables|Default|GetChipInfo_Ver2) (LocalVariables|GetConditionArrayIndex))))) (.ChipIcon (Utilities|Struct|BreakS_ChipStatas_Ver2 (.chipstatas (Utilities|Array|Get(acopy) (Variables|Default|GetChipInfo_Ver2) (LocalVariables|GetConditionArrayIndex))))) (.CastTime (Utilities|Struct|BreakS_ChipStatas_Ver2 (.chipstatas (Utilities|Array|Get(acopy) (Variables|Default|GetChipInfo_Ver2) (LocalVariables|GetConditionArrayIndex))))) (.ChipDamege (Utilities|Struct|BreakS_ChipStatas_Ver2 (.chipstatas (Utilities|Array|Get(acopy) (Variables|Default|GetChipInfo_Ver2) (LocalVariables|GetConditionArrayIndex))))) (.ChipType (Utilities|Struct|BreakS_ChipStatas_Ver2 (.chipstatas (Utilities|Array|Get(acopy) (Variables|Default|GetChipInfo_Ver2) (LocalVariables|GetConditionArrayIndex))))) true) (.chipshape (Utilities|Array|Get(acopy) (Variables|Default|GetChipInfo_Ver2) (LocalVariables|GetConditionArrayIndex))) (.chipmove (Utilities|Array|Get(acopy) (Variables|Default|GetChipInfo_Ver2) (LocalVariables|GetConditionArrayIndex))) (.chipspecial (Utilities|Array|Get(acopy) (Variables|Default|GetChipInfo_Ver2) (LocalVariables|GetConditionArrayIndex))) (.chipif (Utilities|Array|Get(acopy) (Variables|Default|GetChipInfo_Ver2) (LocalVariables|GetConditionArrayIndex))) (.chipcondition (Utilities|Array|Get(acopy) (Variables|Default|GetChipInfo_Ver2) (LocalVariables|GetConditionArrayIndex))) (.chipattribute (Utilities|Array|Get(acopy) (Variables|Default|GetChipInfo_Ver2) (LocalVariables|GetConditionArrayIndex))) (.chipend (Utilities|Array|Get(acopy) (Variables|Default|GetChipInfo_Ver2) (LocalVariables|GetConditionArrayIndex))) "(SpawnType_10_52107B4A4259D2CA42227BB68313A4FA=NewEnumerator0,SpawnDirection_12_0B7D96A54317A03644B11A832E18C4CC=NewEnumerator0,SpawnDistance_8_41B3E582417D993B1C9B4880249F8A0C=0.000000)" "(Value_2_D93B6B5D4295A64E0FDBDFA847A9E7D8=0.000000)"))
                  (switch Utilities|FlowControl|Switch|SwitchonE_ChipType_Ver2 (.ChipType (Utilities|Struct|BreakS_ChipStatas_Ver2 (.chipstatas (Utilities|Array|Get(acopy) (Variables|Default|GetChipInfo_Ver2) (LocalVariables|GetConditionArrayIndex)))))
                    (:NewEnumerator4
                      (switch Utilities|FlowControl|Switch|SwitchonE_ChipIfType_Ver2 (.TypeIf (Utilities|Struct|BreakS_ChipIf_Ver2 (.chipif (Utilities|Array|Get(acopy) (Variables|Default|GetChipInfo_Ver2) (LocalVariables|GetConditionArrayIndex)))))
                        (:NewEnumerator2
                          (if (== (.IfNumber (Utilities|Struct|BreakS_ChipIf_Ver2 (.chipif (Utilities|Array|Get(acopy) (Variables|Default|GetChipInfo_Ver2) (LocalVariables|GetConditionArrayIndex))))) (.IfNumber (Utilities|Struct|BreakS_ChipIf_Ver2 (.chipif (Utilities|Array|Get(acopy) (Variables|Default|GetChipInfo_Ver2) (- (LocalVariables|GetIfArrayIndex_Local) 1))))))
                            (goto _label_3 Break)))))))))))
        (else
          (Utilities|Array|SetArrayElem (Variables|Default|GetChipInfo_Ver2) (LocalVariables|GetIfArrayIndex_Local) (Utilities|Struct|MakeS_MagicChipInfo_Ver2 (.chipstatas (Utilities|Array|Get(acopy) (Variables|Default|GetChipInfo_Ver2) (LocalVariables|GetIfArrayIndex_Local))) "(ChipShapeType_7_D0A7429B4E46D1984142D6AC1C6C09FC=NewEnumerator0,3DTexture_6_CB930A80470CAD92277DEA8DDF15240A=None,IsUsed?_9_A2720F424C1C437CA1F843921FF30AA5=False)" "(ChipMoveDirectionType_10_4915AED94BCCB891B5A92BB92579A3AF=NewEnumerator0,MoveSpeed_5_78DA1AA94C4F84822D5877A8B97AD4FE=0.000000,MoveLocation_9_2809D0F64AB7CC2C411F049EBE2CC596=(X=0.000000,Y=0.000000,Z=0.000000))" "(ChipSpecialType_6_3B5EDCAA4D8FDA68DA74278DC55901C0=NewEnumerator0,ChipDelayTime_5_08E108864A90A42763E241AD80C519F0=(IsUsed?_1_9980ABC845E4CA130FCA5EB9BE1951E7=False,DelayTime_8_0308187F448978D8B3719C94E9EC06C6=0.000000,DelayCount_7_58DA77354FFB2DDC46B2898A19F6431D=0.000000))" "(TypeIf_5_66B94DDD4D78BDA355B03BB5CE781A3D=NewEnumerator0,True_or_False_6_E087641342F38E88B7B6F6BDD7CC07F0=False,IfNumber_12_D3DBE6CD469D99947208E09CD0FC35CD=0)" (Utilities|Struct|MakeS_ChipCondition_Ver2 (.ConditionType (Utilities|Struct|BreakS_ChipCondition_Ver2 (.chipcondition (Utilities|Array|Get(acopy) (Variables|Default|GetChipInfo_Ver2) (LocalVariables|GetIfArrayIndex_Local))))) (.ConditionTime (Utilities|Struct|BreakS_ChipCondition_Ver2 (.chipcondition (Utilities|Array|Get(acopy) (Variables|Default|GetChipInfo_Ver2) (LocalVariables|GetIfArrayIndex_Local))))) (!= (LocalVariables|GetIsBad?_ConditionTypeTime) true) true)))
          (goto _label))))))

(fn EndControl
  (params (LocalArrayIndex :type Integer))
  (LocalVariables|SetEndArrayIndex LocalArrayIndex)
  (switch Utilities|FlowControl|Switch|SwitchonE_ChipEndType_Ver2 (.TypeEnd (Utilities|Struct|BreakS_ChipEnd_Ver2 (.ChipEnd (Utilities|Struct|BreakS_MagicChipInfo_Ver2 (Utilities|Array|Get(acopy) (Variables|Default|GetChipInfo_Ver2) (LocalVariables|GetEndArrayIndex))))))
    (:NewEnumerator1
      (Game|SpawnActorfromClass "/Game/Niagara/BP_Explosion.BP_Explosion_C" (Math|Transform|MakeTransform (Transformation|GetActorLocation) "0, 0, 0" (Math|Conversions|ToVector(Float) (Utilities|Struct|BreakS_ChipEnd_Explosion (.Explosion (Utilities|Struct|BreakS_ChipEnd_Ver2 (.ChipEnd (Utilities|Struct|BreakS_MagicChipInfo_Ver2 (Utilities|Array|Get(acopy) (Variables|Default|GetChipInfo_Ver2) (LocalVariables|GetEndArrayIndex))))))))) "Undefined" "MultiplyWithRoot" 0 0))))

(fn SetSpawnPosition
  (params (LocalArrayIndex :type Integer)))